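; Player-owned knight piece for a Settlers-style hex board game, colored by owner and moved between vertices.
; Clicking checks GameMode phase to start the once-per-turn move or a Sedition card steal.
; Moves highlight free vertices one step away, or two via roads, then a Timeline lerp runs the knight there, chaining two-step runs with a delay.
; It also supports card-driven teleports, outpost overlap offsets and per-player highlights outside pass-and-play.
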(event Custom|run
  (params (endVertex :type Hex%20Vertex%20Object%20Reference))
  (Variables|Default|Setmoving true)
  (bind _alpha (Timeline|Timeline_0 Play)
    (:Update
      (Transformation|SetWorldLocation (Variables|Default|GetKnight) (Math|Vector|Lerp(Vector) (Transformation|GetWorldLocation (Variables|Default|GetKnight)) (Transformation|GetWorldLocation (Variables|/Game/Blueprints/HexGrid/HexVertex.HexVertex_C|GetSphereHighlight endVertex)) _alpha) false false))
    (:Finished
      (Variables|Default|Setmoving false)
      (CallFunction|EditLocationifConflict)
      (Timeline|Timeline_0 SetNewTime))))

(event Custom|runTwice
  (params (firstLocation :type Hex%20Vertex%20Object%20Reference) (secondLocation :type Hex%20Vertex%20Object%20Reference))
  (CallFunction|Run firstLocation)
  (Variables|Default|SetcurrentVertex firstLocation)
  (Utilities|FlowControl|Delay 1.5)
  (CallFunction|Run secondLocation))

(event EventClickInteract
  (CallFunction|MaybeTriggerKnightMovement)
  (CallFunction|MaybeTriggerSedition))

(fn ConstructionScript
  (CallFunction|EditLocationifConflict)
  (CallFunction|SetColor))

(fn CheckforConflict
  (params (vertex :type Hex%20Vertex%20Object%20Reference))
  (return (Utilities|IsValid (Variables|/Game/Blueprints/HexGrid/HexVertex.HexVertex_C|Getoutpost vertex))))

(fn MaybeTriggerKnightMovement
  ;[1 1 1] Make sure we're in the turn phase + it's the current player's knight + current player's knight hasn't already been moved
  (bind _assettlers_game_mode (Utilities|Casting|CastToSettlers_GameMode (Game|GetGameMode)))
  (if (Math|Boolean|ANDBoolean (== (Variables|/Game/Settlers_GameMode.Settlers_GameMode_C|Getphase _assettlers_game_mode) 1) (== (Variables|/Game/Settlers_GameMode.Settlers_GameMode_C|GetcurrentPlayerIndex _assettlers_game_mode) (Variables|Default|GetownerIndex)) (not (Variables|/Game/Blueprints/Handlers/PlayerHandler.PlayerHandler_C|GetcurrentHasMovedKnight (Variables|/Game/Settlers_GameMode.Settlers_GameMode_C|GetplayerHandler _assettlers_game_mode))))
    ;[1 1 1] Set game phase to KnightMovement and highlight vertices.
    (Variables|/Game/Settlers_GameMode.Settlers_GameMode_C|Setphase _assettlers_game_mode 10)
    (CallFunction|HighlightValidMovements)
    ;[1 1 1] hide action panel until knight is moved
    (bind _aspc_player (Utilities|Casting|CastToPC_Player (Game|GetPlayerController 0)))
    (Default|SHideActionPanel _aspc_player)))

(fn HighlightValidMovements
  ;[1 1 1] Highlight each nearby vertex!
  (bind _returnvalue (Actor|GetActorOfClass "/Game/Blueprints/HexGrid/HexGrid.HexGrid_C"))
  (bind _nearbyverticesandedges (Default|GetNearbyfromVertex _returnvalue (Variables|Default|GetcurrentVertex)))
  (bind _keys (Utilities|Map|Keys _nearbyverticesandedges))
  (for _array_element _keys
    (CallFunction|HighlightVertexifValid _array_element)
    (if (Utilities|IsValid _array_element)
      ;[1 1 1] Check if there's a valid road on that vertex...
      (if (.ReturnValue (Utilities|Map|Find _nearbyverticesandedges _array_element))
        (if (Utilities|IsValid (Variables|/Game/Blueprints/HexGrid/HexEdge.HexEdge_C|Getroad (.Value (Utilities|Map|Find _nearbyverticesandedges _array_element))))
          (bind _nearbyverticesandedges_2 (Default|GetNearbyfromVertex _returnvalue _array_element))
          (bind _keys_2 (Utilities|Map|Keys _nearbyverticesandedges_2))
          (for _array_element_2 _keys_2
            (CallFunction|HighlightVertexifValid _array_element_2)))))))

(fn Moveto
  (params (vertex :type Hex%20Vertex%20Object%20Reference))
  ;[1 1 1] handle actual movement
  (Default|UnhighlightVertices vertex)
  (CallFunction|SetRunDirection vertex)
  (CallFunction|MaybeRun vertex)
  (Variables|Default|SetcurrentVertex vertex)
  ;[1 1 1] prevent knight from getting moved again; if using cavalry card, handle end of dcard use; if not just set back to turn phase
  (bind _assettlers_game_mode (Utilities|Casting|CastToSettlers_GameMode (Game|GetGameMode)))
  (Variables|/Game/Blueprints/Handlers/PlayerHandler.PlayerHandler_C|SetcurrentHasMovedKnight (Variables|/Game/Settlers_GameMode.Settlers_GameMode_C|GetplayerHandler _assettlers_game_mode) true)
  (if (== (Variables|/Game/Settlers_GameMode.Settlers_GameMode_C|Getphase _assettlers_game_mode) 11)
    (Default|DoneUsingCard (Variables|/Game/Settlers_GameMode.Settlers_GameMode_C|GetdcardHandler _assettlers_game_mode))
    (else
      (Variables|/Game/Settlers_GameMode.Settlers_GameMode_C|Setphase _assettlers_game_mode 1)))
  (bind _aspc_player (Utilities|Casting|CastToPC_Player (Game|GetPlayerController 0)))
  (Default|SShowActionPanel _aspc_player))

(fn EditLocationifConflict
  (bind _currentvertex (Variables|Default|GetcurrentVertex))
  (bind _knight (Variables|Default|GetKnight))
  (bind _relativelocation (Variables|/Script/Engine.SceneComponent|GetRelativeLocation _knight))
  (bind (_x _y _z) (Math|Vector|BreakVector _relativelocation))
  ;[1 1 1] make sure knight is on a vertex
  (if (Utilities|IsValid _currentvertex)
    (bind _hasconflict (CallFunction|CheckforConflict _currentvertex))
    ;[1 1 1] if conflicting, move it slightly
    (if _hasconflict
      (Transformation|SetRelativeLocation _knight (Math|Vector|MakeVector _x (+ _y 12.0) _z) false false))))

(fn Destroy
  (Components|DestroyComponent (Variables|Default|GetKnight))
  (Actor|DestroyActor))

(fn HighlightVertexifValid
  (params (vertex :type Hex%20Vertex%20Object%20Reference))
  (if (Utilities|IsValid vertex)
    (bind _outactors (Actor|GetAllActorsOfClass "Knight_C"))
    (for _array_element _outactors
      ;[1 1 1] don't highlight this vertex if it already has a knight on it
      (if (== vertex (Variables|Knight_C|GetcurrentVertex _array_element))
        (return)))
    (Default|HighlightVertex vertex)
    (bind _returnvalue (Actor|GetActorOfClass "/Game/Blueprints/HexGrid/HexGrid.HexGrid_C"))
    (Utilities|Array|AddUnique (Variables|/Game/Blueprints/HexGrid/HexGrid.HexGrid_C|GethighlightedVertices _returnvalue) vertex)))

(fn SetRunDirection
  (params (destination :type Hex%20Vertex%20Object%20Reference))
  (bind _spherehighlight (Variables|/Game/Blueprints/HexGrid/HexVertex.HexVertex_C|GetSphereHighlight destination))
  (bind _currentvertex (Variables|Default|GetcurrentVertex))
  (bind _returnvalue (Transformation|GetWorldLocation _spherehighlight))
  (bind _spherehighlight_2 (Variables|/Game/Blueprints/HexGrid/HexVertex.HexVertex_C|GetSphereHighlight _currentvertex))
  (bind _returnvalue_2 (Transformation|GetWorldLocation _spherehighlight_2))
  (bind _returnvalue_3 (Math|Rotator|FindLookatRotation _returnvalue_2 _returnvalue))
  (bind (_roll _pitch _yaw) (Math|Rotator|BreakRotator _returnvalue_3))
  ;[1 1 1] Compare current and target vertex locations and set knight rotation based on that.
  (Transformation|SetWorldRotation (Variables|Default|GetKnight) (Math|Rotator|MakeRotator _roll _pitch (+ _yaw -9e+01)) false false))

(fn SetColor
  (bind _knight (Variables|Default|GetKnight))
  (switch int (Variables|Default|GetownerIndex)
    (:Default
      (Rendering|Material|SetMaterial _knight 0 "/Game/Materials/characters/M_knight_blue.M_knight_blue" :!label _label))
    (:0
      (Rendering|Material|SetMaterial _knight 0 "/Game/Materials/characters/M_knight_red.M_knight_red"))
    (:1
      (goto _label))
    (:2
      (Rendering|Material|SetMaterial _knight 0 "/Game/Materials/characters/M_knight_pink.M_knight_pink"))
    (:3
      (Rendering|Material|SetMaterial _knight 0 "/Game/Materials/characters/M_knight_purple.M_knight_purple"))))

(fn HighlightMoveAnywhere
  (bind _outactors (Actor|GetAllActorsOfClass "/Game/Blueprints/HexGrid/HexVertex.HexVertex_C"))
  (for _array_element _outactors
    (if (!= _array_element (Variables|Default|GetcurrentVertex))
      (CallFunction|HighlightVertexifValid _array_element))))

(fn MaybeTriggerSedition
  ;[1 1 1] make sure we're in the d card phase + player is using sedition + player isnt trying to steal their own knight
  (bind _assettlers_game_mode (Utilities|Casting|CastToSettlers_GameMode (Game|GetGameMode)))
  (if (Math|Boolean|ANDBoolean (== (Variables|/Game/Settlers_GameMode.Settlers_GameMode_C|Getphase _assettlers_game_mode) 11) (!= (Variables|/Game/Settlers_GameMode.Settlers_GameMode_C|GetcurrentPlayerIndex _assettlers_game_mode) (Variables|Default|GetownerIndex)) (Utilities|Enum|Equal(Enum) (Variables|/Game/Blueprints/Handlers/DCardHandler.DCardHandler_C|GetcurrentlyUsedCard (Variables|/Game/Settlers_GameMode.Settlers_GameMode_C|GetdcardHandler _assettlers_game_mode)) "NewEnumerator2"))
    ;[1 1 1] add game log message for sedition
    (bind _aspc_player (Utilities|Casting|CastToPC_Player (Game|GetPlayerController 0)))
    (bind _gamelog (Variables|/Game/Blueprints/Player/PC_Player.PC_Player_C|GetgameLog _aspc_player)
      (:then
        (bind _message (Default|AddSeditionMessage _gamelog (Variables|/Game/Settlers_GameMode.Settlers_GameMode_C|GetcurrentPlayerIndex _assettlers_game_mode) (Variables|Default|GetownerIndex)))
        (if (Variables|/Game/Settlers_GameMode.Settlers_GameMode_C|GetGM_gameIsPP _assettlers_game_mode)
          _
          (else
            (Default|EveryoneLogMessage _assettlers_game_mode _message)))
        ;[1 1 1] remove the knight from the owner and give it to the current player. (if stealing player has no knights to begin with, DoneUsingCard is called AFTER knight asset is spawned)
        (CallFunction|UnhighlightAll)
        (Default|RemovePlayerKnights (Variables|/Game/Settlers_GameMode.Settlers_GameMode_C|GetplayerHandler _assettlers_game_mode) (Variables|Default|GetownerIndex))
        (Default|BuildKnight (Variables|/Game/Settlers_GameMode.Settlers_GameMode_C|GetzombieHandler _assettlers_game_mode) true))
      (:else))))

(fn MaybeRun
  (params (endVertex :type Hex%20Vertex%20Object%20Reference))
  (bind _currentvertex (Variables|Default|GetcurrentVertex))
  ;[1 1 1] Check if we're directly adjacent.
  (bind _isadjacent (Default|IsAdjacenttoVertex endVertex _currentvertex))
  (if _isadjacent
    (CallFunction|Run endVertex)
    (else
      ;[1 1 1] Otherwise, we run twice.
      (bind _vertexbetween (Default|GetVertexBetween _currentvertex endVertex))
      (CallFunction|RunTwice _vertexbetween endVertex))))

(fn Teleportto
  (params (endVertex :type Hex%20Vertex%20Object%20Reference))
  (Default|UnhighlightVertices endVertex)
  (Transformation|SetWorldLocation (Variables|Default|GetKnight) (Transformation|GetWorldLocation (Variables|/Game/Blueprints/HexGrid/HexVertex.HexVertex_C|GetSphereHighlight endVertex)) false false)
  (Variables|Default|SetcurrentVertex endVertex)
  ;[1 1 1] handle usage of cavalry card
  (bind _assettlers_game_mode (Utilities|Casting|CastToSettlers_GameMode (Game|GetGameMode)))
  (Default|DoneUsingCard (Variables|/Game/Settlers_GameMode.Settlers_GameMode_C|GetdcardHandler _assettlers_game_mode))
  (bind _aspc_player (Utilities|Casting|CastToPC_Player (Game|GetPlayerController 0)))
  (Default|UpdateButtons (Variables|/Game/Blueprints/Player/PC_Player.PC_Player_C|GetactionPanel _aspc_player)))

(fn Highlight
  (bind _assettlers_game_instance (Utilities|Casting|CastToSettlersGameInstance (Game|GetGameInstance)))
  (if (Variables|/Game/Blueprints/SettlersGameInstance.SettlersGameInstance_C|GetisPassAndPlay _assettlers_game_instance)
    (Rendering|SetVisibility (Variables|Default|GetKnightHighlight) true true)
    (else
      (bind _assettlers_game_mode (Utilities|Casting|CastToSettlers_GameMode (Game|GetGameMode)))
      (Default|CSetKnightHighlightVis (Utilities|Array|Get(acopy) (Variables|/Game/Settlers_GameMode.Settlers_GameMode_C|GetallPlayerControllers _assettlers_game_mode) (Variables|/Game/Settlers_GameMode.Settlers_GameMode_C|GetcurrentPlayerIndex _assettlers_game_mode)) self false))))

(fn Unhighlight
  (bind _assettlers_game_instance (Utilities|Casting|CastToSettlersGameInstance (Game|GetGameInstance)))
  (if (Variables|/Game/Blueprints/SettlersGameInstance.SettlersGameInstance_C|GetisPassAndPlay _assettlers_game_instance)
    (Rendering|SetVisibility (Variables|Default|GetKnightHighlight) false true)
    (else
      (bind _assettlers_game_mode (Utilities|Casting|CastToSettlers_GameMode (Game|GetGameMode)))
      (Default|CSetKnightHighlightVis (Utilities|Array|Get(acopy) (Variables|/Game/Settlers_GameMode.Settlers_GameMode_C|GetallPlayerControllers _assettlers_game_mode) (Variables|/Game/Settlers_GameMode.Settlers_GameMode_C|GetcurrentPlayerIndex _assettlers_game_mode)) self true))))

(fn UnhighlightAll
  (bind _outactors (Actor|GetAllActorsOfClass "Knight_C"))
  (for _array_element _outactors
    (CallFunction|Unhighlight _array_element)))