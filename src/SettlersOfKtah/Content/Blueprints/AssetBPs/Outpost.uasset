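; Outpost Blueprint, a replicated board piece with Outpost and Apothecary components that can be clicked by the player.
; On begin play it sets both components to replicate.
; A click interaction forwards to its Vertex reference's VertexClicked, and a RepNotify material variable applies the outpost material to the Outpost component on clients.
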(event Collision|EventActorBeginOverlap
  (params (OtherActor :type Actor%20Object%20Reference)))

(event EventTick
  (params (DeltaSeconds :type Float%20%28single-precision%29)))

(event MouseInput|EventActorOnClicked
  (params (ButtonPressed :type Key%20Structure :default "None")))

(event EventClickInteract
  (Default|VertexClicked (Variables|Default|Getvertex)))

(event EventBeginPlay
  (Class|ActorComponent|SetIsReplicated (Variables|Components|Getoutpost) true)
  (Class|ActorComponent|SetIsReplicated (Variables|Components|Getapothecary) true))

(fn ConstructionScript)

(fn OnRepOutpostMaterial
  (Rendering|Material|SetMaterial (Variables|Components|Getoutpost) 0 (Variables|Default|GetoutpostMaterial)))