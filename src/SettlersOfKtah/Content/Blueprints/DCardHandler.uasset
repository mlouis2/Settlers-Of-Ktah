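; Handles development cards in a Settlers-style game: random draws by category, purchase, per-player card counts and card effects.
; UseCard sets the game mode phase and dispatches by card type to tile, knight, barricade or trade handlers, several still stubbed.
; Tile clicks apply permanent or temporary bounty changes, then the card is removed and the phase reset.
; UpdateTempBounties counts turns to expire Fertilizer boosts.
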(event EventBeginPlay)

(event Collision|EventActorBeginOverlap
  (params (OtherActor :type Actor%20Object%20Reference)))

(event EventTick
  (params (DeltaSeconds :type Float%20%28single-precision%29)))

(fn ConstructionScript)

(fn PickRandomCard
  (params (cardCategory :type Integer))
  (switch int cardCategory
    (:0
      (return (Utilities|Enum|ByteToEnumDCards_Enum (Math|Conversions|ToByte(Integer) (Math|Random|RandomIntegerinRange 0 4)))))
    (:1
      (return (Utilities|Enum|ByteToEnumDCards_Enum (Math|Conversions|ToByte(Integer) (Math|Random|RandomIntegerinRange 5 8)))))
    (:2
      (return (Utilities|Enum|ByteToEnumDCards_Enum (Math|Conversions|ToByte(Integer) (Math|Random|RandomIntegerinRange 9 12)))))))

(fn AddCardtoPlayer
  (params (card :type DCards_Enum%20Enum :default "NewEnumerator0") (playerIndex :type Integer))
  (bind _tempmap (Variables|Default|GettempMap))
  (bind _tempmap_2 (Variables|Default|GettempMap))
  (bind _assettlers_game_mode (Utilities|Casting|CastToSettlers_GameMode (Game|GetGameMode)))
  (Utilities|Map|Clear _tempmap)
  (bind _keys (Utilities|Map|Keys (.ownedCards (Utilities|Struct|BreakBP_PlayerStruct (Utilities|Array|Get(acopy) (Variables|/Game/Settlers_GameMode.Settlers_GameMode_C|Getplayers _assettlers_game_mode) playerIndex)))))
  (for _array_element _keys
    (Utilities|Map|Add _tempmap _array_element (.Value (Utilities|Map|Find (.ownedCards (Utilities|Struct|BreakBP_PlayerStruct (Utilities|Array|Get(acopy) (Variables|/Game/Settlers_GameMode.Settlers_GameMode_C|Getplayers _assettlers_game_mode) playerIndex))) _array_element))))
  (Utilities|Map|Add _tempmap_2 card (+ (.Value (Utilities|Map|Find _tempmap_2 card)) 1))
  (Utilities|Struct|SetmembersinBP_PlayerStruct (Utilities|Array|Get(acopy) (Variables|/Game/Settlers_GameMode.Settlers_GameMode_C|Getplayers _assettlers_game_mode) playerIndex) _tempmap_2))

(fn GetDescription
  (params (cardType :type DCards_Enum%20Enum :default "NewEnumerator0"))
  (return (.Value (Utilities|Map|Find (Variables|Default|GetdescriptionsMap) cardType))))

(fn UseCard
  (Utilities|FlowControl|Sequence
    (:then_0
      (bind _assettlers_game_mode (Utilities|Casting|CastToSettlers_GameMode (Game|GetGameMode)))
      (Variables|/Game/Settlers_GameMode.Settlers_GameMode_C|Setphase _assettlers_game_mode 11))
    (:then_1
      (switch Utilities|FlowControl|Switch|SwitchonDCards_Enum (Variables|Default|GetcurrentlyUsedCard)
        (:NewEnumerator0
          (CallFunction|UseTileRelatedCards :!label _label))
        (:NewEnumerator1
          (goto _label))
        (:NewEnumerator2
          (CallFunction|UseKnightRelatedCards :!label _label_2))
        (:NewEnumerator3
          (CallFunction|UseBarricadeRelatedCards :!label _label_3))
        (:NewEnumerator4
          (goto _label_2))
        (:NewEnumerator5
          (goto _label))
        (:NewEnumerator6
          (goto _label_2))
        (:NewEnumerator7
          (goto _label_3))
        (:NewEnumerator8
          (goto _label_2))
        (:NewEnumerator9
          (goto _label))
        (:NewEnumerator10
          (goto _label_3))
        (:NewEnumerator12
          (CallFunction|UseTradeCard))))))

(fn RemoveCardfromPlayer
  (params (cardType :type DCards_Enum%20Enum :default "NewEnumerator0"))
  (bind _tempmap (Variables|Default|GettempMap))
  (bind _tempmap_2 (Variables|Default|GettempMap))
  (bind _value (Utilities|Map|Find _tempmap_2 cardType))
  (bind _assettlers_game_mode (Utilities|Casting|CastToSettlers_GameMode (Game|GetGameMode)))
  (Utilities|Map|Clear _tempmap)
  (bind _keys (Utilities|Map|Keys (.ownedCards (Utilities|Struct|BreakBP_PlayerStruct (Utilities|Array|Get(acopy) (Variables|/Game/Settlers_GameMode.Settlers_GameMode_C|Getplayers _assettlers_game_mode) (Variables|/Game/Settlers_GameMode.Settlers_GameMode_C|GetcurrentPlayerIndex _assettlers_game_mode))))))
  (for _array_element _keys
    (Utilities|Map|Add _tempmap _array_element (.Value (Utilities|Map|Find (.ownedCards (Utilities|Struct|BreakBP_PlayerStruct (Utilities|Array|Get(acopy) (Variables|/Game/Settlers_GameMode.Settlers_GameMode_C|Getplayers _assettlers_game_mode) (Variables|/Game/Settlers_GameMode.Settlers_GameMode_C|GetcurrentPlayerIndex _assettlers_game_mode)))) _array_element))))
  (if (== _value 1)
    (Utilities|Map|Remove _tempmap_2 cardType)
    (else
      (Utilities|Map|Add _tempmap_2 cardType (- _value 1))))
  (Utilities|Struct|SetmembersinBP_PlayerStruct (Utilities|Array|Get(acopy) (Variables|/Game/Settlers_GameMode.Settlers_GameMode_C|Getplayers _assettlers_game_mode) (Variables|/Game/Settlers_GameMode.Settlers_GameMode_C|GetcurrentPlayerIndex _assettlers_game_mode)) _tempmap_2))

(fn AddResearchCardtoPlayer
  (params (playerIndex :type Integer))
  (bind _card (CallFunction|PickRandomCard 2))
  (CallFunction|AddCardtoPlayer _card playerIndex))

(fn AddMilitaryCardtoPlayer
  (params (playerIndex :type Integer))
  (bind _card (CallFunction|PickRandomCard 1))
  (CallFunction|AddCardtoPlayer _card playerIndex))

(fn BuyGenericCard
  (bind _assettlers_game_mode (Utilities|Casting|CastToSettlers_GameMode (Game|GetGameMode)))
  (bind _card (CallFunction|PickRandomCard 0))
  (CallFunction|AddCardtoPlayer _card (Variables|/Game/Settlers_GameMode.Settlers_GameMode_C|GetcurrentPlayerIndex _assettlers_game_mode))
  (Default|RemoveResourcefromPlayer (Variables|/Game/Settlers_GameMode.Settlers_GameMode_C|GetresourceHandler _assettlers_game_mode) (Variables|Default|GetcardCost) (Variables|/Game/Settlers_GameMode.Settlers_GameMode_C|GetcurrentPlayerIndex _assettlers_game_mode))
  (Default|UpdateResourcesUI (Variables|/Game/Settlers_GameMode.Settlers_GameMode_C|GetresourceHandler _assettlers_game_mode))
  (return _card))

(fn UseTileRelatedCards
  (CallFunction|RemoveModalView)
  (bind _outactors (Actor|GetAllActorsOfClass "/Game/Blueprints/HexTile.HexTile_C"))
  (switch Utilities|FlowControl|Switch|SwitchonDCards_Enum (Variables|Default|GetcurrentlyUsedCard)
    (:NewEnumerator0
      (for _array_element _outactors :!label _label
        (Default|HighlightTile _array_element)))
    (:NewEnumerator1
      (goto _label))
    (:NewEnumerator5
      ;[1 1 1] if more than one infected tile, highlight infected tiles that player can transfer
      (bind _returnvalue (Actor|GetActorOfClass "/Game/Blueprints/HexGrid.HexGrid_C"))
      (if (> (Variables|/Game/Blueprints/HexGrid.HexGrid_C|GetnumTilesInfected _returnvalue) 1)
        (bind _assettlers_game_mode (Utilities|Casting|CastToSettlers_GameMode (Game|GetGameMode)))
        (Default|HighlightPlayerSpreadTiles (Variables|/Game/Settlers_GameMode.Settlers_GameMode_C|GetzombieHandler _assettlers_game_mode) true)))
    (:NewEnumerator9
      (goto _label))))

(fn UseTradeCard)

(fn UseKnightRelatedCards
  (bind _assettlers_game_mode (Utilities|Casting|CastToSettlers_GameMode (Game|GetGameMode)))
  (switch Utilities|FlowControl|Switch|SwitchonDCards_Enum (Variables|Default|GetcurrentlyUsedCard)
    (:NewEnumerator6
      (Default|BuildKnight (Variables|/Game/Settlers_GameMode.Settlers_GameMode_C|GetzombieHandler _assettlers_game_mode))
      (CallFunction|DoneUsingCard))))

(fn UseBarricadeRelatedCards
  (CallFunction|RemoveModalView))

(fn HandleTileonClickforDCard
  (params (tileClicked :type Hex%20Tile%20Object%20Reference))
  (Utilities|FlowControl|Sequence
    (:then_0
      (switch Utilities|FlowControl|Switch|SwitchonDCards_Enum (Variables|Default|GetcurrentlyUsedCard)
        (:NewEnumerator0
          ;[1 1 1] salt the earth: if owner's bounty number is greater than 1, reduce it permanently by 1
          (if (> (Variables|/Game/Blueprints/HexTile.HexTile_C|Getbounty tileClicked) 1)
            (Variables|/Game/Blueprints/HexTile.HexTile_C|Setbounty tileClicked (- (Variables|/Game/Blueprints/HexTile.HexTile_C|Getbounty tileClicked) 1))
            (Default|UpdateOwnerBountyText tileClicked)))
        (:NewEnumerator1
          ;[1 1 1] seed the earth: if owner's bounty number is less than 3, permanently increase by 1
          (if (< (Variables|/Game/Blueprints/HexTile.HexTile_C|Getbounty tileClicked) 3)
            (Variables|/Game/Blueprints/HexTile.HexTile_C|Setbounty tileClicked (+ (Variables|/Game/Blueprints/HexTile.HexTile_C|Getbounty tileClicked) 1))
            (Default|UpdateOwnerBountyText tileClicked)))
        (:NewEnumerator9
          ;[1 1 1] fertilizer: if tile doesn't currently have an upgrade, increase its bounty for 3 turns
          (if (not (Utilities|Array|ContainsItem (Variables|Default|GettilesWithTempBountyUpgrade) tileClicked))
            (Variables|/Game/Blueprints/HexTile.HexTile_C|Setbounty tileClicked (+ (Variables|/Game/Blueprints/HexTile.HexTile_C|Getbounty tileClicked) 1))
            (Variables|/Game/Blueprints/HexTile.HexTile_C|SetbountyUpgradeTurnCount tileClicked 0)
            (Default|UpdateOwnerBountyText tileClicked)
            (Utilities|Array|Add (Variables|Default|GettilesWithTempBountyUpgrade) tileClicked)))))
    (:then_1
      (bind _returnvalue (Actor|GetActorOfClass "/Game/Blueprints/HexGrid.HexGrid_C"))
      (Default|UnhighlightAllTiles _returnvalue)
      (CallFunction|DoneUsingCard))))

(fn DoneUsingCard
  (bind _assettlers_game_mode (Utilities|Casting|CastToSettlers_GameMode (Game|GetGameMode)))
  (Variables|/Game/Settlers_GameMode.Settlers_GameMode_C|Setphase _assettlers_game_mode 1)
  (CallFunction|RemoveCardfromPlayer (Variables|Default|GetcurrentlyUsedCard)))

(fn RemoveModalView
  (Widget|RemovefromParent (Variables|Default|GetdevCardMainScreen))
  (Variables|Default|SetdevCardMainScreen 0))

(fn UpdateTempBounties
  (for _array_element (Variables|Default|GettilesWithTempBountyUpgrade)
    ;[1 1 1] if bounty upgrade turn count reached, restore bounty to original number
    (if (== (Variables|/Game/Blueprints/HexTile.HexTile_C|GetbountyUpgradeTurnCount _array_element) 3)
      (Variables|/Game/Blueprints/HexTile.HexTile_C|Setbounty _array_element (- (Variables|/Game/Blueprints/HexTile.HexTile_C|Getbounty _array_element) 1))
      (Default|UpdateOwnerBountyText _array_element)
      (Utilities|Array|RemoveItem (Variables|Default|GettilesWithTempBountyUpgrade) _array_element)
      (else
        ;[1 1 1] otherwise, increment turn count
        (Variables|/Game/Blueprints/HexTile.HexTile_C|SetbountyUpgradeTurnCount _array_element (+ (Variables|/Game/Blueprints/HexTile.HexTile_C|GetbountyUpgradeTurnCount _array_element) 1))))))