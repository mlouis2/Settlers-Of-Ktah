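; Handler for development cards in the Settlers game: draws random cards by category, adjusts player counts and plays card effects.
; UseCard routes CurrentlyUsedCard to tile, knight, barricade or resource functions, which highlight targets or call ZombieHandler, PlayerHandler and TradeHandler.
; DoneUsingCard removes the card, resets the phase and logs locally or to everyone.
; Fertilizer's temporary bounties are tracked in a tile-to-player map and expired by round count.
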(fn ConstructionScript)

(fn PickRandomCard
  (params (cardCategory :type Integer))
  (switch int cardCategory
    (:0
      (return (Utilities|Enum|ByteToEnumDCards_Enum (Math|Conversions|ToByte(Integer) (Math|Random|RandomIntegerinRange 0 4)))))
    (:1
      (return (Utilities|Enum|ByteToEnumDCards_Enum (Math|Conversions|ToByte(Integer) (Math|Random|RandomIntegerinRange 5 8)))))
    (:2
      (return (Utilities|Enum|ByteToEnumDCards_Enum (Math|Conversions|ToByte(Integer) (Math|Random|RandomIntegerinRange 9 12)))))))

(fn AddCardtoPlayer
  (params (card :type DCards_Enum%20Enum :default "NewEnumerator0") (playerIndex :type Integer))
  (bind _assettlers_game_mode (Utilities|Casting|CastToSettlers_GameMode (Game|GetGameMode)))
  (for (_array_element _array_index) (.numDCardsStructs (Utilities|Struct|BreakBP_PlayerStruct (Utilities|Array|Get(acopy) (Variables|/Game/Settlers_GameMode.Settlers_GameMode_C|Getplayers _assettlers_game_mode) playerIndex)))
    (if (== card (.DcardType (Utilities|Struct|BreakDCardStruct _array_element)))
      (Utilities|Array|SetArrayElem (.numDCardsStructs (Utilities|Struct|BreakBP_PlayerStruct (Utilities|Array|Get(acopy) (Variables|/Game/Settlers_GameMode.Settlers_GameMode_C|Getplayers _assettlers_game_mode) playerIndex))) _array_index (Utilities|Struct|MakeDCardStruct card (+ (.count (Utilities|Struct|BreakDCardStruct _array_element)) 1)))
      ;[1 1 1] if multiplayer, update player struct for each player
      (bind _assettlers_game_instance (Utilities|Casting|CastToSettlersGameInstance (Game|GetGameInstance)))
      (if (not (Variables|/Game/Blueprints/SettlersGameInstance.SettlersGameInstance_C|GetisPassAndPlay _assettlers_game_instance))
        (Default|UpdateAllPlayersInfo _assettlers_game_mode)))))

(fn GetDescription
  (params (cardType :type DCards_Enum%20Enum :default "NewEnumerator0"))
  (bind _assettlers_game_state (Utilities|Casting|CastToSettlersGameState (Game|GetGameState)))
  (return (.Value (Utilities|Map|Find (Variables|/Game/Blueprints/SettlersGameState.SettlersGameState_C|GetGS_DcardDescriptions _assettlers_game_state) cardType))))

(fn UseCard
  (Utilities|FlowControl|Sequence
    (:then_0
      (bind _assettlers_game_mode (Utilities|Casting|CastToSettlers_GameMode (Game|GetGameMode)))
      (Variables|/Game/Settlers_GameMode.Settlers_GameMode_C|Setphase _assettlers_game_mode 11))
    (:then_1
      (switch Utilities|FlowControl|Switch|SwitchonDCards_Enum (Variables|Temp|GetcurrentlyUsedCard)
        (:NewEnumerator0
          (CallFunction|UseTileRelatedCards :!label _label))
        (:NewEnumerator1
          (goto _label))
        (:NewEnumerator2
          (CallFunction|UseKnightRelatedCards :!label _label_2))
        (:NewEnumerator3
          (CallFunction|UseBarricadeRelatedCards :!label _label_3))
        (:NewEnumerator4
          (goto _label_2))
        (:NewEnumerator5
          (goto _label))
        (:NewEnumerator6
          (goto _label_2))
        (:NewEnumerator7
          (goto _label_3))
        (:NewEnumerator8
          (goto _label_2))
        (:NewEnumerator9
          (goto _label))
        (:NewEnumerator10
          (CallFunction|UseResourceRelatedCards :!label _label_4))
        (:NewEnumerator11
          (goto _label))
        (:NewEnumerator12
          (goto _label_4))))))

(fn RemoveCardfromPlayer
  (params (cardType :type DCards_Enum%20Enum :default "NewEnumerator0"))
  (bind _assettlers_game_mode (Utilities|Casting|CastToSettlers_GameMode (Game|GetGameMode)))
  (for (_array_element _array_index) (.numDCardsStructs (Utilities|Struct|BreakBP_PlayerStruct (Utilities|Array|Get(acopy) (Variables|/Game/Settlers_GameMode.Settlers_GameMode_C|Getplayers _assettlers_game_mode) (Variables|/Game/Settlers_GameMode.Settlers_GameMode_C|GetcurrentPlayerIndex _assettlers_game_mode))))
    (if (== cardType (.DcardType (Utilities|Struct|BreakDCardStruct _array_element)))
      (Utilities|Array|SetArrayElem (.numDCardsStructs (Utilities|Struct|BreakBP_PlayerStruct (Utilities|Array|Get(acopy) (Variables|/Game/Settlers_GameMode.Settlers_GameMode_C|Getplayers _assettlers_game_mode) (Variables|/Game/Settlers_GameMode.Settlers_GameMode_C|GetcurrentPlayerIndex _assettlers_game_mode)))) _array_index (Utilities|Struct|MakeDCardStruct cardType (- (.count (Utilities|Struct|BreakDCardStruct _array_element)) 1)))
      ;[1 1 1] if multiplayer, update player struct for each player
      (bind _assettlers_game_instance (Utilities|Casting|CastToSettlersGameInstance (Game|GetGameInstance)))
      (if (not (Variables|/Game/Blueprints/SettlersGameInstance.SettlersGameInstance_C|GetisPassAndPlay _assettlers_game_instance))
        (Default|UpdateAllPlayersInfo _assettlers_game_mode)))))

(fn AddResearchCardtoPlayer
  (params (playerIndex :type Integer))
  (bind _card (CallFunction|PickRandomCard 2 :!label _label))
  ;[1 1 1] extra caution to make sure invalid card not chosen
  (if (Utilities|Enum|Equal(Enum) _card "NewEnumerator13")
    (goto _label)
    (else
      (CallFunction|AddCardtoPlayer _card playerIndex))))

(fn AddMilitaryCardtoPlayer
  (params (playerIndex :type Integer))
  (bind _card (CallFunction|PickRandomCard 1 :!label _label))
  ;[1 1 1] extra caution to make sure invalid card not chosen
  (if (Utilities|Enum|Equal(Enum) _card "NewEnumerator13")
    (goto _label)
    (else
      (CallFunction|AddCardtoPlayer _card playerIndex))))

(fn BuyGenericCard
  (bind _assettlers_game_mode (Utilities|Casting|CastToSettlers_GameMode (Game|GetGameMode)))
  (bind _card (CallFunction|PickRandomCard 0 :!label _label))
  ;[1 1 1] extra caution to make sure invalid card not chosen
  (if (Utilities|Enum|Equal(Enum) _card "NewEnumerator13")
    (goto _label)
    (else
      (CallFunction|AddCardtoPlayer _card (Variables|/Game/Settlers_GameMode.Settlers_GameMode_C|GetcurrentPlayerIndex _assettlers_game_mode))
      (bind _assettlers_game_state (Utilities|Casting|CastToSettlersGameState (Game|GetGameState)))
      (Default|RemoveResourcefromPlayer (Variables|/Game/Settlers_GameMode.Settlers_GameMode_C|GetresourceHandler _assettlers_game_mode) (Variables|/Game/Settlers_GameMode.Settlers_GameMode_C|GetcurrentPlayerIndex _assettlers_game_mode) (Variables|/Game/Blueprints/SettlersGameState.SettlersGameState_C|GetdCardCost _assettlers_game_state))
      (Default|UpdateResourcesUI (Variables|/Game/Settlers_GameMode.Settlers_GameMode_C|GetresourceHandler _assettlers_game_mode))
      (return _card))))

(fn UseTileRelatedCards
  (bind _currentlyusedcard (Variables|Temp|GetcurrentlyUsedCard))
  (CallFunction|RemoveModalView)
  (switch Utilities|FlowControl|Switch|SwitchonDCards_Enum _currentlyusedcard
    (:NewEnumerator0
      ;[1 1 1] highlight tiles that can be used
      (CallFunction|GetValidTilesforBounty _currentlyusedcard :!label _label)
      (for _array_element (Variables|Temp|GetvalidTilesToBeUsed)
        (Default|HighlightTile _array_element)))
    (:NewEnumerator1
      (goto _label))
    (:NewEnumerator5
      ;[1 1 1] highlight infected tiles that player can transfer / uninfect
      (bind _assettlers_game_mode (Utilities|Casting|CastToSettlers_GameMode (Game|GetGameMode) :!label _label_2))
      (Default|HighlightPlayerSpreadTiles (Variables|/Game/Settlers_GameMode.Settlers_GameMode_C|GetzombieHandler _assettlers_game_mode) true))
    (:NewEnumerator9
      (goto _label))
    (:NewEnumerator11
      (goto _label_2))))

(fn UseResourceRelatedCards
  (switch Utilities|FlowControl|Switch|SwitchonDCards_Enum (Variables|Temp|GetcurrentlyUsedCard)
    (:NewEnumerator10
      (bind _assettlers_game_mode (Utilities|Casting|CastToSettlers_GameMode (Game|GetGameMode)))
      (Variables|/Game/Blueprints/Handlers/TradeHandler.TradeHandler_C|SetnumSelectedForResourceful (Variables|/Game/Settlers_GameMode.Settlers_GameMode_C|GettradeHandler _assettlers_game_mode) 0)
      (bind _aspc_player (Utilities|Casting|CastToPC_Player (Game|GetPlayerController 0)))
      (bind _dcardmodal (Variables|/Game/Blueprints/Player/PC_Player.PC_Player_C|GetdCardModal _aspc_player)
        (:then
          (Class|WidgetSwitcher|SetActiveWidgetIndex (Variables|/Game/Blueprints/UI/DCards/DCards_Main.DCards_Main_C|GetdcardSwitcher _dcardmodal) 1)
          (Default|ResetResourcefulModal (Variables|/Game/Blueprints/UI/DCards/DCards_Main.DCards_Main_C|GetDCards_Resourceful _dcardmodal)))
        (:else)))
    (:NewEnumerator12
      (CallFunction|RemoveModalView)
      (bind _assettlers_game_mode_2 (Utilities|Casting|CastToSettlers_GameMode (Game|GetGameMode)))
      (Variables|/Game/Blueprints/Handlers/TradeHandler.TradeHandler_C|SettransmuteEnabled (Variables|/Game/Settlers_GameMode.Settlers_GameMode_C|GettradeHandler _assettlers_game_mode_2) true)
      (CallFunction|DoneUsingCard))))

(fn UseKnightRelatedCards
  (bind _assettlers_game_mode (Utilities|Casting|CastToSettlers_GameMode (Game|GetGameMode)))
  (switch Utilities|FlowControl|Switch|SwitchonDCards_Enum (Variables|Temp|GetcurrentlyUsedCard)
    (:NewEnumerator2
      (Default|UseSeditionCard (Variables|/Game/Settlers_GameMode.Settlers_GameMode_C|GetzombieHandler _assettlers_game_mode))
      (CallFunction|RemoveModalView))
    (:NewEnumerator4
      (CallFunction|RemoveModalView)
      (Default|UseCavalryCard (Variables|/Game/Settlers_GameMode.Settlers_GameMode_C|GetzombieHandler _assettlers_game_mode)))
    (:NewEnumerator6
      (Default|BuildKnight (Variables|/Game/Settlers_GameMode.Settlers_GameMode_C|GetzombieHandler _assettlers_game_mode) false)
      (bind _aspc_player (Utilities|Casting|CastToPC_Player (Game|GetPlayerController 0)))
      (bind _dcardmodal (Variables|/Game/Blueprints/Player/PC_Player.PC_Player_C|GetdCardModal _aspc_player)
        (:then
          (Default|ResetGrid _dcardmodal)
          (CallFunction|DoneUsingCard))
        (:else)))
    (:NewEnumerator8
      (Default|InspireCurrentPlayer (Variables|/Game/Settlers_GameMode.Settlers_GameMode_C|GetplayerHandler _assettlers_game_mode))
      (CallFunction|RemoveModalView)
      (CallFunction|DoneUsingCard))))

(fn UseBarricadeRelatedCards
  (Utilities|Casting|CastToSettlers_GameMode (Game|GetGameMode))
  (switch Utilities|FlowControl|Switch|SwitchonDCards_Enum (Variables|Temp|GetcurrentlyUsedCard)
    (:NewEnumerator3
      (bind _returnvalue (Actor|GetActorOfClass "/Game/Blueprints/HexGrid/HexEdge.HexEdge_C"))
      (Default|HighlightValidRoads _returnvalue)
      (CallFunction|RemoveModalView))
    (:NewEnumerator7
      (bind _returnvalue_2 (Actor|GetActorOfClass "/Game/Blueprints/HexGrid/HexEdge.HexEdge_C"))
      (Default|HighlightValidBarricades _returnvalue_2)
      (CallFunction|RemoveModalView))))

(fn HandleTileonClickforDCard
  (params (tileClicked :type Hex%20Tile%20Object%20Reference))
  (bind _validtilestobeused (Variables|Temp|GetvalidTilesToBeUsed))
  (bind _bountytext (Variables|/Game/Blueprints/HexGrid/HexTile.HexTile_C|GetbountyText tileClicked))
  (bind _bountytext_2 (Variables|/Game/Blueprints/HexGrid/HexTile.HexTile_C|GetbountyText tileClicked))
  (bind _bountytext_3 (Variables|/Game/Blueprints/HexGrid/HexTile.HexTile_C|GetbountyText tileClicked))
  ;[1 1 1] ignore click if tile not highlighted
  (if (Utilities|IsValid (Variables|/Game/Blueprints/HexGrid/HexTile.HexTile_C|Gethighlight tileClicked))
    (Utilities|FlowControl|Sequence
      (:then_0
        (switch Utilities|FlowControl|Switch|SwitchonDCards_Enum (Variables|Temp|GetcurrentlyUsedCard)
          (:NewEnumerator0
            ;[1 1 1] salt the earth: permanently reduce owner's bounty number by 1
            (if (Utilities|Array|ContainsItem _validtilestobeused tileClicked)
              (Variables|/Game/Blueprints/HexGrid/HexTile.HexTile_C|Setbounty tileClicked (- (Variables|/Game/Blueprints/HexGrid/HexTile.HexTile_C|Getbounty tileClicked) 1))
              (Default|UpdateOwnerBountyText tileClicked)
              ;[1 1 1] bounty animation
              (if (Widget|IsVisible _bountytext)
                (UserInterface|Animation|PlayAnimation _bountytext (Variables|/Game/Blueprints/UI/BountyText.BountyText_C|GetscaleAnimation _bountytext) 0.0 1 "Forward" 1.0 false))))
          (:NewEnumerator1
            ;[1 1 1] seed the earth: permanently increase owner's bounty number by 1
            (if (Utilities|Array|ContainsItem _validtilestobeused tileClicked)
              (Variables|/Game/Blueprints/HexGrid/HexTile.HexTile_C|Setbounty tileClicked (+ (Variables|/Game/Blueprints/HexGrid/HexTile.HexTile_C|Getbounty tileClicked) 1))
              (Default|UpdateOwnerBountyText tileClicked)
              ;[1 1 1] bounty animation
              (if (Widget|IsVisible _bountytext_2)
                (UserInterface|Animation|PlayAnimation _bountytext_2 (Variables|/Game/Blueprints/UI/BountyText.BountyText_C|GetscaleAnimation _bountytext_2) 0.0 1 "Forward" 1.0 false))))
          (:NewEnumerator9
            ;[1 1 1] fertilizer: increase tile's bounty for 3 rounds
            (if (Utilities|Array|ContainsItem (Variables|Temp|GetvalidTilesToBeUsed) tileClicked)
              (Variables|/Game/Blueprints/HexGrid/HexTile.HexTile_C|Setbounty tileClicked (+ (Variables|/Game/Blueprints/HexGrid/HexTile.HexTile_C|Getbounty tileClicked) 1))
              (Variables|/Game/Blueprints/HexGrid/HexTile.HexTile_C|SetbountyUpgradeRoundCount tileClicked 0)
              (Default|UpdateOwnerBountyText tileClicked)
              (bind _assettlers_game_mode (Utilities|Casting|CastToSettlers_GameMode (Game|GetGameMode)))
              (Utilities|Map|Add (Variables|Temp|GettilesWithTempBountyUpgrade) tileClicked (Variables|/Game/Settlers_GameMode.Settlers_GameMode_C|GetcurrentPlayerIndex _assettlers_game_mode))
              ;[1 1 1] bounty animation
              (if (Widget|IsVisible _bountytext_3)
                (UserInterface|Animation|PlayAnimation _bountytext_3 (Variables|/Game/Blueprints/UI/BountyText.BountyText_C|GetscaleAnimation _bountytext_3) 0.0 1 "Forward" 1.0 false))))
          (:NewEnumerator11
            ;[1 1 1] potions: uninfect tile
            (Default|UninfectTile tileClicked))))
      (:then_1
        (bind _returnvalue (Actor|GetActorOfClass "/Game/Blueprints/HexGrid/HexGrid.HexGrid_C"))
        (Default|UnhighlightAllTiles _returnvalue)
        (CallFunction|DoneUsingCard)))))

(fn DoneUsingCard
  (bind _assettlers_game_mode (Utilities|Casting|CastToSettlers_GameMode (Game|GetGameMode)))
  (Variables|/Game/Settlers_GameMode.Settlers_GameMode_C|Setphase _assettlers_game_mode 1)
  (CallFunction|RemoveCardfromPlayer (Variables|Temp|GetcurrentlyUsedCard))
  (bind _assettlers_game_instance (Utilities|Casting|CastToSettlersGameInstance (Game|GetGameInstance)))
  (if (Variables|/Game/Blueprints/SettlersGameInstance.SettlersGameInstance_C|GetisPassAndPlay _assettlers_game_instance)
    (bind _aspc_player (Utilities|Casting|CastToPC_Player (Game|GetPlayerController 0)))
    (bind _gamelog (Variables|/Game/Blueprints/Player/PC_Player.PC_Player_C|GetgameLog _aspc_player)
      (:then
        (Default|AddMessage _gamelog (Utilities|Text|ToText(String) (Utilities|String|Append (.name (Utilities|Struct|BreakBP_PlayerStruct (Utilities|Array|Get(acopy) (Variables|/Game/Settlers_GameMode.Settlers_GameMode_C|Getplayers _assettlers_game_mode) (Variables|/Game/Settlers_GameMode.Settlers_GameMode_C|GetcurrentPlayerIndex _assettlers_game_mode)))) (Utilities|String|MakeLiteralString " has played the ") (Utilities|String|EnumtoString (Variables|Temp|GetcurrentlyUsedCard)) (Utilities|String|MakeLiteralString " card.")))))
      (:else))
    (else
      (Default|EveryoneLogMessage _assettlers_game_mode (Utilities|Text|ToText(String) (Utilities|String|Append (.name (Utilities|Struct|BreakBP_PlayerStruct (Utilities|Array|Get(acopy) (Variables|/Game/Settlers_GameMode.Settlers_GameMode_C|Getplayers _assettlers_game_mode) (Variables|/Game/Settlers_GameMode.Settlers_GameMode_C|GetcurrentPlayerIndex _assettlers_game_mode)))) (Utilities|String|MakeLiteralString " has played the ") (Utilities|String|EnumtoString (Variables|Temp|GetcurrentlyUsedCard)) (Utilities|String|MakeLiteralString " card."))))))
  ;[1 1 1] reset variable to none
  (Variables|DCardHandler_C|SetcurrentlyUsedCard (Variables|/Game/Settlers_GameMode.Settlers_GameMode_C|GetdcardHandler _assettlers_game_mode) "NewEnumerator13")
  ;[1 0.1868 0.1868] TODO: needs to be different for MP?
  (bind _aspc_player_2 (Utilities|Casting|CastToPC_Player (Game|GetPlayerController 0)))
  (Default|ShowActionPanel _aspc_player_2))

(fn RemoveModalView
  (bind _aspc_player (Utilities|Casting|CastToPC_Player (Game|GetPlayerController 0)))
  (bind _dcardmodal (Variables|/Game/Blueprints/Player/PC_Player.PC_Player_C|GetdCardModal _aspc_player)
    (:then
      (Widget|RemovefromParent _dcardmodal))
    (:else)))

(fn UpdateTempBounties
  (params (playerIndex :type Integer))
  (bind _tileswithtempbountyupgrade (Variables|Temp|GettilesWithTempBountyUpgrade))
  (bind _keys (Utilities|Map|Keys _tileswithtempbountyupgrade))
  (for _array_element _keys
    ;[1 1 1] only update round count if it's the turn of the player who upgraded the bounty
    (if (== (.Value (Utilities|Map|Find _tileswithtempbountyupgrade _array_element)) playerIndex)
      ;[1 1 1] if bounty upgrade round count reached, restore bounty to original number
      (if (>= (Variables|/Game/Blueprints/HexGrid/HexTile.HexTile_C|GetbountyUpgradeRoundCount _array_element) 3)
        (Variables|/Game/Blueprints/HexGrid/HexTile.HexTile_C|Setbounty _array_element (- (Variables|/Game/Blueprints/HexGrid/HexTile.HexTile_C|Getbounty _array_element) 1))
        (Default|UpdateOwnerBountyText _array_element)
        (Utilities|Map|Remove (Variables|Temp|GettilesWithTempBountyUpgrade) _array_element)
        ;[1 1 1] inform players that fertilizer upgrade has expired
        (bind _assettlers_game_mode (Utilities|Casting|CastToSettlers_GameMode (Game|GetGameMode)))
        (bind _assettlers_game_instance (Utilities|Casting|CastToSettlersGameInstance (Game|GetGameInstance)))
        (if (Variables|/Game/Blueprints/SettlersGameInstance.SettlersGameInstance_C|GetisPassAndPlay _assettlers_game_instance)
          (bind _aspc_player (Utilities|Casting|CastToPC_Player (Game|GetPlayerController 0)))
          (bind _gamelog (Variables|/Game/Blueprints/Player/PC_Player.PC_Player_C|GetgameLog _aspc_player)
            (:then
              (Default|AddMessage _gamelog (Utilities|Text|ToText(String) (Utilities|String|Append (.name (Utilities|Struct|BreakBP_PlayerStruct (Utilities|Array|Get(acopy) (Variables|/Game/Settlers_GameMode.Settlers_GameMode_C|Getplayers _assettlers_game_mode) (Variables|/Game/Settlers_GameMode.Settlers_GameMode_C|GetcurrentPlayerIndex _assettlers_game_mode)))) (Utilities|String|MakeLiteralString "'s Fertilizer upgrade has expired.")))))
            (:else))
          (else
            (Default|EveryoneLogMessage _assettlers_game_mode (Utilities|Text|ToText(String) (Utilities|String|Append (.name (Utilities|Struct|BreakBP_PlayerStruct (Utilities|Array|Get(acopy) (Variables|/Game/Settlers_GameMode.Settlers_GameMode_C|Getplayers _assettlers_game_mode) (Variables|/Game/Settlers_GameMode.Settlers_GameMode_C|GetcurrentPlayerIndex _assettlers_game_mode)))) (Utilities|String|MakeLiteralString "'s Fertilizer upgrade has expired."))))))
        (else
          ;[1 1 1] otherwise, increment round count
          (Variables|/Game/Blueprints/HexGrid/HexTile.HexTile_C|SetbountyUpgradeRoundCount _array_element (+ (Variables|/Game/Blueprints/HexGrid/HexTile.HexTile_C|GetbountyUpgradeRoundCount _array_element) 1)))))))

(fn CheckValidityforTileCards
  (params (cardType :type DCards_Enum%20Enum :default "NewEnumerator0"))
  (switch Utilities|FlowControl|Switch|SwitchonDCards_Enum cardType
    (:NewEnumerator0
      _)
    (:NewEnumerator1
      _)
    (:NewEnumerator5
      (bind _returnvalue (Actor|GetActorOfClass "/Game/Blueprints/HexGrid/HexGrid.HexGrid_C" :!label _label))
      (if (> (Variables|/Game/Blueprints/HexGrid/HexGrid.HexGrid_C|GetnumTilesInfected _returnvalue) 1)
        (return true)
        (else
          (return false))))
    (:NewEnumerator9
      _)
    (:NewEnumerator11
      (goto _label)))
  (CallFunction|GetValidTilesforBounty cardType)
  (if (== (Utilities|Array|Length (Variables|Temp|GetvalidTilesToBeUsed)) 0)
    (return false)
    (else
      (return true))))

(fn GetValidTilesforBounty
  (params (cardType :type DCards_Enum%20Enum :default "NewEnumerator0"))
  (bind _validtilestobeused (Variables|Temp|GetvalidTilesToBeUsed))
  (Utilities|Array|Clear (Variables|Temp|GetvalidTilesToBeUsed))
  (bind _outactors (Actor|GetAllActorsOfClass "/Game/Blueprints/HexGrid/HexTile.HexTile_C"))
  (switch Utilities|FlowControl|Switch|SwitchonDCards_Enum cardType
    (:NewEnumerator0
      (for _array_element _outactors
        (if (> (Variables|/Game/Blueprints/HexGrid/HexTile.HexTile_C|Getbounty _array_element) 1)
          (Utilities|Array|Add _validtilestobeused _array_element))))
    (:NewEnumerator1
      (for _array_element_2 _outactors
        (if (< (Variables|/Game/Blueprints/HexGrid/HexTile.HexTile_C|Getbounty _array_element_2) 3)
          (Utilities|Array|Add _validtilestobeused _array_element_2))))
    (:NewEnumerator9
      (bind _keys (Utilities|Map|Keys (Variables|Temp|GettilesWithTempBountyUpgrade)))
      (for _array_element_3 _outactors
        (if (not (Utilities|Array|ContainsItem _keys _array_element_3))
          (Utilities|Array|Add (Variables|Temp|GetvalidTilesToBeUsed) _array_element_3))))))