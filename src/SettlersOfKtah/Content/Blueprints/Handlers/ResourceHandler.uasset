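; Handles the resource economy of a Settlers-style game: rolling, paying out, checking and changing player resources.
; Rolls use weighted probabilities that can be rebalanced against the selected result; zombie rolls trigger infection spreading instead of payouts.
; Outposts collect from adjacent uninfected matching tiles, earning full bounty unless another player owns the tile.
; Spinner completion updates UI, checks research victory and opens turn actions, branching between pass-and-play and multiplayer.
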(event EventBeginPlay
  (bind _assettlers_game_instance (Utilities|Casting|CastToSettlersGameInstance (Game|GetGameInstance)))
  (Variables|Default|Setresource_gameIsPP (Variables|/Game/Blueprints/SettlersGameInstance.SettlersGameInstance_C|GetisPassAndPlay _assettlers_game_instance)))

(fn ConstructionScript)

(fn SelectRandomResource
  (bind _resourceprobabilities (Variables|Default|GetresourceProbabilities))
  ;[1 1 1] First, reset temp vars.
  (Variables|Temp|SettempCurrentProb 0.0)
  (bind _output_get (Variables|Temp|SettempRandProb (Math|Random|RandomFloat)))
  ;[1 1 1] For each resource, check if the probability is a match
  (bind _keys (Utilities|Map|Keys _resourceprobabilities))
  (for _array_element _keys
    (Variables|Temp|SettempCurrentProb (+ (.Value (Utilities|Map|Find _resourceprobabilities _array_element)) (Variables|Temp|GettempCurrentProb)))
    ;[1 1 1] When we get a match, return the resource.
    (if (<= _output_get (Variables|Temp|GettempCurrentProb))
      (return _array_element))))

(fn UpdateResourcesUI
  (if (Variables|Default|Getresource_gameIsPP)
    ;[1 1 1] Loop through current player's resource amounts
    (bind _assettlers_game_mode (Utilities|Casting|CastToSettlers_GameMode (Game|GetGameMode)))
    (if (> (Utilities|Array|Length (Variables|/Game/Settlers_GameMode.Settlers_GameMode_C|Getplayers _assettlers_game_mode)) 0)
      (bind _aspc_player (Utilities|Casting|CastToPC_Player (Game|GetPlayerController 0)))
      (bind _resourcepanel (Variables|/Game/Blueprints/Player/PC_Player.PC_Player_C|GetresourcePanel _aspc_player)
        (:then
          (for _array_element (.numResourcesStructs (Utilities|Struct|BreakBP_PlayerStruct (Utilities|Array|Get(acopy) (Variables|/Game/Settlers_GameMode.Settlers_GameMode_C|Getplayers _assettlers_game_mode) (Variables|/Game/Settlers_GameMode.Settlers_GameMode_C|GetcurrentPlayerIndex _assettlers_game_mode))))
            ;[1 1 1] Update each text value of the resources UI panel accordingly
            (switch string (.resourceType (Utilities|Struct|BreakResourceStruct _array_element))
              (:wheat
                (Default|SetWheatAmount _resourcepanel (Utilities|String|ToString(Integer) (.count (Utilities|Struct|BreakResourceStruct _array_element)))))
              (:wood
                (Default|SetWoodAmount _resourcepanel (Utilities|String|ToString(Integer) (.count (Utilities|Struct|BreakResourceStruct _array_element)))))
              (:brick
                (Default|SetBrickAmount _resourcepanel (Utilities|String|ToString(Integer) (.count (Utilities|Struct|BreakResourceStruct _array_element)))))
              (:steel
                (Default|SetSteelAmount _resourcepanel (Utilities|String|ToString(Integer) (.count (Utilities|Struct|BreakResourceStruct _array_element))))))))
        (:else)))))

(fn CollectResources
  (params (resource :type String))
  (bind _assettlers_game_mode (Utilities|Casting|CastToSettlers_GameMode (Game|GetGameMode)))
  (if (Utilities|Enum|Equal(Enum) resource "zombie")
    (Default|AllowPlayerSpreadZombie (Variables|/Game/Settlers_GameMode.Settlers_GameMode_C|GetzombieHandler _assettlers_game_mode))
    (else
      (for (_array_element _array_index) (Variables|/Game/Settlers_GameMode.Settlers_GameMode_C|Getplayers _assettlers_game_mode)
        (Variables|Temp|SettempNumResourceToAdd 0)
        ;[1 1 1] check if player has an outpost adjacent to a tile with that resource
        (for _array_element_2 (.verticesWithOutposts (Utilities|Struct|BreakBP_PlayerStruct _array_element))
          (for _array_element_3 (Variables|/Game/Blueprints/HexGrid/HexVertex.HexVertex_C|GetadjacentHexagons _array_element_2)
            (if (Utilities|Array|ContainsItem (Variables|Temp|GettilesWithResourceRolled) _array_element_3)
              ;[1 1 1] add 1 or bounty based on whether player owns tile
              (if (or (== (Variables|/Game/Blueprints/HexGrid/HexTile.HexTile_C|GettileOwnerPlayerIndex _array_element_3) _array_index) (== (Variables|/Game/Blueprints/HexGrid/HexTile.HexTile_C|GettileOwnerPlayerIndex _array_element_3) -1))
                (Variables|Temp|SettempNumResourceToAdd (+ (Variables|Temp|GettempNumResourceToAdd) (Variables|/Game/Blueprints/HexGrid/HexTile.HexTile_C|Getbounty _array_element_3)))
                (else
                  (Variables|Temp|SettempNumResourceToAdd (+ (Variables|Temp|GettempNumResourceToAdd) 1))))))
          ;[1 1 1] handle apothecaries
          (bind _assettlers_game_mode_2 (Utilities|Casting|CastToSettlers_GameMode (Game|GetGameMode)))
          (Default|MaybeAddResearchPoint (Variables|/Game/Settlers_GameMode.Settlers_GameMode_C|GetplayerHandler _assettlers_game_mode_2) _array_element_2))
        ;[1 1 1] when done with that player, update their resources struct array and update players array
        (bind _outputstructarray (CallFunction|UpdateResourceStructsArray (.numResourcesStructs (Utilities|Struct|BreakBP_PlayerStruct _array_element)) (Variables|Temp|GettempNumResourceToAdd) resource))
        (bind _structout (Utilities|Struct|SetmembersinBP_PlayerStruct _array_element _outputstructarray))
        (Utilities|Array|SetArrayElem (Variables|/Game/Settlers_GameMode.Settlers_GameMode_C|Getplayers _assettlers_game_mode) _array_index _structout)))))

(fn CollectInitialResources
  (params (vertex :type Hex%20Vertex%20Object%20Reference))
  (bind _assettlers_game_mode (Utilities|Casting|CastToSettlers_GameMode (Game|GetGameMode)))
  (for _array_element (Variables|/Game/Blueprints/HexGrid/HexVertex.HexVertex_C|GetadjacentHexagons vertex)
    ;[1 1 1] add 1 or bounty based on whether player owns tile
    (if (or (== (Variables|/Game/Blueprints/HexGrid/HexTile.HexTile_C|GettileOwnerPlayerIndex _array_element) (Variables|/Game/Settlers_GameMode.Settlers_GameMode_C|GetcurrentPlayerIndex _assettlers_game_mode)) (== (Variables|/Game/Blueprints/HexGrid/HexTile.HexTile_C|GettileOwnerPlayerIndex _array_element) -1))
      (bind _outputstructarray (CallFunction|UpdateResourceStructsArray (.numResourcesStructs (Utilities|Struct|BreakBP_PlayerStruct (Utilities|Array|Get(acopy) (Variables|/Game/Settlers_GameMode.Settlers_GameMode_C|Getplayers _assettlers_game_mode) (Variables|/Game/Settlers_GameMode.Settlers_GameMode_C|GetcurrentPlayerIndex _assettlers_game_mode)))) (Variables|/Game/Blueprints/HexGrid/HexTile.HexTile_C|Getbounty _array_element) (Variables|/Game/Blueprints/HexGrid/HexTile.HexTile_C|GetresourceType _array_element)))
      (Utilities|Struct|SetmembersinBP_PlayerStruct (Utilities|Array|Get(acopy) (Variables|/Game/Settlers_GameMode.Settlers_GameMode_C|Getplayers _assettlers_game_mode) (Variables|/Game/Settlers_GameMode.Settlers_GameMode_C|GetcurrentPlayerIndex _assettlers_game_mode)) _outputstructarray)
      (else
        (bind _outputstructarray_2 (CallFunction|UpdateResourceStructsArray (.numResourcesStructs (Utilities|Struct|BreakBP_PlayerStruct (Utilities|Array|Get(acopy) (Variables|/Game/Settlers_GameMode.Settlers_GameMode_C|Getplayers _assettlers_game_mode) (Variables|/Game/Settlers_GameMode.Settlers_GameMode_C|GetcurrentPlayerIndex _assettlers_game_mode)))) 1 (Variables|/Game/Blueprints/HexGrid/HexTile.HexTile_C|GetresourceType _array_element)))
        (Utilities|Struct|SetmembersinBP_PlayerStruct (Utilities|Array|Get(acopy) (Variables|/Game/Settlers_GameMode.Settlers_GameMode_C|Getplayers _assettlers_game_mode) (Variables|/Game/Settlers_GameMode.Settlers_GameMode_C|GetcurrentPlayerIndex _assettlers_game_mode)) _outputstructarray_2))))
  (Utilities|Array|SetArrayElem (Variables|/Game/Settlers_GameMode.Settlers_GameMode_C|Getplayers _assettlers_game_mode) (Variables|/Game/Settlers_GameMode.Settlers_GameMode_C|GetcurrentPlayerIndex _assettlers_game_mode) (Utilities|Array|Get(acopy) (Variables|/Game/Settlers_GameMode.Settlers_GameMode_C|Getplayers _assettlers_game_mode) (Variables|/Game/Settlers_GameMode.Settlers_GameMode_C|GetcurrentPlayerIndex _assettlers_game_mode)))
  ;[1 1 1] if multiplayer, set the info struct for all players
  (if (not (Variables|Default|Getresource_gameIsPP))
    (Default|UpdateAllPlayersInfo _assettlers_game_mode)))

(fn PlayResourceSpinner
  (params (resource :type String))
  (Variables|Temp|SetlastResourceRolled resource)
  (if (Variables|Default|Getresource_gameIsPP)
    (bind _aspc_player (Utilities|Casting|CastToPC_Player (Game|GetPlayerController 0)))
    (bind _spinnerui (Variables|/Game/Blueprints/Player/PC_Player.PC_Player_C|GetspinnerUI _aspc_player)
      (:then
        (UserInterface|Viewport|AddtoViewport _spinnerui 0)
        (bind _spinnerplayer (Variables|/Game/Blueprints/Player/PC_Player.PC_Player_C|GetspinnerPlayer _aspc_player)
          (:then
            (switch string resource
              (:wheat
                (Media|MediaPlayer|OpenSource _spinnerplayer "/Game/Movies/SpinnerWheat.SpinnerWheat"))
              (:wood
                (Media|MediaPlayer|OpenSource _spinnerplayer "/Game/Movies/SpinnerWood.SpinnerWood"))
              (:brick
                (Media|MediaPlayer|OpenSource _spinnerplayer "/Game/Movies/SpinnerBrick.SpinnerBrick"))
              (:steel
                (Media|MediaPlayer|OpenSource _spinnerplayer "/Game/Movies/SpinnerSteel.SpinnerSteel"))
              (:zombie
                (Media|MediaPlayer|OpenSource _spinnerplayer "/Game/Movies/SpinnerZombie.SpinnerZombie"))))
          (:else)))
      (:else))
    (else
      (bind _assettlers_game_mode (Utilities|Casting|CastToSettlers_GameMode (Game|GetGameMode)))
      (for _array_element (Variables|/Game/Settlers_GameMode.Settlers_GameMode_C|GetallPlayerControllers _assettlers_game_mode)
        (bind _aspc_player_2 (Utilities|Casting|CastToPC_Player _array_element))
        (Default|CPlaySpinner _aspc_player_2 resource)))))

(fn CheckifPlayerHasEnoughResources
  (params (playerIndex :type Integer) (resourceStructsToCheck :type Array%20of%20Resource%20Struct%20Structures))
  (bind _assettlers_game_mode (Utilities|Casting|CastToSettlers_GameMode (Game|GetGameMode)))
  (for _array_element resourceStructsToCheck
    (for _array_element_2 (.numResourcesStructs (Utilities|Struct|BreakBP_PlayerStruct (Utilities|Array|Get(acopy) (Variables|/Game/Settlers_GameMode.Settlers_GameMode_C|Getplayers _assettlers_game_mode) playerIndex)))
      (if (Utilities|Enum|Equal(Enum) (.resourceType (Utilities|Struct|BreakResourceStruct _array_element)) (.resourceType (Utilities|Struct|BreakResourceStruct _array_element_2)))
        (if (not (<= (.count (Utilities|Struct|BreakResourceStruct _array_element)) (.count (Utilities|Struct|BreakResourceStruct _array_element_2))))
          (return false)))))
  (return true))

(fn RemoveResourcefromPlayer
  (params (playerIndex :type Integer) (resourceStructsToRemove :type Array%20of%20Resource%20Struct%20Structures))
  (bind _assettlers_game_mode (Utilities|Casting|CastToSettlers_GameMode (Game|GetGameMode)))
  (for _array_element resourceStructsToRemove
    (bind _result (Utilities|NegateInt (.count (Utilities|Struct|BreakResourceStruct _array_element)))
      (:%20%20
        (bind _outputstructarray (CallFunction|UpdateResourceStructsArray (.numResourcesStructs (Utilities|Struct|BreakBP_PlayerStruct (Utilities|Array|Get(acopy) (Variables|/Game/Settlers_GameMode.Settlers_GameMode_C|Getplayers _assettlers_game_mode) playerIndex))) _result (.resourceType (Utilities|Struct|BreakResourceStruct _array_element))))
        (Utilities|Struct|SetmembersinBP_PlayerStruct (Utilities|Array|Get(acopy) (Variables|/Game/Settlers_GameMode.Settlers_GameMode_C|Getplayers _assettlers_game_mode) playerIndex) _outputstructarray)
        (if (not (Variables|Default|Getresource_gameIsPP))
          (Default|UpdateAllPlayersInfo _assettlers_game_mode))))))

(fn AddResourcetoPlayer
  (params (playerIndex :type Integer) (resourceStructsToAdd :type Array%20of%20Resource%20Struct%20Structures))
  (bind _assettlers_game_mode (Utilities|Casting|CastToSettlers_GameMode (Game|GetGameMode)))
  (for _array_element resourceStructsToAdd
    (bind _outputstructarray (CallFunction|UpdateResourceStructsArray (.numResourcesStructs (Utilities|Struct|BreakBP_PlayerStruct (Utilities|Array|Get(acopy) (Variables|/Game/Settlers_GameMode.Settlers_GameMode_C|Getplayers _assettlers_game_mode) playerIndex))) (.count (Utilities|Struct|BreakResourceStruct _array_element)) (.resourceType (Utilities|Struct|BreakResourceStruct _array_element))))
    (Utilities|Struct|SetmembersinBP_PlayerStruct (Utilities|Array|Get(acopy) (Variables|/Game/Settlers_GameMode.Settlers_GameMode_C|Getplayers _assettlers_game_mode) playerIndex) _outputstructarray)))

(fn FindTileswithResourceWithoutInfection
  (params (resource :type String))
  (Utilities|Array|Clear (Variables|Temp|GettilesWithResourceRolled))
  (bind _outactors (Actor|GetAllActorsOfClass "/Game/Blueprints/HexGrid/HexTile.HexTile_C"))
  (for _array_element _outactors
    (if (and (Utilities|Enum|Equal(Enum) (Variables|/Game/Blueprints/HexGrid/HexTile.HexTile_C|GetresourceType _array_element) resource) (not (Variables|/Game/Blueprints/HexGrid/HexTile.HexTile_C|Getinfected _array_element)))
      (Utilities|Array|Add (Variables|Temp|GettilesWithResourceRolled) _array_element))))

(fn OnSpinnerComplete
  (params (triggeredByFirstClient :type Boolean))
  ;[1 1 1] add game log message for which resource is rolled
  (bind _assettlers_game_mode (Utilities|Casting|CastToSettlers_GameMode (Game|GetGameMode)))
  (if triggeredByFirstClient
    (bind _aspc_player (Utilities|Casting|CastToPC_Player (Game|GetPlayerController 0)))
    (bind _gamelog (Variables|/Game/Blueprints/Player/PC_Player.PC_Player_C|GetgameLog _aspc_player)
      (:then
        (bind _message (Default|AddResourceMessage _gamelog (Variables|Temp|GetlastResourceRolled)))
        (if (Variables|Default|Getresource_gameIsPP)
          _
          (else
            (Default|EveryoneLogMessage _assettlers_game_mode _message))))
      (:else)))
  ;[1 1 1] show player spread tiles if zombie rolled
  (if (Utilities|Enum|Equal(Enum) (Variables|Temp|GetlastResourceRolled) "Zombie")
    (Default|HighlightPlayerSpreadTiles (Variables|/Game/Settlers_GameMode.Settlers_GameMode_C|GetzombieHandler _assettlers_game_mode) true)
    (else
      ;[1 1 1] bounty animation if not zombie
      (for _array_element (Variables|Temp|GettilesWithResourceRolled)
        (if (Widget|IsVisible (Variables|/Game/Blueprints/HexGrid/HexTile.HexTile_C|GetbountyText _array_element))
          (UserInterface|Animation|PlayAnimation (Variables|/Game/Blueprints/HexGrid/HexTile.HexTile_C|GetbountyText _array_element) (Variables|/Game/Blueprints/UI/BountyText.BountyText_C|GetscaleAnimation (Variables|/Game/Blueprints/HexGrid/HexTile.HexTile_C|GetbountyText _array_element)) 0.0 1 "Forward" 1.0 false)))))
  ;[1 1 1] update resource UI and players' research points on player panel
  (CallFunction|UpdateResourcesUI)
  (if (Variables|Default|Getresource_gameIsPP)
    (bind _aspc_player_2 (Utilities|Casting|CastToPC_Player (Game|GetPlayerController 0)))
    (bind _playerpanel (Variables|/Game/Blueprints/Player/PC_Player.PC_Player_C|GetplayerPanel _aspc_player_2)
      (:then
        (Default|UpdateAllPlayersResearchPoints _playerpanel))
      (:else))
    (else
      (Default|UpdateAllPlayersInfo _assettlers_game_mode)))
  ;[1 1 1] check for research victory
  (Default|CheckforResearchVictory (Variables|/Game/Settlers_GameMode.Settlers_GameMode_C|GetplayerHandler _assettlers_game_mode))
  ;[1 1 1] if game isn't over, enable player actions
  (if (!= (Variables|/Game/Settlers_GameMode.Settlers_GameMode_C|Getphase _assettlers_game_mode) 7)
    (if (Variables|Default|Getresource_gameIsPP)
      (bind _aspc_player_3 (Utilities|Casting|CastToPC_Player (Game|GetPlayerController 0)))
      (Default|ShowActionPanel _aspc_player_3)
      (bind _resourcepanel (Variables|/Game/Blueprints/Player/PC_Player.PC_Player_C|GetresourcePanel _aspc_player_3)
        (:then
          (Widget|SetIsEnabled (Variables|/Game/Blueprints/UI/ResourcesPanel.ResourcesPanel_C|GetdevCardButton _resourcepanel) true)
          (Widget|SetIsEnabled (Variables|/Game/Blueprints/UI/ResourcesPanel.ResourcesPanel_C|GetshowBountyButton _resourcepanel) true))
        (:else))
      (elif triggeredByFirstClient
        (bind _assettlers_game_mode_2 (Utilities|Casting|CastToSettlers_GameMode (Game|GetGameMode)))
        (Default|EveryoneUpdateStartTurnWidgets _assettlers_game_mode_2)))))

(fn UpdateProbWeights
  (params (selected :type String))
  (bind _resourceprobabilities (Variables|Default|GetresourceProbabilities))
  ;[1 1 1] Check if each resource is the selected resource, and increase/decrease probability accordingly.
  (bind _keys (Utilities|Map|Keys _resourceprobabilities))
  (for _array_element _keys
    (if (Utilities|Enum|Equal(Enum) _array_element selected)
      (Utilities|Map|Add _resourceprobabilities _array_element (- (.Value (Utilities|Map|Find _resourceprobabilities _array_element)) 0.04))
      (else
        (Utilities|Map|Add _resourceprobabilities _array_element (+ (.Value (Utilities|Map|Find _resourceprobabilities _array_element)) 0.01))))))

(fn UpdateResourceStructsArray
  (params (inputStructArray :type Array%20of%20Resource%20Struct%20Structures) (numToAdd :type Integer) (resource :type String))
  (for (_array_element _array_index) inputStructArray
    (if (Utilities|Enum|Equal(Enum) resource (.resourceType (Utilities|Struct|BreakResourceStruct _array_element)))
      (Utilities|Array|SetArrayElem inputStructArray _array_index (Utilities|Struct|MakeResourceStruct resource (+ (.count (Utilities|Struct|BreakResourceStruct _array_element)) numToAdd)))
      (return inputStructArray))))