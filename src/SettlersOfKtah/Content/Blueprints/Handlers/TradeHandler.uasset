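; Handler actor that runs player-to-player and bank resource trades in a Settlers-style game by swapping trade widgets.
; An offer passes around the table via the game mode's CurrentPlayerIndex, skipping players as needed and recording each response until it returns to the offerer.
; The offerer then finalizes with one player, with give and take reversed for that side.
; Completed trades update the ResourceHandler and game log, then reset state.
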(event EventBeginPlay)

(event Collision|EventActorBeginOverlap
  (params (OtherActor :type Actor%20Object%20Reference)))

(event EventTick
  (params (DeltaSeconds :type Float%20%28single-precision%29)))

(fn ConstructionScript)

(fn InitializeMakeOffer
  (Widget|RemovefromParent (Variables|Default|GettradePanel))
  (bind _returnvalue (UserInterface|CreateWidget "/Game/Blueprints/UI/Trade/Trade_MakeOffer.Trade_MakeOffer_C"))
  (UserInterface|Viewport|AddtoViewport _returnvalue 0)
  (Variables|Default|SetmakeOfferUI _returnvalue)
  (CallFunction|GetOfferingPlayer))

(fn CompleteMakeOffer
  (bind _makeofferui (Variables|Default|GetmakeOfferUI))
  ;[1 1 1] grab offer numbers
  (CallFunction|GetTradeNumbers (Variables|/Game/Blueprints/UI/Trade/Trade_MakeOffer.Trade_MakeOffer_C|GetpickedResources _makeofferui))
  ;[1 1 1] remove make offer UI, move to next player, show receive offer UI
  (Widget|RemovefromParent _makeofferui)
  (CallFunction|MovetoNextPlayerinTradePhase)
  (CallFunction|InitializeReceiveOffer)
  ;[1 1 1] add to game log
  (CallFunction|AddTradeMessagestoLog (Utilities|String|Append (Variables|Default|GetofferingPlayerNameString) " has initiated a trade offer!")))

(fn InitializeReceiveOffer
  (bind _returnvalue (UserInterface|CreateWidget "/Game/Blueprints/UI/Trade/Trade_ReceiveOffer.Trade_ReceiveOffer_C"))
  (Utilities|FlowControl|Sequence
    (:then_0
      ;[1 1 1] give and take are swapped!
      (Variables|/Game/Blueprints/UI/Trade/Trade_ReceiveOffer.Trade_ReceiveOffer_C|SetgiveNumbers _returnvalue (Variables|Default|GetofferingPlayerTake))
      (Variables|/Game/Blueprints/UI/Trade/Trade_ReceiveOffer.Trade_ReceiveOffer_C|SettakeNumbers _returnvalue (Variables|Default|GetofferingPlayerGive))
      (bind _assettlers_game_mode (Utilities|Casting|CastToSettlers_GameMode (Game|GetGameMode)))
      (Rendering|Components|TextRender|SetText (Variables|/Game/Blueprints/UI/Trade/Trade_ReceiveOffer.Trade_ReceiveOffer_C|GetofferingPlayerName _returnvalue) (Utilities|Text|ToText(String) (Variables|Default|GetofferingPlayerNameString)))
      (Rendering|Components|TextRender|SetText (Variables|/Game/Blueprints/UI/Trade/Trade_ReceiveOffer.Trade_ReceiveOffer_C|GetofferedPlayerName _returnvalue) (Utilities|Text|ToText(String) (.name (Utilities|Struct|BreakBP_PlayerStruct (Utilities|Array|Get(acopy) (Variables|/Game/Settlers_GameMode.Settlers_GameMode_C|Getplayers _assettlers_game_mode) (Variables|/Game/Settlers_GameMode.Settlers_GameMode_C|GetcurrentPlayerIndex _assettlers_game_mode)))))))
    (:then_1
      (UserInterface|Viewport|AddtoViewport _returnvalue 0)
      (Variables|Default|SetreceiveOfferUI _returnvalue))))

(fn CompleteReceiveOffer
  (params (acceptedOffer :type Boolean))
  ;[1 1 1] record whether player accepted offer
  (Utilities|Map|Add (Variables|Default|GetoffersAccepted) (Variables|/Game/Blueprints/UI/Trade/Trade_ReceiveOffer.Trade_ReceiveOffer_C|GetreceivingPlayerIndex (Variables|Default|GetreceiveOfferUI)) acceptedOffer)
  (Widget|RemovefromParent (Variables|Default|GetreceiveOfferUI))
  (bind _assettlers_game_mode (Utilities|Casting|CastToSettlers_GameMode (Game|GetGameMode)))
  ;[1 1 1] move to next player, either intialize receive offer UI (if not yet back to original player) or initialize finalize offer UI
  (CallFunction|MovetoNextPlayerinTradePhase)
  (if (== (Variables|/Game/Settlers_GameMode.Settlers_GameMode_C|GetcurrentPlayerIndex _assettlers_game_mode) (Variables|Default|GetofferingPlayerIndex))
    (CallFunction|InitializeFinalizeOffer)
    (else
      (CallFunction|InitializeReceiveOffer))))

(fn InitializeFinalizeOffer
  (bind _returnvalue (UserInterface|CreateWidget "/Game/Blueprints/UI/Trade/Trade_FinalizeOffer.Trade_FinalizeOffer_C"))
  (Variables|/Game/Blueprints/UI/Trade/Trade_FinalizeOffer.Trade_FinalizeOffer_C|SettakeNumbers _returnvalue (Variables|Default|GetofferingPlayerTake))
  (Variables|/Game/Blueprints/UI/Trade/Trade_FinalizeOffer.Trade_FinalizeOffer_C|SetgiveNumbers _returnvalue (Variables|Default|GetofferingPlayerGive))
  (Variables|/Game/Blueprints/UI/Trade/Trade_FinalizeOffer.Trade_FinalizeOffer_C|SetplayerResponses _returnvalue (Variables|Default|GetoffersAccepted))
  (UserInterface|Viewport|AddtoViewport _returnvalue 0)
  (Variables|Default|SetfinalizeOfferUI _returnvalue))

(fn CompleteFinalizeOffer
  (params (tradingPlayerIndex :type Integer))
  (bind _offeringplayerindex (Variables|Default|GetofferingPlayerIndex))
  (bind _offeringplayertake (Variables|Default|GetofferingPlayerTake))
  (bind _offeringplayergive (Variables|Default|GetofferingPlayerGive))
  (bind _assettlers_game_mode (Utilities|Casting|CastToSettlers_GameMode (Game|GetGameMode)))
  (Utilities|FlowControl|Sequence
    (:then_0
      (Default|AddResourcetoPlayer (Variables|/Game/Settlers_GameMode.Settlers_GameMode_C|GetresourceHandler _assettlers_game_mode) _offeringplayertake _offeringplayerindex)
      (Default|RemoveResourcefromPlayer (Variables|/Game/Settlers_GameMode.Settlers_GameMode_C|GetresourceHandler _assettlers_game_mode) _offeringplayergive _offeringplayerindex))
    (:then_1
      (Default|RemoveResourcefromPlayer (Variables|/Game/Settlers_GameMode.Settlers_GameMode_C|GetresourceHandler _assettlers_game_mode) _offeringplayertake tradingPlayerIndex)
      (Default|AddResourcetoPlayer (Variables|/Game/Settlers_GameMode.Settlers_GameMode_C|GetresourceHandler _assettlers_game_mode) _offeringplayergive tradingPlayerIndex))
    (:then_2
      (Default|UpdateResourcesUI (Variables|/Game/Settlers_GameMode.Settlers_GameMode_C|GetresourceHandler _assettlers_game_mode))
      (CallFunction|AddTradeMessagestoLog (Utilities|String|Append (Variables|Default|GetofferingPlayerNameString) " has completed a trade with " (.name (Utilities|Struct|BreakBP_PlayerStruct (Utilities|Array|Get(acopy) (Variables|/Game/Settlers_GameMode.Settlers_GameMode_C|Getplayers _assettlers_game_mode) tradingPlayerIndex))) "!"))
      (CallFunction|CompleteTrade))))

(fn CompleteTrade
  ;[1 1 1] reset all trade variables, remove trade UI and show trade panel
  (CallFunction|ResetVariables)
  (Widget|RemovefromParent (Variables|Default|GetfinalizeOfferUI))
  (CallFunction|ShowTradePanel))

(fn MovetoNextPlayerinTradePhase
  (bind _assettlers_game_mode (Utilities|Casting|CastToSettlers_GameMode (Game|GetGameMode)))
  (Default|UnhighlightPlayer (Variables|/Game/Blueprints/Handlers/PlayerHandler.PlayerHandler_C|GetplayerUI (Variables|/Game/Settlers_GameMode.Settlers_GameMode_C|GetplayerHandler _assettlers_game_mode)) (Variables|/Game/Settlers_GameMode.Settlers_GameMode_C|GetcurrentPlayerIndex _assettlers_game_mode))
  ;[1 1 1] reset player index to 0 if we're at last player
  (if (== (Variables|/Game/Settlers_GameMode.Settlers_GameMode_C|GetcurrentPlayerIndex _assettlers_game_mode) (- (Utilities|Array|Length (Variables|/Game/Settlers_GameMode.Settlers_GameMode_C|Getplayers _assettlers_game_mode)) 1)) :!label _label
    (Variables|/Game/Settlers_GameMode.Settlers_GameMode_C|SetcurrentPlayerIndex _assettlers_game_mode 0)
    (else
      ;[1 1 1] otherwise, increment index
      (Variables|/Game/Settlers_GameMode.Settlers_GameMode_C|SetcurrentPlayerIndex _assettlers_game_mode (+ (Variables|/Game/Settlers_GameMode.Settlers_GameMode_C|GetcurrentPlayerIndex _assettlers_game_mode) 1))))
  ;[1 1 1] if need to skip player, go back to setting player index
  (bind _shouldskipplayer (Default|MaybeSkipPlayer _assettlers_game_mode))
  (if _shouldskipplayer
    (goto _label)
    (else
      (Default|HighlightPlayer (Variables|/Game/Blueprints/Handlers/PlayerHandler.PlayerHandler_C|GetplayerUI (Variables|/Game/Settlers_GameMode.Settlers_GameMode_C|GetplayerHandler _assettlers_game_mode)) (Variables|/Game/Settlers_GameMode.Settlers_GameMode_C|GetcurrentPlayerIndex _assettlers_game_mode))
      (Default|UpdateResourcesUI (Variables|/Game/Settlers_GameMode.Settlers_GameMode_C|GetresourceHandler _assettlers_game_mode)))))

(fn ResetVariables
  (Utilities|Map|Clear (Variables|Default|GetofferingPlayerTake))
  (Utilities|Map|Clear (Variables|Default|GetofferingPlayerGive))
  (Utilities|Map|Clear (Variables|Default|GetoffersAccepted))
  (Variables|Default|SetofferingPlayerIndex -1)
  (Variables|Default|SetofferingPlayerNameString ""))

(fn AddTradeMessagestoLog
  (params (message :type String))
  (bind _assettlers_game_mode (Utilities|Casting|CastToSettlers_GameMode (Game|GetGameMode)))
  (Default|AddMessage (Variables|/Game/Settlers_GameMode.Settlers_GameMode_C|GetgameLog _assettlers_game_mode) (Utilities|Text|ToText(String) message)))

(fn InitializeBankTrade
  (Widget|RemovefromParent (Variables|Default|GettradePanel))
  (bind _returnvalue (UserInterface|CreateWidget "/Game/Blueprints/UI/Trade/Trade_BankTrade.Trade_BankTrade_C"))
  (Variables|Default|SetbankTradeUI _returnvalue)
  (UserInterface|Viewport|AddtoViewport _returnvalue 0)
  (CallFunction|GetOfferingPlayer))

(fn CompleteBankTrade
  (params (canceled :type Boolean))
  (if canceled
    _
    (else
      (bind _assettlers_game_mode (Utilities|Casting|CastToSettlers_GameMode (Game|GetGameMode)))
      (Default|AddResourcetoPlayer (Variables|/Game/Settlers_GameMode.Settlers_GameMode_C|GetresourceHandler _assettlers_game_mode) (Variables|Default|GetofferingPlayerTake) (Variables|/Game/Settlers_GameMode.Settlers_GameMode_C|GetcurrentPlayerIndex _assettlers_game_mode))
      (Default|RemoveResourcefromPlayer (Variables|/Game/Settlers_GameMode.Settlers_GameMode_C|GetresourceHandler _assettlers_game_mode) (Variables|Default|GetofferingPlayerGive) (Variables|/Game/Settlers_GameMode.Settlers_GameMode_C|GetcurrentPlayerIndex _assettlers_game_mode))
      (Default|UpdateResourcesUI (Variables|/Game/Settlers_GameMode.Settlers_GameMode_C|GetresourceHandler _assettlers_game_mode))
      (CallFunction|AddTradeMessagestoLog (Utilities|String|Append (Variables|Default|GetofferingPlayerNameString) " has completed a trade with the bank!"))))
  (Widget|RemovefromParent (Variables|Default|GetbankTradeUI))
  (CallFunction|ResetVariables)
  (CallFunction|ShowTradePanel))

(fn GetTradeNumbers
  (params (panels :type Trade%20Resource%20Panels%20Object%20Reference))
  (Utilities|FlowControl|Sequence
    (:then_0
      (for _array_element (Class|PanelWidget|GetAllChildren (Variables|/Game/Blueprints/UI/Trade/Trade_ResourcePanels.Trade_ResourcePanels_C|GetgiveResourcesPanel panels))
        (bind _astrade_resource_selector (Utilities|Casting|CastToTrade_ResourceSelector _array_element))
        (Utilities|Map|Add (Variables|Default|GetofferingPlayerGive) (Variables|/Game/Blueprints/UI/Trade/Trade_ResourceSelector.Trade_ResourceSelector_C|GetresourceType _astrade_resource_selector) (Math|Conversions|ToInteger(Byte) (Utilities|String|ToString(Text) (Class|TextBlock|GetText (Variables|/Game/Blueprints/UI/Trade/Trade_ResourceSelector.Trade_ResourceSelector_C|GetNumResource _astrade_resource_selector)))))))
    (:then_1
      (for _array_element_2 (Class|PanelWidget|GetAllChildren (Variables|/Game/Blueprints/UI/Trade/Trade_ResourcePanels.Trade_ResourcePanels_C|GettakeResourcesPanel panels))
        (bind _astrade_resource_selector_2 (Utilities|Casting|CastToTrade_ResourceSelector _array_element_2))
        (Utilities|Map|Add (Variables|Default|GetofferingPlayerTake) (Variables|/Game/Blueprints/UI/Trade/Trade_ResourceSelector.Trade_ResourceSelector_C|GetresourceType _astrade_resource_selector_2) (Math|Conversions|ToInteger(Byte) (Utilities|String|ToString(Text) (Class|TextBlock|GetText (Variables|/Game/Blueprints/UI/Trade/Trade_ResourceSelector.Trade_ResourceSelector_C|GetNumResource _astrade_resource_selector_2)))))))))

(fn ShowTradePanel
  (bind _returnvalue (UserInterface|CreateWidget "/Game/Blueprints/UI/Trade/TradePanel.TradePanel_C"))
  (UserInterface|Viewport|AddtoViewport _returnvalue 0)
  (Variables|Default|SettradePanel _returnvalue))

(fn HideTradePanel
  (Widget|RemovefromParent (Variables|Default|GettradePanel))
  (bind _assettlers_game_mode (Utilities|Casting|CastToSettlers_GameMode (Game|GetGameMode)))
  (Default|ShowActionPanel _assettlers_game_mode))

(fn GetOfferingPlayer
  (bind _assettlers_game_mode (Utilities|Casting|CastToSettlers_GameMode (Game|GetGameMode)))
  (bind _output_get (Variables|Default|SetofferingPlayerIndex (Variables|/Game/Settlers_GameMode.Settlers_GameMode_C|GetcurrentPlayerIndex _assettlers_game_mode)))
  (Variables|Default|SetofferingPlayerNameString (.name (Utilities|Struct|BreakBP_PlayerStruct (Utilities|Array|Get(acopy) (Variables|/Game/Settlers_GameMode.Settlers_GameMode_C|Getplayers _assettlers_game_mode) _output_get)))))