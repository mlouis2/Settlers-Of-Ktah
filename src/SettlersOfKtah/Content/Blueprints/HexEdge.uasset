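; HexEdge is an edge actor on a hexagon board that lets the player place a road on it.
; Clicking its Cylinder calls MaybeSpawnRoad, currently a stub that always returns true, then spawns a Road at the edge's transform and stores the reference.
; Hover logic to swap materials on adjacent hexagons and vertices and toggle vertex visibility exists but is disconnected from the cursor events.
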(event OnClicked(Cylinder)
  (params (TouchedComponent :type Primitive%20Component%20Object%20Reference) (ButtonPressed :type Key%20Structure :default "None"))
  (bind _shouldspawnroad (CallFunction|MaybeSpawnRoad))
  (if _shouldspawnroad
    (bind _returnvalue (Game|SpawnActorfromClass "/Game/Blueprints/Road.Road_C" (Transformation|GetActorTransform self) "Undefined" 0 0))
    (Variables|Default|Setroad _returnvalue)))

(event EventBeginPlay)

(event Collision|EventActorBeginOverlap
  (params (OtherActor :type Actor%20Object%20Reference)))

(event EventTick
  (params (DeltaSeconds :type Float%20%28single-precision%29)))

(event MouseInput|EventActorBeginCursorOver
  ;[1 1 1] Highlight adjacent hexagons and vertices when mouse over
)

(event MouseInput|EventActorEndCursorOver
  ;[1 1 1] Highlight adjacent hexagons and vertices when mouse over
)

(fn ConstructionScript)

(fn MaybeSpawnRoad
  (return true))