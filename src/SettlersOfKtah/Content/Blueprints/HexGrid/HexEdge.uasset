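; HexEdge is a clickable edge on the Settlers hex grid where the current player builds roads and upgrades them to barricades.
; Clicking validates the game phase or active development card, plus adjacency to the player's outposts or roads, or road ownership for barricades.
; Building spawns a player-colored Road or Barricade, updates player data, UI, log and card progress.
; Valid edges are highlighted by unhiding HexEdge actors, tracked through a HexGrid flag.
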(event OnClicked(Cylinder)
  (params (TouchedComponent :type Primitive%20Component%20Object%20Reference) (ButtonPressed :type Key%20Structure))
  (bind _isvalid (CallFunction|CheckifRoadSpawnIsValid))
  (if _isvalid
    (CallFunction|SpawnRoadifValid)
    (else
      (bind _barricadeisvalid (CallFunction|CheckifBarricadeSpawnIsValid))
      (if _barricadeisvalid
        (CallFunction|UpgradeRoadtoBarricade)))))

(event EventBeginPlay
  ;[1 1 1] Placeholder for showing highlighting edges that are available for placement
)

(event Collision|EventActorBeginOverlap
  (params (OtherActor :type Actor%20Object%20Reference)))

(event EventTick
  (params (DeltaSeconds :type Float%20%28single-precision%29)))

(event MouseInput|EventActorBeginCursorOver
  ;[1 1 1] Highlight adjacent hexagons and vertices when mouse over
)

(event MouseInput|EventActorEndCursorOver
  ;[1 1 1] Highlight adjacent hexagons and vertices when mouse over
)

(fn ConstructionScript)

(fn CheckifRoadSpawnIsValid
  ;[1 1 1] check if we're in road placement phase
  (bind _assettlers_game_mode (Utilities|Casting|CastToSettlers_GameMode (Game|GetGameMode)))
  (if (== (Variables|/Game/Settlers_GameMode.Settlers_GameMode_C|Getphase _assettlers_game_mode) 4)
    (bind _isvalid (CallFunction|CheckifValidBuildLocation))
    (return _isvalid)
    (else
      ;[1 1 1] If we're not in road placement phase, could be a D-card.
      (if (and (Utilities|Enum|Equal(Enum) (Variables|/Game/Blueprints/Handlers/DCardHandler.DCardHandler_C|GetcurrentlyUsedCard (Variables|/Game/Settlers_GameMode.Settlers_GameMode_C|GetdcardHandler _assettlers_game_mode)) "NewEnumerator3") (< (Variables|/Game/Blueprints/Handlers/DCardHandler.DCardHandler_C|GetinfrastructureProgress (Variables|/Game/Settlers_GameMode.Settlers_GameMode_C|GetdcardHandler _assettlers_game_mode)) 2))
        (bind _isvalid_2 (CallFunction|CheckifValidBuildLocation))
        (return _isvalid_2)
        (else
          (return false))))))

(fn SpawnRoadifValid
  (bind _self self)
  (bind _returnvalue (Game|SpawnActorfromClass "/Game/Blueprints/AssetBPs/Road.Road_C" (Transformation|GetActorTransform self) "Undefined" 0 0))
  (Variables|Default|Setroad _returnvalue)
  (CallFunction|SetRoadorBarricadeColor false)
  (bind _assettlers_game_mode (Utilities|Casting|CastToSettlers_GameMode (Game|GetGameMode)))
  (Utilities|Array|Add (.edgesWithRoads (Utilities|Struct|BreakBP_PlayerStruct (Utilities|Array|Get(acopy) (Variables|/Game/Settlers_GameMode.Settlers_GameMode_C|Getplayers _assettlers_game_mode) (Variables|/Game/Settlers_GameMode.Settlers_GameMode_C|GetcurrentPlayerIndex _assettlers_game_mode)))) _self)
  (CallFunction|UnhighlightRoads _self)
  (bind _assettlers_game_mode_2 (Utilities|Casting|CastToSettlers_GameMode (Game|GetGameMode)))
  (Default|HandleRoadBuilt (Variables|/Game/Settlers_GameMode.Settlers_GameMode_C|GetbuildUI _assettlers_game_mode_2))
  (Default|AddBuiltMessage (Variables|/Game/Settlers_GameMode.Settlers_GameMode_C|GetgameLog _assettlers_game_mode_2) "Road" (Variables|/Game/Settlers_GameMode.Settlers_GameMode_C|GetcurrentPlayerIndex _assettlers_game_mode))
  ;[1 1 1] If it was from a D-Card, need to update Infrastructure.
  (if (== (Variables|/Game/Settlers_GameMode.Settlers_GameMode_C|Getphase _assettlers_game_mode_2) 11)
    (bind _output_get (Variables|/Game/Blueprints/Handlers/DCardHandler.DCardHandler_C|SetinfrastructureProgress (Variables|/Game/Settlers_GameMode.Settlers_GameMode_C|GetdcardHandler _assettlers_game_mode_2) (+ (Variables|/Game/Blueprints/Handlers/DCardHandler.DCardHandler_C|GetinfrastructureProgress (Variables|/Game/Settlers_GameMode.Settlers_GameMode_C|GetdcardHandler _assettlers_game_mode_2)) 1)))
    ;[1 1 1] If it's one, this is the first road we've placed -- highlight roads again. If it's two, highlight valid barricades instead.
    (if (== _output_get 1)
      (CallFunction|HighlightValidRoads)
      (elif (== _output_get 2)
        (CallFunction|HighlightValidBarricades)))))

(fn HighlightValidRoads
  (bind _outactors (Actor|GetAllActorsOfClass "HexEdge_C"))
  (for _array_element _outactors
    (bind _isvalid (CallFunction|CheckifValidBuildLocation _array_element))
    (if _isvalid
      (Rendering|SetActorHiddenInGame _array_element false)))
  (bind _returnvalue (Actor|GetActorOfClass "/Game/Blueprints/HexGrid/HexGrid.HexGrid_C"))
  (Variables|/Game/Blueprints/HexGrid/HexGrid.HexGrid_C|SetedgesHighlighted _returnvalue true))

(fn CheckifValidBuildLocation
  ;[1 1 1] if edge already has a road on it
  (if (Utilities|IsValid (Variables|Default|Getroad))
    (return false)
    (else
      (bind _assettlers_game_mode (Utilities|Casting|CastToSettlers_GameMode (Game|GetGameMode)))
      ;[1 1 1] check if edge is adjacent to a player's road or outpost
      (for _array_element (Variables|Default|GetadjacentVertices)
        (if (Utilities|Array|ContainsItem (.verticesWithOutposts (Utilities|Struct|BreakBP_PlayerStruct (Utilities|Array|Get(acopy) (Variables|/Game/Settlers_GameMode.Settlers_GameMode_C|Getplayers _assettlers_game_mode) (Variables|/Game/Settlers_GameMode.Settlers_GameMode_C|GetcurrentPlayerIndex _assettlers_game_mode)))) _array_element)
          (return true)
          (else
            (for _array_element_2 (Variables|/Game/Blueprints/HexGrid/HexVertex.HexVertex_C|GetadjacentEdges _array_element)
              (if (Utilities|Array|ContainsItem (.edgesWithRoads (Utilities|Struct|BreakBP_PlayerStruct (Utilities|Array|Get(acopy) (Variables|/Game/Settlers_GameMode.Settlers_GameMode_C|Getplayers _assettlers_game_mode) (Variables|/Game/Settlers_GameMode.Settlers_GameMode_C|GetcurrentPlayerIndex _assettlers_game_mode)))) _array_element_2)
                (return true))))))
      (return false))))

(fn UnhighlightRoads
  (bind _returnvalue (Actor|GetActorOfClass "/Game/Blueprints/HexGrid/HexGrid.HexGrid_C"))
  (if (Variables|/Game/Blueprints/HexGrid/HexGrid.HexGrid_C|GetedgesHighlighted _returnvalue)
    (bind _outactors (Actor|GetAllActorsOfClass "HexEdge_C"))
    (for _array_element _outactors
      (Rendering|SetActorHiddenInGame _array_element true))
    (Variables|/Game/Blueprints/HexGrid/HexGrid.HexGrid_C|SetedgesHighlighted _returnvalue false)))

(fn SetRoadorBarricadeColor
  (params (barricade :type Boolean))
  (bind _assettlers_game_mode (Utilities|Casting|CastToSettlers_GameMode (Game|GetGameMode)))
  (if barricade
    (bind _asbarricade (Utilities|Casting|CastToBarricade (Variables|Default|Getbarricade)))
    (switch string (Utilities|Array|Get(acopy) (Variables|/Game/Blueprints/Handlers/PlayerHandler.PlayerHandler_C|GetplayerColors (Variables|/Game/Settlers_GameMode.Settlers_GameMode_C|GetplayerHandler _assettlers_game_mode)) (Variables|/Game/Settlers_GameMode.Settlers_GameMode_C|GetcurrentPlayerIndex _assettlers_game_mode))
      (:Red
        (Rendering|Material|SetMaterial (Variables|/Game/Blueprints/AssetBPs/Barricade.Barricade_C|Getbarricade _asbarricade) 0 "/Game/Materials/roads/M_road_red.M_road_red"))
      (:Blue
        (Rendering|Material|SetMaterial (Variables|/Game/Blueprints/AssetBPs/Barricade.Barricade_C|Getbarricade _asbarricade) 0 "/Game/Materials/roads/M_road_blue.M_road_blue"))
      (:Pink
        (Rendering|Material|SetMaterial (Variables|/Game/Blueprints/AssetBPs/Barricade.Barricade_C|Getbarricade _asbarricade) 0 "/Game/Materials/roads/M_road_pink.M_road_pink"))
      (:Purple
        (Rendering|Material|SetMaterial (Variables|/Game/Blueprints/AssetBPs/Barricade.Barricade_C|Getbarricade _asbarricade) 0 "/Game/Materials/roads/M_road_purple.M_road_purple")))
    (else
      (bind _asroad (Utilities|Casting|CastToRoad (Variables|Default|Getroad)))
      (switch string (Utilities|Array|Get(acopy) (Variables|/Game/Blueprints/Handlers/PlayerHandler.PlayerHandler_C|GetplayerColors (Variables|/Game/Settlers_GameMode.Settlers_GameMode_C|GetplayerHandler _assettlers_game_mode)) (Variables|/Game/Settlers_GameMode.Settlers_GameMode_C|GetcurrentPlayerIndex _assettlers_game_mode))
        (:Default
          (Rendering|Material|SetMaterial (Variables|/Game/Blueprints/AssetBPs/Road.Road_C|GetCube _asroad) 0 "/Game/Materials/roads/M_road_purple.M_road_purple" :!label _label))
        (:red
          (Rendering|Material|SetMaterial (Variables|/Game/Blueprints/AssetBPs/Road.Road_C|GetCube _asroad) 0 "/Game/Materials/roads/M_road_red.M_road_red"))
        (:blue
          (Rendering|Material|SetMaterial (Variables|/Game/Blueprints/AssetBPs/Road.Road_C|GetCube _asroad) 0 "/Game/Materials/roads/M_road_blue.M_road_blue"))
        (:pink
          (Rendering|Material|SetMaterial (Variables|/Game/Blueprints/AssetBPs/Road.Road_C|GetCube _asroad) 0 "/Game/Materials/roads/M_road_pink.M_road_pink"))
        (:purple
          (goto _label))))))

(fn HighlightValidBarricades
  ;[1 1 1] First, highlight all of the current player's roads that aren't already barricades.
  (bind _assettlers_game_mode (Utilities|Casting|CastToSettlers_GameMode (Game|GetGameMode)))
  (for _array_element (.edgesWithRoads (Utilities|Struct|BreakBP_PlayerStruct (Utilities|Array|Get(acopy) (Variables|/Game/Settlers_GameMode.Settlers_GameMode_C|Getplayers _assettlers_game_mode) (Variables|/Game/Settlers_GameMode.Settlers_GameMode_C|GetcurrentPlayerIndex _assettlers_game_mode))))
    (if (not (Variables|HexEdge_C|GetisBarricade _array_element))
      (CallFunction|HighlightRoad _array_element)))
  ;[1 1 1] Then, mark some edges as highlighted.
  (bind _returnvalue (Actor|GetActorOfClass "/Game/Blueprints/HexGrid/HexGrid.HexGrid_C"))
  (Variables|/Game/Blueprints/HexGrid/HexGrid.HexGrid_C|SetedgesHighlighted _returnvalue true))

(fn HighlightRoad
  (Rendering|SetActorHiddenInGame false))

(fn CheckifBarricadeSpawnIsValid
  ;[1 1 1] First, we have to be in barricade upgrade phase OR be using the Fortify D-card.
  (bind _assettlers_game_mode (Utilities|Casting|CastToSettlers_GameMode (Game|GetGameMode)))
  (if (or (== (Variables|/Game/Settlers_GameMode.Settlers_GameMode_C|Getphase _assettlers_game_mode) 8) (and (== (Variables|/Game/Settlers_GameMode.Settlers_GameMode_C|Getphase _assettlers_game_mode) 11) (Utilities|Enum|Equal(Enum) (Variables|/Game/Blueprints/Handlers/DCardHandler.DCardHandler_C|GetcurrentlyUsedCard (Variables|/Game/Settlers_GameMode.Settlers_GameMode_C|GetdcardHandler _assettlers_game_mode)) "NewEnumerator7")))
    _
    (else
      ;[1 1 1] OR could be Infrastructure D-card.
      (if (and (Utilities|Enum|Equal(Enum) (Variables|/Game/Blueprints/Handlers/DCardHandler.DCardHandler_C|GetcurrentlyUsedCard (Variables|/Game/Settlers_GameMode.Settlers_GameMode_C|GetdcardHandler _assettlers_game_mode)) "NewEnumerator3") (== (Variables|/Game/Blueprints/Handlers/DCardHandler.DCardHandler_C|GetinfrastructureProgress (Variables|/Game/Settlers_GameMode.Settlers_GameMode_C|GetdcardHandler _assettlers_game_mode)) 2))
        _
        (else
          (return false)))))
  ;[1 1 1] And it has to be a valid road belonging to the player.
  (if (Utilities|IsValid (Variables|Default|Getroad))
    (return (Utilities|Array|ContainsItem (.edgesWithRoads (Utilities|Struct|BreakBP_PlayerStruct (Utilities|Array|Get(acopy) (Variables|/Game/Settlers_GameMode.Settlers_GameMode_C|Getplayers _assettlers_game_mode) (Variables|/Game/Settlers_GameMode.Settlers_GameMode_C|GetcurrentPlayerIndex _assettlers_game_mode)))) self))
    (else
      (return false))))

(fn UpgradeRoadtoBarricade
  ;[1 1 1] Set the edge to be a barricade
  (Variables|Default|SetisBarricade true)
  ;[1 1 1] Add barricade actor
  (bind _returnvalue (Game|SpawnActorfromClass "/Game/Blueprints/AssetBPs/Barricade.Barricade_C" (Transformation|GetActorTransform (Variables|Default|Getroad)) "Undefined" 0 0))
  (Variables|Default|Setbarricade _returnvalue)
  (CallFunction|SetRoadorBarricadeColor true)
  (Rendering|SetActorHiddenInGame (Variables|Default|Getroad) true)
  ;[1 1 1] Unhighlight roads, update buttons, indicate that barricade was built, return to turn phase
  (CallFunction|UnhighlightRoads)
  (bind _assettlers_game_mode (Utilities|Casting|CastToSettlers_GameMode (Game|GetGameMode)))
  (Default|UpdateButtons (Variables|/Game/Settlers_GameMode.Settlers_GameMode_C|GetbuildUI _assettlers_game_mode))
  (Default|PlayBuildSound (Variables|/Game/Settlers_GameMode.Settlers_GameMode_C|GetbuildUI _assettlers_game_mode))
  (Default|AddBarricadeMessage (Variables|/Game/Settlers_GameMode.Settlers_GameMode_C|GetgameLog _assettlers_game_mode) true)
  (if (== (Variables|/Game/Settlers_GameMode.Settlers_GameMode_C|Getphase _assettlers_game_mode) 11)
    (Variables|/Game/Blueprints/Handlers/DCardHandler.DCardHandler_C|SetinfrastructureProgress (Variables|/Game/Settlers_GameMode.Settlers_GameMode_C|GetdcardHandler _assettlers_game_mode) 0)
    (Default|DoneUsingCard (Variables|/Game/Settlers_GameMode.Settlers_GameMode_C|GetdcardHandler _assettlers_game_mode)))
  (Variables|/Game/Settlers_GameMode.Settlers_GameMode_C|Setphase _assettlers_game_mode 1))

(fn RemoveBarricade
  (Variables|Default|SetisBarricade false)
  (Variables|Default|SetbarricadeRoundCount 0)
  (Actor|DestroyActor (Variables|Default|Getbarricade))
  (Rendering|SetActorHiddenInGame (Variables|Default|Getroad) false))

(fn CheckifPossibleBarricadeLocation
  (bind _assettlers_game_mode (Utilities|Casting|CastToSettlers_GameMode (Game|GetGameMode)))
  (for _array_element (.edgesWithRoads (Utilities|Struct|BreakBP_PlayerStruct (Utilities|Array|Get(acopy) (Variables|/Game/Settlers_GameMode.Settlers_GameMode_C|Getplayers _assettlers_game_mode) (Variables|/Game/Settlers_GameMode.Settlers_GameMode_C|GetcurrentPlayerIndex _assettlers_game_mode))))
    (if (not (Variables|HexEdge_C|GetisBarricade _array_element))
      (return true)))
  (return false))