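; Hex board tile for a Settlers-style game with resource types, player castles, zombie infection and bounty text.
; During placement, hover previews a transparent castle in the current player's color and style, and a valid click builds it, then highlights outpost vertices.
; Other clicks route to the game mode's zombie or D-card handlers.
; Castle placement, infection and cure swap the tile's mesh by resource, with infection changes updating HexGrid's count.
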(event EventBeginPlay
  (bind _transform (CallFunction|CreateCastleTransform))
  (Variables|Default|SetcastleTransform _transform))

(event Collision|EventActorBeginOverlap
  (params (OtherActor :type Actor%20Object%20Reference)))

(event MouseInput|EventActorOnClicked
  (params (ButtonPressed :type Key%20Structure :default "None"))
  ;[1 1 1] onClick event
  (CallFunction|TileonClick))

(event MouseInput|EventActorEndCursorOver
  ;[1 1 1] if in placement phase, destroy half transparent actor when hover ends
  (CallFunction|TileonUnhover))

(event MouseInput|EventActorBeginCursorOver
  ;[1 1 1] if in placement phase and no castle already built, show half transparent castle on hover -- TODO: SET OPACITY
  (CallFunction|TileonHover))

(event EventTick
  (params (DeltaSeconds :type Float%20%28single-precision%29))
  (bind _bountytext (Variables|Default|GetbountyText))
  ;[1 1 1] if there's bounty, update position accordingly (kinda a hack with the first tick)
  (if (Utilities|IsValid _bountytext)
    (if true
      (Variables|Default|SetisFirstTick false)
      (Default|UpdateWidgetPosition _bountytext)
      (else
        (Default|MaybeUpdateWidgetPosition _bountytext)))))

(fn ConstructionScript)

(fn CheckifCastleSpawnIsValid
  ;[1 1 1] Check if there's already a castle or if tile is infected
  (if (Utilities|IsValid (Variables|Default|Getcastle))
    _
    (elif (Variables|Default|Getinfected)
      _
      (else
        ;[1 1 1] placement phase logic
        (bind _assettlers_game_mode (Utilities|Casting|CastToSettlers_GameMode (Game|GetGameMode)))
        (if (== (Variables|/Game/Settlers_GameMode.Settlers_GameMode_C|Getphase _assettlers_game_mode) 0)
          (if (== (Utilities|Array|Length (.castleTiles (Utilities|Struct|BreakBP_PlayerStruct (Utilities|Array|Get(acopy) (Variables|/Game/Settlers_GameMode.Settlers_GameMode_C|Getplayers _assettlers_game_mode) (Variables|/Game/Settlers_GameMode.Settlers_GameMode_C|GetcurrentPlayerIndex _assettlers_game_mode))))) 0)
            (return true)
            (elif (== (Utilities|Array|Length (.castleTiles (Utilities|Struct|BreakBP_PlayerStruct (Utilities|Array|Get(acopy) (Variables|/Game/Settlers_GameMode.Settlers_GameMode_C|Getplayers _assettlers_game_mode) (Variables|/Game/Settlers_GameMode.Settlers_GameMode_C|GetcurrentPlayerIndex _assettlers_game_mode))))) 1)
              (if (== (Utilities|Array|Length (.vertices (Utilities|Struct|BreakBP_PlayerStruct (Utilities|Array|Get(acopy) (Variables|/Game/Settlers_GameMode.Settlers_GameMode_C|Getplayers _assettlers_game_mode) (Variables|/Game/Settlers_GameMode.Settlers_GameMode_C|GetcurrentPlayerIndex _assettlers_game_mode))))) 1)
                (return true)
                (else
                  (return false)))
              (else
                (return (!= (Utilities|Array|Length (.castleTiles (Utilities|Struct|BreakBP_PlayerStruct (Utilities|Array|Get(acopy) (Variables|/Game/Settlers_GameMode.Settlers_GameMode_C|Getplayers _assettlers_game_mode) (Variables|/Game/Settlers_GameMode.Settlers_GameMode_C|GetcurrentPlayerIndex _assettlers_game_mode))))) 2)))))
          (else
            (return false))))))
  (return false))

(fn SpawnCastle
  (bind _returnvalue (Game|SpawnActorfromClass "/Game/Blueprints/AssetBPs/Castle.Castle_C" (Variables|Default|GetcastleTransform) "Undefined" 0 0))
  (bind _assettlers_game_mode (Utilities|Casting|CastToSettlers_GameMode (Game|GetGameMode)))
  (Utilities|FlowControl|Sequence
    (:then_0
      ;[1 1 1] Give castle to player and assign player to tile, also update castle color/rotation and update tile to full version
      (Utilities|Array|Add (.castleTiles (Utilities|Struct|BreakBP_PlayerStruct (Utilities|Array|Get(acopy) (Variables|/Game/Settlers_GameMode.Settlers_GameMode_C|Getplayers _assettlers_game_mode) (Variables|/Game/Settlers_GameMode.Settlers_GameMode_C|GetcurrentPlayerIndex _assettlers_game_mode)))) self)
      (bind _output_get (Variables|Default|Setcastle _returnvalue))
      (CallFunction|SetCastleColor _output_get false)
      (CallFunction|SetTiletoVersionforCastle)
      (Variables|Default|SettileOwnerPlayerIndex (Variables|/Game/Settlers_GameMode.Settlers_GameMode_C|GetcurrentPlayerIndex _assettlers_game_mode)))
    (:then_1
      ;[1 1 1] destroy temp transparent castle, don't spawn it anymore until outpost is placed
      (Actor|DestroyActor (Variables|Default|GettransparentCastle))
      (bind _returnvalue_2 (Actor|GetActorOfClass "/Game/Blueprints/HexGrid/HexGrid.HexGrid_C"))
      (Variables|/Game/Blueprints/HexGrid/HexGrid.HexGrid_C|SetspawnTransparentCastles _returnvalue_2 false))
    (:then_2
      ;[1 1 1] update bounty text on tile
      (CallFunction|UpdateBountywhenCastlePlaced))
    (:then_3
      (return true))))

(fn MaybeHighlightVertices
  (bind _assettlers_game_mode (Utilities|Casting|CastToSettlers_GameMode (Game|GetGameMode)))
  (if (== (Variables|/Game/Settlers_GameMode.Settlers_GameMode_C|Getphase _assettlers_game_mode) 0)
    (bind _values (Utilities|Map|Values (Variables|Default|Getvertices)))
    (bind _hasvalidlocation (Default|CheckifAnyValidOutpostLocation (Utilities|Array|Get(acopy) _values)))
    (if _hasvalidlocation
      (Default|HighlightValidVertices (Utilities|Array|Get(acopy) _values))
      (else
        (Default|HandleTurnPhase _assettlers_game_mode)))))

(fn SetCastleColor
  (params (castle :type Castle%20Object%20Reference%20%28by%20ref%29) (transparent :type Boolean))
  (bind _castle (Variables|/Game/Blueprints/AssetBPs/Castle.Castle_C|GetCastle castle))
  (if transparent
    (CallFunction|SetTempCastleColor)
    (else
      (Utilities|Casting|CastToSettlers_GameMode (Game|GetGameMode))
      (bind _output (CallFunction|GetPlayerColor))
      (bind _castlestyle (CallFunction|GetCastleStyle))
      (switch string _castlestyle
        (:Default
          (switch string _output :!label _label
            (:Default
              (Rendering|Material|SetMaterial _castle 0 "/Game/Materials/castles/M_castle_purple.M_castle_purple" :!label _label_2))
            (:red
              (Rendering|Material|SetMaterial _castle 0 "/Game/Materials/castles/M_castle_red.M_castle_red"))
            (:blue
              (Rendering|Material|SetMaterial _castle 0 "/Game/Materials/castles/M_castle_blue.M_castle_blue"))
            (:pink
              (Rendering|Material|SetMaterial _castle 0 "/Game/Materials/castles/M_castle_pink.M_castle_pink"))
            (:purple
              (goto _label_2))))
        (:fairy%20tale
          (goto _label))
        (:gothic
          (Components|StaticMesh|SetStaticMesh (Variables|/Game/Blueprints/AssetBPs/Castle.Castle_C|GetCastle (Variables|Default|Getcastle)) "/Game/Assets/gothic_castle_uv.gothic_castle_uv")
          (switch string _output
            (:Red
              (Rendering|Material|SetMaterial _castle 0 "/Game/Materials/castles/gothic_castle/M_gothic_castle_red.M_gothic_castle_red"))
            (:Blue
              (Rendering|Material|SetMaterial _castle 0 "/Game/Materials/castles/gothic_castle/M_gothic_castle_blue.M_gothic_castle_blue"))
            (:Pink
              (Rendering|Material|SetMaterial _castle 0 "/Game/Materials/castles/gothic_castle/M_gothic_castle_pink.M_gothic_castle_pink"))
            (:Purple
              (Rendering|Material|SetMaterial _castle 0 "/Game/Materials/castles/gothic_castle/M_gothic_castle_purple.M_gothic_castle_purple")))
          (bind _newtransform (CallFunction|UpdateGothicCastleTransform))
          (Transformation|SetActorTransform (Variables|Default|Getcastle) _newtransform))))))

(fn InfectTile
  (bind _resourcetype (Variables|Default|GetresourceType))
  (bind _hexagon_basic (Variables|Default|Gethexagon_basic))
  (if (not (Variables|Default|Getinfected))
    (Variables|Default|Setinfected true)
    (bind _returnvalue (Actor|GetActorOfClass "/Game/Blueprints/HexGrid/HexGrid.HexGrid_C"))
    (Variables|/Game/Blueprints/HexGrid/HexGrid.HexGrid_C|SetnumTilesInfected _returnvalue (+ (Variables|/Game/Blueprints/HexGrid/HexGrid.HexGrid_C|GetnumTilesInfected _returnvalue) 1))
    (if (Utilities|IsValid (Variables|Default|Getcastle))
      ;[1 1 1] zombified tile with castle (full)
      (switch string _resourcetype
        (:wood
          (Components|StaticMesh|SetStaticMesh _hexagon_basic "/Game/Assets/resources/wood_full_dead.wood_full_dead"))
        (:wheat
          (Components|StaticMesh|SetStaticMesh _hexagon_basic "/Game/Assets/resources/wheat_full_dead.wheat_full_dead"))
        (:brick
          (Components|StaticMesh|SetStaticMesh _hexagon_basic "/Game/Assets/resources/brick_tile_zombiefied01.brick_tile_zombiefied01"))
        (:steel
          (Components|StaticMesh|SetStaticMesh _hexagon_basic "/Game/Assets/resources/steel_tile_full_zombiefied.steel_tile_full_zombiefied")))
      (else
        (switch string _resourcetype
          (:brick
            (Components|StaticMesh|SetStaticMesh _hexagon_basic "/Game/Assets/resources/brick_tile_zombiefied01.brick_tile_zombiefied01"))
          (:wood
            (Components|StaticMesh|SetStaticMesh _hexagon_basic "/Game/Assets/resources/wood_dead.wood_dead"))
          (:wheat
            (Components|StaticMesh|SetStaticMesh _hexagon_basic "/Game/Assets/resources/wheat_dead.wheat_dead"))
          (:steel
            (Components|StaticMesh|SetStaticMesh _hexagon_basic "/Game/Assets/resources/steel_tile_empty_zombiefied.steel_tile_empty_zombiefied")))))))

(fn TileonClick
  (bind _isvalid (CallFunction|CheckifCastleSpawnIsValid))
  (if _isvalid
    (CallFunction|SpawnCastle)
    (CallFunction|MaybeHighlightVertices)
    (else
      (bind _assettlers_game_mode (Utilities|Casting|CastToSettlers_GameMode (Game|GetGameMode)))
      ;[1 1 1] if tile clicked during phase 11 and a dcard that is not outbreak is being used
      (if (== (Variables|/Game/Settlers_GameMode.Settlers_GameMode_C|Getphase _assettlers_game_mode) 11)
        (if (Utilities|Enum|Equal(Enum) (Variables|/Game/Blueprints/Handlers/DCardHandler.DCardHandler_C|GetcurrentlyUsedCard (Variables|/Game/Settlers_GameMode.Settlers_GameMode_C|GetdcardHandler _assettlers_game_mode)) "NewEnumerator5")
          ;[1 1 1] if not phase 11 (d-card use) or is using outbreak card
          (Default|HandlePlayerSpreadZombie (Variables|/Game/Settlers_GameMode.Settlers_GameMode_C|GetzombieHandler _assettlers_game_mode) self :!label _label)
          (Default|HandlePlayerAttack (Variables|/Game/Settlers_GameMode.Settlers_GameMode_C|GetzombieHandler _assettlers_game_mode) self)
          (else
            (Default|HandleTileonClickforDCard (Variables|/Game/Settlers_GameMode.Settlers_GameMode_C|GetdcardHandler _assettlers_game_mode) self)))
        (else
          (goto _label))))))

(fn UninfectTile
  (bind _resourcetype (Variables|Default|GetresourceType))
  (bind _hexagon_basic (Variables|Default|Gethexagon_basic))
  (if (Variables|Default|Getinfected)
    (Variables|Default|Setinfected false)
    (bind _returnvalue (Actor|GetActorOfClass "/Game/Blueprints/HexGrid/HexGrid.HexGrid_C"))
    (Variables|/Game/Blueprints/HexGrid/HexGrid.HexGrid_C|SetnumTilesInfected _returnvalue (- (Variables|/Game/Blueprints/HexGrid/HexGrid.HexGrid_C|GetnumTilesInfected _returnvalue) 1))
    (if (Utilities|IsValid (Variables|Default|Getcastle))
      ;[1 1 1] has castle
      (switch string _resourcetype
        (:wood
          (Components|StaticMesh|SetStaticMesh _hexagon_basic "/Game/Assets/resources/wood_full.wood_full"))
        (:wheat
          (Components|StaticMesh|SetStaticMesh _hexagon_basic "/Game/Assets/resources/wheat_full_v2.wheat_full_v2"))
        (:brick
          (Components|StaticMesh|SetStaticMesh _hexagon_basic "/Game/Assets/resources/brick_tile_full02.brick_tile_full02"))
        (:steel
          (Components|StaticMesh|SetStaticMesh _hexagon_basic "/Game/Assets/resources/steel_tile_full.steel_tile_full")))
      (else
        (switch string _resourcetype
          (:brick
            (Components|StaticMesh|SetStaticMesh _hexagon_basic "/Game/Assets/resources/brick_tile_empty03.brick_tile_empty03"))
          (:wood
            (Components|StaticMesh|SetStaticMesh _hexagon_basic "/Game/Assets/resources/wood_v10.wood_v10"))
          (:wheat
            (Components|StaticMesh|SetStaticMesh _hexagon_basic "/Game/Assets/resources/wheat_v17.wheat_v17"))
          (:steel
            (Components|StaticMesh|SetStaticMesh _hexagon_basic "/Game/Assets/resources/steel_tile_empty.steel_tile_empty")))))))

(fn HighlightTile
  (bind _self self)
  (bind _returnvalue (Transformation|GetActorTransform _self))
  (bind (_location _rotation _scale) (Math|Transform|BreakTransform _returnvalue))
  (bind (_x _y _z) (Math|Vector|BreakVector _scale))
  (if (not (Utilities|IsValid (Variables|Default|Gethighlight)))
    (bind _returnvalue_2 (Game|SpawnActorfromClass "/Game/Blueprints/AssetBPs/Highlight.Highlight_C" (Math|Transform|MakeTransform _location _rotation (Math|Vector|MakeVector _x _y (- _z 0.75))) "Undefined" 0 0))
    (Variables|Default|Sethighlight _returnvalue_2)
    (bind _returnvalue_3 (Actor|GetActorOfClass "/Game/Blueprints/HexGrid/HexGrid.HexGrid_C"))
    (Variables|/Game/Blueprints/HexGrid/HexGrid.HexGrid_C|SettilesHighlighted _returnvalue_3 true)))

(fn SetTiletoVersionforCastle
  (bind _hexagon_basic (Variables|Default|Gethexagon_basic))
  (switch string (Variables|Default|GetresourceType)
    (:wood
      (Components|StaticMesh|SetStaticMesh _hexagon_basic "/Game/Assets/resources/wood_full.wood_full"))
    (:wheat
      (Components|StaticMesh|SetStaticMesh _hexagon_basic "/Game/Assets/resources/wheat_full_v2.wheat_full_v2"))
    (:brick
      (Components|StaticMesh|SetStaticMesh _hexagon_basic "/Game/Assets/resources/brick_tile_full02.brick_tile_full02"))
    (:steel
      (Components|StaticMesh|SetStaticMesh _hexagon_basic "/Game/Assets/resources/steel_tile_full.steel_tile_full"))))

(fn CreateCastleTransform
  (bind _returnvalue (Transformation|GetActorTransform))
  (bind (_location _rotation _scale) (Math|Transform|BreakTransform _returnvalue))
  (return (Math|Transform|MakeTransform _location (Math|Rotator|MakeRotator 0.0 0.0 (* (* (Math|Conversions|ToFloat(Integer) (Math|Random|RandomIntegerinRange -2 2)) 15.0) -1.0)) _scale)))

(fn TileonUnhover
  (bind _assettlers_game_mode (Utilities|Casting|CastToSettlers_GameMode (Game|GetGameMode)))
  (if (and (== (Variables|/Game/Settlers_GameMode.Settlers_GameMode_C|Getphase _assettlers_game_mode) 0) (Utilities|IsValid (Variables|Default|GettransparentCastle)))
    (Actor|DestroyActor (Variables|Default|GettransparentCastle))))

(fn TileonHover
  (bind _returnvalue (Actor|GetActorOfClass "/Game/Blueprints/HexGrid/HexGrid.HexGrid_C"))
  (bind _assettlers_game_mode (Utilities|Casting|CastToSettlers_GameMode (Game|GetGameMode)))
  (if (Math|Boolean|ANDBoolean (== (Variables|/Game/Settlers_GameMode.Settlers_GameMode_C|Getphase _assettlers_game_mode) 0) (not (Utilities|IsValid (Variables|Default|GettransparentCastle))) (not (Utilities|IsValid (Variables|Default|Getcastle))) (not (Utilities|Enum|Equal(Enum) (Variables|Default|GetresourceType) "Zombie")) (Variables|/Game/Blueprints/HexGrid/HexGrid.HexGrid_C|GetspawnTransparentCastles _returnvalue))
    (bind _returnvalue_2 (Game|SpawnActorfromClass "/Game/Blueprints/AssetBPs/Castle.Castle_C" (Variables|Default|GetcastleTransform) "Undefined" 0 0))
    (bind _output_get (Variables|Default|SettransparentCastle _returnvalue_2))
    (CallFunction|SetCastleColor _output_get true)))

(fn SetTempCastleColor
  (bind _transparentcastle (Variables|Default|GettransparentCastle))
  (bind _transparentcastle_2 (Variables|Default|GettransparentCastle))
  (bind _castle (Variables|/Game/Blueprints/AssetBPs/Castle.Castle_C|GetCastle _transparentcastle))
  (bind _castle_2 (Variables|/Game/Blueprints/AssetBPs/Castle.Castle_C|GetCastle _transparentcastle_2))
  (bind _output (CallFunction|GetPlayerColor))
  (bind _castlestyle (CallFunction|GetCastleStyle))
  (switch string _castlestyle
    (:Default
      (switch string _output :!label _label
        (:Default
          (Rendering|Material|SetMaterial _castle_2 0 "/Game/Materials/castles/transparent_castles/M_castle_purple_transparent.M_castle_purple_transparent" :!label _label_2))
        (:Red
          (Rendering|Material|SetMaterial _castle_2 0 "/Game/Materials/castles/transparent_castles/M_castle_red_transparent.M_castle_red_transparent"))
        (:Blue
          (Rendering|Material|SetMaterial _castle_2 0 "/Game/Materials/castles/transparent_castles/M_castle_blue_transparent.M_castle_blue_transparent"))
        (:Pink
          (Rendering|Material|SetMaterial _castle_2 0 "/Game/Materials/castles/transparent_castles/M_castle_pink_transparent.M_castle_pink_transparent"))
        (:Purple
          (goto _label_2))))
    (:Fairy%20Tale
      (goto _label))
    (:Gothic
      (Components|StaticMesh|SetStaticMesh _castle "/Game/Assets/gothic_castle_uv.gothic_castle_uv")
      (switch string _output
        (:Default
          (Rendering|Material|SetMaterial _castle 0 "/Game/Materials/castles/gothic_castle/transparent_castles/M_gothic_castle_purple_transparent.M_gothic_castle_purple_transparent" :!label _label_3))
        (:Red
          (Rendering|Material|SetMaterial _castle 0 "/Game/Materials/castles/gothic_castle/transparent_castles/M_gothic_castle_red_transparent.M_gothic_castle_red_transparent"))
        (:Blue
          (Rendering|Material|SetMaterial _castle 0 "/Game/Materials/castles/gothic_castle/transparent_castles/M_gothic_castle_blue_transparent.M_gothic_castle_blue_transparent"))
        (:Pink
          (Rendering|Material|SetMaterial _castle 0 "/Game/Materials/castles/gothic_castle/transparent_castles/M_gothic_castle_pink_transparent.M_gothic_castle_pink_transparent"))
        (:Purple
          (goto _label_3)))
      (bind _newtransform (CallFunction|UpdateGothicCastleTransform))
      (Transformation|SetActorTransform _transparentcastle _newtransform))))

(fn GetCastleStyle
  (bind _assettlers_game_mode (Utilities|Casting|CastToSettlers_GameMode (Game|GetGameMode)))
  (return (.castleStyle (Utilities|Struct|BreakBP_PlayerStruct (Utilities|Array|Get(acopy) (Variables|/Game/Settlers_GameMode.Settlers_GameMode_C|Getplayers _assettlers_game_mode) (Variables|/Game/Settlers_GameMode.Settlers_GameMode_C|GetcurrentPlayerIndex _assettlers_game_mode))))))

(fn GetPlayerColor
  (bind _assettlers_game_mode (Utilities|Casting|CastToSettlers_GameMode (Game|GetGameMode)))
  (return (Utilities|Array|Get(acopy) (Variables|/Game/Blueprints/Handlers/PlayerHandler.PlayerHandler_C|GetplayerColors (Variables|/Game/Settlers_GameMode.Settlers_GameMode_C|GetplayerHandler _assettlers_game_mode)) (Variables|/Game/Settlers_GameMode.Settlers_GameMode_C|GetcurrentPlayerIndex _assettlers_game_mode))))

(fn UpdateGothicCastleTransform
  (bind _castletransform (Variables|Default|GetcastleTransform))
  (bind (_location _rotation _scale) (Math|Transform|BreakTransform _castletransform))
  (return (Math|Transform|MakeTransform _location (Math|Rotator|MakeRotator 0.0 0.0 (+ (.Yaw (Math|Rotator|BreakRotator _rotation)) 9e+01)) _scale)))

(fn GetSharedEdge
  (params (other :type Hex%20Tile%20Object%20Reference))
  (bind _values (Utilities|Map|Values (Variables|HexTile_C|Getedges other)))
  (bind _values_2 (Utilities|Map|Values (Variables|Default|Getedges)))
  (for _array_element _values_2
    (if (Utilities|Array|ContainsItem _values _array_element)
      (return _array_element)))
  (return 0))

(fn UpdateBountywhenCastlePlaced
  (bind _bountytext (Variables|Default|GetbountyText))
  (bind _ownerbountynum (Variables|/Game/Blueprints/UI/BountyText.BountyText_C|GetownerBountyNum _bountytext))
  (Widget|SetVisibility (Variables|/Game/Blueprints/UI/BountyText.BountyText_C|GetnonOwnerBountyNum (Variables|Default|GetbountyText)) "Visible")
  (bind _assettlers_game_mode (Utilities|Casting|CastToSettlers_GameMode (Game|GetGameMode)))
  (switch string (Utilities|Array|Get(acopy) (Variables|/Game/Blueprints/Handlers/PlayerHandler.PlayerHandler_C|GetplayerColors (Variables|/Game/Settlers_GameMode.Settlers_GameMode_C|GetplayerHandler _assettlers_game_mode)) (Variables|Default|GettileOwnerPlayerIndex))
    (:Default
      (Appearance|SetColorandOpacity _ownerbountynum (Utilities|Struct|MakeSlateColor "(R=0.699524,G=0.006236,B=0.048025,A=1.000000)") :!class /Script/UMG.TextBlock :!label _label))
    (:red
      (goto _label))
    (:blue
      (Appearance|SetColorandOpacity _ownerbountynum (Utilities|Struct|MakeSlateColor "(R=0.000000,G=0.105253,B=0.642081,A=1.000000)") :!class /Script/UMG.TextBlock))
    (:pink
      (Appearance|SetColorandOpacity _ownerbountynum (Utilities|Struct|MakeSlateColor "(R=0.699524,G=0.091184,B=0.680860,A=1.000000)") :!class /Script/UMG.TextBlock))
    (:purple
      (Appearance|SetColorandOpacity _ownerbountynum (Utilities|Struct|MakeSlateColor "(R=0.162613,G=0.000000,B=0.699524,A=1.000000)") :!class /Script/UMG.TextBlock))))

(fn UpdateOwnerBountyText
  (Rendering|Components|TextRender|SetText (Variables|/Game/Blueprints/UI/BountyText.BountyText_C|GetownerBountyNum (Variables|Default|GetbountyText)) (Utilities|Text|ToText(Integer) (Variables|Default|Getbounty))))

(fn RandomlyRotateTile
  (Transformation|SetWorldRotation (Variables|Default|Gethexagon_basic) (Math|Rotator|MakeRotator 0.0 0.0 (* (Math|Random|RandomIntegerinRange 0 5) 6e+01)) false false))