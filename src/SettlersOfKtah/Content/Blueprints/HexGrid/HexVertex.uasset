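; HexVertex is a clickable hex-grid corner in a Settlers-style game, where players build outposts, upgrade them to apothecaries and position knights.
; VertexClicked routes clicks by game phase, with outposts requiring spacing plus the player's adjacent castle or road.
; Placement-phase outposts collect initial resources and drive the ascending-then-descending player order.
; Pass-and-play handles clicks and highlights directly, while multiplayer routes them through PC_Player.
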(event EventBeginPlay
  (bind _assettlers_game_instance (Utilities|Casting|CastToSettlersGameInstance (Game|GetGameInstance)))
  (bind _output_get (Variables|Default|Setvertex_gameIsPP (Variables|/Game/Blueprints/SettlersGameInstance.SettlersGameInstance_C|GetisPassAndPlay _assettlers_game_instance)))
  (if (not _output_get)
    (bind _aspc_player (Utilities|Casting|CastToPC_Player (Game|GetPlayerController 0)))
    (Default|CToggleActorVisibility _aspc_player self true)))

(event EventClickInteract
  ;[1 1 1] handles clicks for both pass and play + MP
  (if (Variables|Default|Getvertex_gameIsPP)
    (CallFunction|VertexClicked)
    (else
      (bind _aspc_player (Utilities|Casting|CastToPC_Player (Game|GetPlayerController 0)))
      (Default|CHandleClick _aspc_player self))))

(event Input|KeyboardEvents|1
  (params (Key :type Key%20Structure))
  (:Pressed
    (CallFunction|HighlightValidVertices))
  (:Released
    (CallFunction|UnhighlightValidVertices)))

(fn ConstructionScript)

(fn SpawnOutpostifValid
  ;[1 1 1] Check to make sure it's valid to build outpost on this vertex
  (bind _isvalid (CallFunction|CheckifValidBuildLocation))
  (if _isvalid
    ;[1 1 1] If it's the placement phase, maybe spawn outpost
    (bind _placementphase (CallFunction|IsPlacementPhase))
    (if _placementphase
      (bind _spawnedoutpost (CallFunction|SpawnOutpostDuringPlacementPhase))
      (CallFunction|UnhighlightValidVertices)
      (return _spawnedoutpost)
      (else
        ;[1 1 1] Otherwise, if it's the outpost build phase, we can spawn an outpost
        (bind _outpostbuildphase (CallFunction|IsOutpostBuildPhase))
        (if _outpostbuildphase
          (bind _returnvalue (Game|SpawnActorfromClass "/Game/Blueprints/AssetBPs/Outpost.Outpost_C" (Transformation|GetActorTransform self) "Undefined" 0 0))
          (Variables|/Game/Blueprints/AssetBPs/Outpost.Outpost_C|Setvertex _returnvalue self)
          (Variables|Board|Setoutpost _returnvalue)
          (CallFunction|SetOutpostColor)
          (CallFunction|UpdatePlayerOwnedVertices)
          (CallFunction|UnhighlightValidVertices)
          ;[1 1 1] Tell the build panel to remove resources from the player, will also set the phase back to turn phase.
          (bind _assettlers_game_mode (Utilities|Casting|CastToSettlers_GameMode (Game|GetGameMode)))
          (bind _aspc_player (Utilities|Casting|CastToPC_Player (Game|GetPlayerController 0)))
          (bind _actionpanel (Variables|/Game/Blueprints/Player/PC_Player.PC_Player_C|GetactionPanel _aspc_player)
            (:then
              (Default|HandleOutpostBuilt (Variables|/Game/Blueprints/UI/ActionPanel.ActionPanel_C|GetBuildPanel _actionpanel))
              (bind _aspc_player_2 (Utilities|Casting|CastToPC_Player (Game|GetPlayerController 0)))
              (bind _gamelog (Variables|/Game/Blueprints/Player/PC_Player.PC_Player_C|GetgameLog _aspc_player_2)
                (:then
                  (Default|AddBuiltMessage _gamelog "Outpost" (Variables|/Game/Settlers_GameMode.Settlers_GameMode_C|GetcurrentPlayerIndex _assettlers_game_mode))
                  ;[1 1 1] Could have been placed on a knight, so might need to move knight location.
                  (bind _outactors (Actor|GetAllActorsOfClass "/Game/Blueprints/AssetBPs/Knight.Knight_C"))
                  (for _array_element _outactors
                    (Default|EditLocationifConflict _array_element))
                  (return true))
                (:else)))
            (:else))
          (else
            (return false)))))
    (else
      (return false))))

(fn SpawnOutpostDuringPlacementPhase
  (bind _assettlers_game_mode (Utilities|Casting|CastToSettlers_GameMode (Game|GetGameMode)))
  (if (Variables|/Game/Settlers_GameMode.Settlers_GameMode_C|GetplayerIsAscending _assettlers_game_mode)
    ;[1 1 1] if ascending, needs one castle; if descending, needs two castles
    (bind _hasonecastle (CallFunction|DoesPlayerHaveOneCastle))
    (if _hasonecastle
      _
      (else
        (return false)))
    (else
      (bind _hastwocastles (CallFunction|DoesPlayerHaveTwoCastles))
      (if _hastwocastles
        _
        (else
          (return false)))))
  (bind _returnvalue (Game|SpawnActorfromClass "/Game/Blueprints/AssetBPs/Outpost.Outpost_C" (Transformation|GetActorTransform self) "Undefined" 0 0))
  (Variables|/Game/Blueprints/AssetBPs/Outpost.Outpost_C|Setvertex _returnvalue self)
  (Variables|Board|Setoutpost _returnvalue)
  (CallFunction|SetOutpostColor)
  (CallFunction|UpdatePlayerOwnedVertices)
  (bind _assettlers_game_mode_2 (Utilities|Casting|CastToSettlers_GameMode (Game|GetGameMode)))
  ;[1 1 1] either go to the next player (either ascending or descending) or go to the turn phase
  (Default|CollectInitialResources (Variables|/Game/Settlers_GameMode.Settlers_GameMode_C|GetresourceHandler _assettlers_game_mode_2) self)
  (if (== (Variables|/Game/Settlers_GameMode.Settlers_GameMode_C|GetcurrentPlayerIndex _assettlers_game_mode_2) (- (Utilities|Array|Length (Variables|/Game/Settlers_GameMode.Settlers_GameMode_C|Getplayers _assettlers_game_mode_2)) 1))
    ;;[1 1 1] if last player, either stay or move to previous player (cycle back)
    (bind _hastwocastles_2 (CallFunction|DoesPlayerHaveTwoCastles))
    (if _hastwocastles_2
      (Default|MovetoNextPlayer _assettlers_game_mode_2)
      (else
        (Variables|/Game/Settlers_GameMode.Settlers_GameMode_C|SetplayerIsAscending _assettlers_game_mode_2 false)))
    ;[1 1 1] update resource ui after initial collection
    (bind _assettlers_game_mode_3 (Utilities|Casting|CastToSettlers_GameMode (Game|GetGameMode) :!label _label))
    (Default|UpdateResourcesUI (Variables|/Game/Settlers_GameMode.Settlers_GameMode_C|GetresourceHandler _assettlers_game_mode_3))
    ;[1 1 1] allow transparent castles to spawn
    (bind _returnvalue_2 (Actor|GetActorOfClass "/Game/Blueprints/HexGrid/HexGrid.HexGrid_C"))
    (Variables|/Game/Blueprints/HexGrid/HexGrid.HexGrid_C|SetspawnTransparentCastles _returnvalue_2 true)
    (else
      ;;[1 1 1] if first player, either move to second player or go to turn phase
      (if (== 0 (Variables|/Game/Settlers_GameMode.Settlers_GameMode_C|GetcurrentPlayerIndex _assettlers_game_mode_2))
        (bind _hastwocastles_3 (CallFunction|DoesPlayerHaveTwoCastles))
        (if _hastwocastles_3
          ;[1 1 1] go to turn phase
          (Default|HandleTurnPhase _assettlers_game_mode_2)
          (if (Variables|Default|Getvertex_gameIsPP)
            _
            (else
              (Default|SetupMPTurnPhase _assettlers_game_mode_2)))
          (else
            (Default|MovetoNextPlayer _assettlers_game_mode_2)
            (goto _label)))
        (else
          ;;[1 1 1] otherwise either move forwards or backwards to next player
          (Default|MovetoNextPlayer _assettlers_game_mode_2)
          (goto _label)))))
  (return true))

(fn HasAdjacentRoad
  (bind _assettlers_game_mode (Utilities|Casting|CastToSettlers_GameMode (Game|GetGameMode)))
  (for _array_element (Variables|Board|GetadjacentEdges)
    (if (Utilities|Array|ContainsItem (.edgesWithRoads (Utilities|Struct|BreakBP_PlayerStruct (Utilities|Array|Get(acopy) (Variables|/Game/Settlers_GameMode.Settlers_GameMode_C|Getplayers _assettlers_game_mode) (Variables|/Game/Settlers_GameMode.Settlers_GameMode_C|GetcurrentPlayerIndex _assettlers_game_mode)))) _array_element)
      (return true)))
  (return false))

(fn HasAdjacentCastle
  (for _array_element (Variables|Board|GetadjacentHexagons)
    (if (Utilities|IsValid (Variables|/Game/Blueprints/HexGrid/HexTile.HexTile_C|Getcastle _array_element))
      (bind _assettlers_game_mode (Utilities|Casting|CastToSettlers_GameMode (Game|GetGameMode)))
      (if (== (Variables|/Game/Settlers_GameMode.Settlers_GameMode_C|GetcurrentPlayerIndex _assettlers_game_mode) (Variables|/Game/Blueprints/HexGrid/HexTile.HexTile_C|GettileOwnerPlayerIndex _array_element))
        (return true))))
  (return false))

(fn IsTwoAway
  (for _array_element (Variables|Board|GetadjacentEdges)
    (for _array_element_2 (Variables|/Game/Blueprints/HexGrid/HexEdge.HexEdge_C|GetadjacentVertices _array_element)
      (if (Utilities|IsValid (Variables|HexVertex_C|Getoutpost _array_element_2))
        (return false))))
  (return true))

(fn IsPlacementPhase
  (bind _assettlers_game_mode (Utilities|Casting|CastToSettlers_GameMode (Game|GetGameMode)))
  (return (== (Variables|/Game/Settlers_GameMode.Settlers_GameMode_C|Getphase _assettlers_game_mode) 0)))

(fn DoesPlayerHaveTwoCastles
  (bind _assettlers_game_mode (Utilities|Casting|CastToSettlers_GameMode (Game|GetGameMode)))
  (return (== (Utilities|Array|Length (.castleTiles (Utilities|Struct|BreakBP_PlayerStruct (Utilities|Array|Get(acopy) (Variables|/Game/Settlers_GameMode.Settlers_GameMode_C|Getplayers _assettlers_game_mode) (Variables|/Game/Settlers_GameMode.Settlers_GameMode_C|GetcurrentPlayerIndex _assettlers_game_mode))))) 2)))

(fn DoesPlayerHaveOneCastle
  (bind _assettlers_game_mode (Utilities|Casting|CastToSettlers_GameMode (Game|GetGameMode)))
  (return (== (Utilities|Array|Length (.castleTiles (Utilities|Struct|BreakBP_PlayerStruct (Utilities|Array|Get(acopy) (Variables|/Game/Settlers_GameMode.Settlers_GameMode_C|Getplayers _assettlers_game_mode) (Variables|/Game/Settlers_GameMode.Settlers_GameMode_C|GetcurrentPlayerIndex _assettlers_game_mode))))) 1)))

(fn UpdatePlayerOwnedVertices
  (bind _assettlers_game_mode (Utilities|Casting|CastToSettlers_GameMode (Game|GetGameMode)))
  (Utilities|Array|Add (.verticesWithOutposts (Utilities|Struct|BreakBP_PlayerStruct (Utilities|Array|Get(acopy) (Variables|/Game/Settlers_GameMode.Settlers_GameMode_C|Getplayers _assettlers_game_mode) (Variables|/Game/Settlers_GameMode.Settlers_GameMode_C|GetcurrentPlayerIndex _assettlers_game_mode)))) self)
  (Variables|Default|SetownerPlayerIndex (Variables|/Game/Settlers_GameMode.Settlers_GameMode_C|GetcurrentPlayerIndex _assettlers_game_mode)))

(fn CheckifValidBuildLocation
  ;[1 1 1] Check if there's already an outpost on the vertex
  (Utilities|IsValid (Variables|Board|Getoutpost)
    (:Is%20Valid
      (return false))
    (:Is%20Not%20Valid
      ;[1 1 1] Check if it's two away from other outposts
      (bind _twoaway (CallFunction|IsTwoAway))
      (if _twoaway
        ;[1 1 1] Check if there's an adjacent castle owned by current player
        (bind _hasadjacentcastle (CallFunction|HasAdjacentCastle))
        (if _hasadjacentcastle
          (return true)
          (else
            ;[1 1 1] Otherwise, there might be an adjacent road
            (bind _hasadjacentroad (CallFunction|HasAdjacentRoad))
            (return _hasadjacentroad)))
        (else
          (return false))))))

(fn HighlightValidVertices
  (bind _returnvalue (Actor|GetActorOfClass "/Game/Blueprints/HexGrid/HexGrid.HexGrid_C"))
  (Utilities|Array|Clear (Variables|/Game/Blueprints/HexGrid/HexGrid.HexGrid_C|GethighlightedVertices _returnvalue))
  (bind _outactors (Actor|GetAllActorsOfClass "HexVertex_C"))
  (for _array_element _outactors
    (bind _isvalid (CallFunction|CheckifValidBuildLocation _array_element))
    (if _isvalid
      (if (Variables|Default|Getvertex_gameIsPP)
        (Rendering|SetVisibility (Variables|HexVertex_C|GetSphere _array_element) true true)
        (else
          (bind _assettlers_game_mode (Utilities|Casting|CastToSettlers_GameMode (Game|GetGameMode)))
          (for _array_element_2 (Variables|/Game/Settlers_GameMode.Settlers_GameMode_C|GetallPlayerControllers _assettlers_game_mode)
            (bind _aspc_player (Utilities|Casting|CastToPC_Player _array_element_2))
            (Default|CToggleActorVisibility _aspc_player _array_element false))))
      (Utilities|Array|AddUnique (Variables|/Game/Blueprints/HexGrid/HexGrid.HexGrid_C|GethighlightedVertices _returnvalue) _array_element)))
  (bind _returnvalue_2 (Actor|GetActorOfClass "/Game/Blueprints/HexGrid/HexGrid.HexGrid_C"))
  (Variables|/Game/Blueprints/HexGrid/HexGrid.HexGrid_C|SetverticesHighlighted _returnvalue_2 true))

(fn UnhighlightValidVertices
  (bind _returnvalue (Actor|GetActorOfClass "/Game/Blueprints/HexGrid/HexGrid.HexGrid_C"))
  (if (Variables|/Game/Blueprints/HexGrid/HexGrid.HexGrid_C|GetverticesHighlighted _returnvalue)
    (if (Variables|Default|Getvertex_gameIsPP)
      (for _array_element (Variables|/Game/Blueprints/HexGrid/HexGrid.HexGrid_C|GethighlightedVertices _returnvalue)
        (Rendering|SetVisibility (Variables|HexVertex_C|GetSphere _array_element) false true))
      (Variables|/Game/Blueprints/HexGrid/HexGrid.HexGrid_C|SetverticesHighlighted _returnvalue false)
      (else
        (bind _assettlers_game_mode (Utilities|Casting|CastToSettlers_GameMode (Game|GetGameMode)))
        (for _array_element_2 (Variables|/Game/Blueprints/HexGrid/HexGrid.HexGrid_C|GethighlightedVertices _returnvalue)
          (for _array_element_3 (Variables|/Game/Settlers_GameMode.Settlers_GameMode_C|GetallPlayerControllers _assettlers_game_mode)
            (bind _aspc_player (Utilities|Casting|CastToPC_Player _array_element_3))
            (Default|CToggleActorVisibility _aspc_player _array_element_2 true)))
        (Variables|/Game/Blueprints/HexGrid/HexGrid.HexGrid_C|SetverticesHighlighted _returnvalue false)))))

(fn SetOutpostColor
  (bind _outpost (Variables|Board|Getoutpost))
  (bind _assettlers_game_mode (Utilities|Casting|CastToSettlers_GameMode (Game|GetGameMode)))
  (bind _playerhandler (Variables|/Game/Settlers_GameMode.Settlers_GameMode_C|GetplayerHandler _assettlers_game_mode)
    (:then
      (switch string (Utilities|Array|Get(acopy) (Variables|/Game/Blueprints/Handlers/PlayerHandler.PlayerHandler_C|GetplayerColors _playerhandler) (Variables|/Game/Settlers_GameMode.Settlers_GameMode_C|GetcurrentPlayerIndex _assettlers_game_mode))
        (:Default
          (Variables|/Game/Blueprints/AssetBPs/Outpost.Outpost_C|SetoutpostMaterial _outpost "/Game/Materials/outposts/M_outpost_purple.M_outpost_purple" :!label _label))
        (:red
          (Variables|/Game/Blueprints/AssetBPs/Outpost.Outpost_C|SetoutpostMaterial _outpost "/Game/Materials/outposts/M_outpost_red.M_outpost_red"))
        (:blue
          (Variables|/Game/Blueprints/AssetBPs/Outpost.Outpost_C|SetoutpostMaterial _outpost "/Game/Materials/outposts/M_outpost_blue.M_outpost_blue"))
        (:pink
          (Variables|/Game/Blueprints/AssetBPs/Outpost.Outpost_C|SetoutpostMaterial _outpost "/Game/Materials/outposts/M_outpost_pink.M_outpost_pink"))
        (:purple
          (goto _label))))
    (:else)))

(fn IsOutpostBuildPhase
  (bind _assettlers_game_mode (Utilities|Casting|CastToSettlers_GameMode (Game|GetGameMode)))
  (return (== (Variables|/Game/Settlers_GameMode.Settlers_GameMode_C|Getphase _assettlers_game_mode) 3)))

(fn CheckifAnyValidOutpostLocation
  (bind _outactors (Actor|GetAllActorsOfClass "HexVertex_C"))
  (for _array_element _outactors
    (bind _isvalid (CallFunction|CheckifValidBuildLocation _array_element))
    (if _isvalid
      (return true)))
  (return false))

(fn HighlightOutpost
  (bind _returnvalue (Math|Float|MakeLiteralFloat 0.5))
  (bind _self self)
  (bind _returnvalue_2 (Transformation|GetActorTransform _self))
  (bind (_location _rotation _scale) (Math|Transform|BreakTransform _returnvalue_2))
  (if (not (Utilities|IsValid (Variables|Board|GetvertexHighlight)))
    (bind _returnvalue_3 (Game|SpawnActorfromClass "/Game/Blueprints/AssetBPs/VertexHighlight.VertexHighlight_C" (Math|Transform|MakeTransform _location _rotation (Math|Vector|MakeVector _returnvalue _returnvalue (- (.Z (Math|Vector|BreakVector _scale)) 0.75))) "Undefined" 0 0))
    (Variables|Board|SetvertexHighlight _returnvalue_3)))

(fn UnhighlightAllOutposts
  (bind _assettlers_game_mode (Utilities|Casting|CastToSettlers_GameMode (Game|GetGameMode)))
  (for _array_element (.verticesWithOutposts (Utilities|Struct|BreakBP_PlayerStruct (Utilities|Array|Get(acopy) (Variables|/Game/Settlers_GameMode.Settlers_GameMode_C|Getplayers _assettlers_game_mode) (Variables|/Game/Settlers_GameMode.Settlers_GameMode_C|GetcurrentPlayerIndex _assettlers_game_mode))))
    (if (Utilities|IsValid (Variables|HexVertex_C|GetvertexHighlight _array_element))
      (Actor|DestroyActor (Variables|HexVertex_C|GetvertexHighlight _array_element)))))

(fn UpgradeOutposttoApothecary
  ;[1 1 1] show apothecary component
  (Rendering|SetVisibility (Variables|/Game/Blueprints/AssetBPs/Outpost.Outpost_C|Getapothecary (Variables|Board|Getoutpost)) true false)
  (Variables|Default|SethasApothecary true)
  (CallFunction|UnhighlightAllOutposts)
  (bind _assettlers_game_mode (Utilities|Casting|CastToSettlers_GameMode (Game|GetGameMode)))
  (bind _aspc_player (Utilities|Casting|CastToPC_Player (Game|GetPlayerController 0)))
  (bind _actionpanel (Variables|/Game/Blueprints/Player/PC_Player.PC_Player_C|GetactionPanel _aspc_player)
    (:then
      (Default|HandleApothecaryBuilt (Variables|/Game/Blueprints/UI/ActionPanel.ActionPanel_C|GetBuildPanel _actionpanel))
      (bind _gamelog (Variables|/Game/Blueprints/Player/PC_Player.PC_Player_C|GetgameLog _aspc_player)
        (:then
          (Default|AddBuiltMessage _gamelog "Apothecary" (Variables|/Game/Settlers_GameMode.Settlers_GameMode_C|GetcurrentPlayerIndex _assettlers_game_mode)))
        (:else)))
    (:else)))

(fn VertexClicked
  ;[1 1 1] Check if we're in Knight Movement Phase, or we're using the Cavalry D-Card, or we're in Knight Placement Phase
  (bind _assettlers_game_mode (Utilities|Casting|CastToSettlers_GameMode (Game|GetGameMode)))
  (switch int (Variables|/Game/Settlers_GameMode.Settlers_GameMode_C|Getphase _assettlers_game_mode)
    (:Default
      ;[1 1 1] Check if there's an outpost
      (if (Utilities|IsValid (Variables|Board|Getoutpost))
        ;[1 1 1] check if apothecary upgrade phase
        (if (== (Variables|/Game/Settlers_GameMode.Settlers_GameMode_C|Getphase _assettlers_game_mode) 9)
          (CallFunction|UpgradeOutposttoApothecary))
        (return false)
        (else
          (bind _spawnedoutpost (CallFunction|SpawnOutpostifValid))
          (return _spawnedoutpost))))
    (:10
      (Default|MaybeMoveKnight (Variables|/Game/Settlers_GameMode.Settlers_GameMode_C|GetplayerHandler _assettlers_game_mode) self :!label _label))
    (:11
      (if (== (Variables|/Game/Blueprints/Handlers/DCardHandler.DCardHandler_C|GetcurrentlyUsedCard (Variables|/Game/Settlers_GameMode.Settlers_GameMode_C|GetdcardHandler _assettlers_game_mode)) (Utilities|Enum|LiteralenumDCards_Enum "NewEnumerator4"))
        (goto _label)
        (else
          _)))
    (:12
      (Default|MaybeSpawnKnight (Variables|/Game/Settlers_GameMode.Settlers_GameMode_C|GetzombieHandler _assettlers_game_mode) self)
      (return false)))
  (return false))

(fn Highlight
  (bind _returnvalue (Actor|GetActorOfClass "/Game/Blueprints/HexGrid/HexGrid.HexGrid_C"))
  (Variables|/Game/Blueprints/HexGrid/HexGrid.HexGrid_C|SetverticesHighlighted _returnvalue true)
  (if (Variables|Default|Getvertex_gameIsPP)
    (bind _returnvalue_2 (Actor|GetActorOfClass "/Game/Blueprints/HexGrid/HexGrid.HexGrid_C"))
    (Utilities|Array|Add (Variables|/Game/Blueprints/HexGrid/HexGrid.HexGrid_C|GethighlightedVertices _returnvalue_2) self)
    (Rendering|SetVisibility (Variables|Default|GetDefaultSceneRoot) true true)
    (else
      (bind _aspc_player (Utilities|Casting|CastToPC_Player (Game|GetPlayerController 0)))
      (Default|CToggleActorVisibility _aspc_player self false))))

(fn IsAdjacenttoVertex
  (params (vertex :type Hex%20Vertex%20Object%20Reference))
  (for _array_element (Variables|Board|GetadjacentEdges)
    (if (Utilities|Array|ContainsItem (Variables|/Game/Blueprints/HexGrid/HexEdge.HexEdge_C|GetadjacentVertices _array_element) vertex)
      (return true)))
  (return false))

(fn GetVertexBetween
  (params (vertex :type Hex%20Vertex%20Object%20Reference))
  ;[1 1 1] For each adjacent vertex
  (for _array_element (Variables|HexVertex_C|GetadjacentEdges vertex)
    (for _array_element_2 (Variables|/Game/Blueprints/HexGrid/HexEdge.HexEdge_C|GetadjacentVertices _array_element)
      ;[1 1 1] Check if that one is also adjacent to self
      (if (!= _array_element_2 vertex)
        (for _array_element_3 (Variables|HexVertex_C|GetadjacentEdges _array_element_2)
          (if (Utilities|Array|ContainsItem (Variables|/Game/Blueprints/HexGrid/HexEdge.HexEdge_C|GetadjacentVertices _array_element_3) self)
            (return _array_element_2)))))))