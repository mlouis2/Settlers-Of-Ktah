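; HexVertex is a clickable board vertex in a Settlers-style game where the current player builds outposts.
; A click spawns a player-colored outpost if the spot is empty, spaced from other outposts and beside the player's castle or road.
; Settlers_GameMode supplies phase and player state: placement collects initial resources and advances snake-order turns, while the build phase notifies BuildPanel.
; Holding key 1 reveals valid vertices through an all-actor scan.
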(event OnClicked(Sphere)
  (params (TouchedComponent :type Primitive%20Component%20Object%20Reference) (ButtonPressed :type Key%20Structure :default "None"))
  (CallFunction|SpawnOutpostifValid))

(event EventBeginPlay
  (Input|EnableInput (Game|GetPlayerController 0)))

(event Collision|EventActorBeginOverlap
  (params (OtherActor :type Actor%20Object%20Reference)))

(event EventTick
  (params (DeltaSeconds :type Float%20%28single-precision%29)))

(event MouseInput|EventActorBeginCursorOver
  ;[1 1 1] Highlight adjacent hexagons and edges when mouse over
)

(event MouseInput|EventActorEndCursorOver
  ;[1 1 1] Highlight adjacent hexagons and edges when mouse over
)

(event Input|KeyboardEvents|1
  (params (Key :type Key%20Structure :default "None"))
  (:Pressed
    (CallFunction|HighlightValidVertices))
  (:Released
    (CallFunction|UnhighlightAllVertices)))

(fn ConstructionScript)

(fn SpawnOutpostifValid
  ;[1 1 1] Check to make sure it's valid to build outpost on this vertex
  (bind _isvalid (CallFunction|CheckifValidBuildLocation))
  (if _isvalid
    ;[1 1 1] If it's the placement phase, maybe spawn outpost
    (bind _placementphase (CallFunction|IsPlacementPhase))
    (if _placementphase
      (CallFunction|SpawnOutpostDuringPlacementPhase)
      (CallFunction|UnhighlightAllVertices)
      (else
        ;[1 1 1] Otherwise, if it's the outpost build phase, we can spawn an outpost
        (bind _outpostbuildphase (CallFunction|IsOutpostBuildPhase))
        (if _outpostbuildphase
          (bind _returnvalue (Game|SpawnActorfromClass "/Game/Blueprints/Outpost.Outpost_C" (Transformation|GetActorTransform self) "Undefined" 0 0))
          (Variables|Default|Setoutpost _returnvalue)
          (CallFunction|SetOutpostColor)
          (CallFunction|UpdatePlayerOwnedVertices)
          (CallFunction|UnhighlightAllVertices)
          ;[1 1 1] Tell the build panel to remove resources from the player, will also set the phase back to turn phase.
          (bind _assettlers_game_mode (Utilities|Casting|CastToSettlers_GameMode (Game|GetGameMode)))
          (bind _asbuild_panel (Utilities|Casting|CastToBuildPanel (Variables|/Game/Settlers_GameMode.Settlers_GameMode_C|GetbuildUI _assettlers_game_mode)))
          (Default|HandleOutpostBuilt _asbuild_panel))))))

(fn SpawnOutpostDuringPlacementPhase
  (bind _assettlers_game_mode (Utilities|Casting|CastToSettlers_GameMode (Game|GetGameMode)))
  (if (Variables|/Game/Settlers_GameMode.Settlers_GameMode_C|GetplayerIsAscending _assettlers_game_mode)
    ;[1 1 1] if ascending, needs one castle; if descending, needs two castles
    (bind _hasonecastle (CallFunction|DoesPlayerHaveOneCastle))
    (if _hasonecastle
      (bind _returnvalue (Game|SpawnActorfromClass "/Game/Blueprints/Outpost.Outpost_C" (Transformation|GetActorTransform self) "Undefined" 0 0 :!label _label))
      (Variables|Default|Setoutpost _returnvalue)
      (CallFunction|SetOutpostColor)
      (CallFunction|UpdatePlayerOwnedVertices)
      (bind _assettlers_game_mode_2 (Utilities|Casting|CastToSettlers_GameMode (Game|GetGameMode)))
      (Default|CollectInitialResource _assettlers_game_mode_2 self)
      ;[1 1 1] either go to the next player (either ascending or descending) or go to the turn phase
      (if (== (Variables|/Game/Settlers_GameMode.Settlers_GameMode_C|GetcurrentPlayerIndex _assettlers_game_mode_2) (- (Utilities|Array|Length (Variables|/Game/Settlers_GameMode.Settlers_GameMode_C|Getplayers _assettlers_game_mode_2)) 1))
        ;;[1 1 1] if last player, either stay or move to previous player (cycle back)
        (bind _hastwocastles (CallFunction|DoesPlayerHaveTwoCastles))
        (if _hastwocastles
          (Default|MovetoNextPlayer _assettlers_game_mode_2)
          (else
            (Variables|/Game/Settlers_GameMode.Settlers_GameMode_C|SetplayerIsAscending _assettlers_game_mode_2 false)))
        ;[1 1 1] update resource ui after initial collection
        (bind _assettlers_game_mode_3 (Utilities|Casting|CastToSettlers_GameMode (Game|GetGameMode) :!label _label_2))
        (Default|UpdateResourcesUI _assettlers_game_mode_3)
        (else
          ;;[1 1 1] if first player, either move to second player or go to turn phase
          (if (== 0 (Variables|/Game/Settlers_GameMode.Settlers_GameMode_C|GetcurrentPlayerIndex _assettlers_game_mode_2))
            (bind _hastwocastles_2 (CallFunction|DoesPlayerHaveTwoCastles))
            (if _hastwocastles_2
              (Default|HandleTurnPhase _assettlers_game_mode_2)
              (else
                (Default|MovetoNextPlayer _assettlers_game_mode_2)
                (goto _label_2)))
            (else
              ;;[1 1 1] otherwise either move forwards or backwards to next player
              (Default|MovetoNextPlayer _assettlers_game_mode_2)
              (goto _label_2))))))
    (else
      (bind _hastwocastles_3 (CallFunction|DoesPlayerHaveTwoCastles))
      (if _hastwocastles_3
        (goto _label)))))

(fn HasAdjacentRoad
  (bind _assettlers_game_mode (Utilities|Casting|CastToSettlers_GameMode (Game|GetGameMode)))
  (for _array_element (Variables|Default|GetadjacentEdges)
    (if (Utilities|Array|ContainsItem (.edgesWithRoads (Utilities|Struct|BreakBP_PlayerStruct (Utilities|Array|Get(acopy) (Variables|/Game/Settlers_GameMode.Settlers_GameMode_C|Getplayers _assettlers_game_mode) (Variables|/Game/Settlers_GameMode.Settlers_GameMode_C|GetcurrentPlayerIndex _assettlers_game_mode)))) _array_element)
      (return true)))
  (return false))

(fn HasAdjacentCastle
  (for _array_element (Variables|Default|GetadjacentHexagons)
    (if (Utilities|IsValid (Variables|/Game/Blueprints/HexTile.HexTile_C|Getcastle _array_element))
      (bind _assettlers_game_mode (Utilities|Casting|CastToSettlers_GameMode (Game|GetGameMode)))
      (if (Utilities|Array|ContainsItem (.castles (Utilities|Struct|BreakBP_PlayerStruct (Utilities|Array|Get(acopy) (Variables|/Game/Settlers_GameMode.Settlers_GameMode_C|Getplayers _assettlers_game_mode) (Variables|/Game/Settlers_GameMode.Settlers_GameMode_C|GetcurrentPlayerIndex _assettlers_game_mode)))) (Variables|/Game/Blueprints/HexTile.HexTile_C|Getcastle _array_element))
        (return true))))
  (return false))

(fn IsTwoAway
  (for _array_element (Variables|Default|GetadjacentEdges)
    (for _array_element_2 (Variables|/Game/Blueprints/HexEdge.HexEdge_C|GetadjacentVertices _array_element)
      (if (Utilities|IsValid (Variables|HexVertex_C|Getoutpost _array_element_2))
        (return false))))
  (return true))

(fn IsPlacementPhase
  (bind _assettlers_game_mode (Utilities|Casting|CastToSettlers_GameMode (Game|GetGameMode)))
  (return (== (Variables|/Game/Settlers_GameMode.Settlers_GameMode_C|Getphase _assettlers_game_mode) 0)))

(fn DoesPlayerHaveTwoCastles
  (bind _assettlers_game_mode (Utilities|Casting|CastToSettlers_GameMode (Game|GetGameMode)))
  (return (== (Utilities|Array|Length (.castles (Utilities|Struct|BreakBP_PlayerStruct (Utilities|Array|Get(acopy) (Variables|/Game/Settlers_GameMode.Settlers_GameMode_C|Getplayers _assettlers_game_mode) (Variables|/Game/Settlers_GameMode.Settlers_GameMode_C|GetcurrentPlayerIndex _assettlers_game_mode))))) 2)))

(fn DoesPlayerHaveOneCastle
  (bind _assettlers_game_mode (Utilities|Casting|CastToSettlers_GameMode (Game|GetGameMode)))
  (return (== (Utilities|Array|Length (.castles (Utilities|Struct|BreakBP_PlayerStruct (Utilities|Array|Get(acopy) (Variables|/Game/Settlers_GameMode.Settlers_GameMode_C|Getplayers _assettlers_game_mode) (Variables|/Game/Settlers_GameMode.Settlers_GameMode_C|GetcurrentPlayerIndex _assettlers_game_mode))))) 1)))

(fn UpdatePlayerOwnedVertices
  (bind _assettlers_game_mode (Utilities|Casting|CastToSettlers_GameMode (Game|GetGameMode)))
  (Utilities|Array|Add (.vertices (Utilities|Struct|BreakBP_PlayerStruct (Utilities|Array|Get(acopy) (Variables|/Game/Settlers_GameMode.Settlers_GameMode_C|Getplayers _assettlers_game_mode) (Variables|/Game/Settlers_GameMode.Settlers_GameMode_C|GetcurrentPlayerIndex _assettlers_game_mode)))) self))

(fn CheckifValidBuildLocation
  ;[1 1 1] Check if there's already an outpost on the vertex
  (Utilities|IsValid (Variables|Default|Getoutpost)
    (:Is%20Valid
      (return false))
    (:Is%20Not%20Valid
      ;[1 1 1] Check if it's two away from other outposts
      (bind _twoaway (CallFunction|IsTwoAway))
      (if _twoaway
        ;[1 1 1] Check if there's an adjacent castle owned by current player
        (bind _hasadjacentcastle (CallFunction|HasAdjacentCastle))
        (if _hasadjacentcastle
          (return true)
          (else
            ;[1 1 1] Otherwise, there might be an adjacent road
            (bind _hasadjacentroad (CallFunction|HasAdjacentRoad))
            (return _hasadjacentroad)))
        (else
          (return false))))))

(fn HighlightValidVertices
  (bind _outactors (Actor|GetAllActorsOfClass "HexVertex_C"))
  (for _array_element _outactors
    (bind _isvalid (CallFunction|CheckifValidBuildLocation _array_element))
    (if _isvalid
      (Rendering|SetActorHiddenInGame _array_element false))))

(fn UnhighlightAllVertices
  (bind _outactors (Actor|GetAllActorsOfClass "HexVertex_C"))
  (for _array_element _outactors
    (Rendering|SetActorHiddenInGame _array_element true)))

(fn SetOutpostColor
  (bind _outpost (Variables|Default|Getoutpost))
  (bind _cone (Variables|/Game/Blueprints/Outpost.Outpost_C|GetCone _outpost))
  (bind _assettlers_game_mode (Utilities|Casting|CastToSettlers_GameMode (Game|GetGameMode)))
  (switch string (Utilities|Array|Get(acopy) (Variables|/Game/Settlers_GameMode.Settlers_GameMode_C|GetplayerColors _assettlers_game_mode) (Variables|/Game/Settlers_GameMode.Settlers_GameMode_C|GetcurrentPlayerIndex _assettlers_game_mode))
    (:Default
      (Rendering|Material|SetMaterial _cone 0 "/Game/Materials/outposts/M_outpost_purple.M_outpost_purple" :!label _label))
    (:red
      (Rendering|Material|SetMaterial _cone 0 "/Game/Materials/outposts/M_outpost_red.M_outpost_red"))
    (:blue
      (Rendering|Material|SetMaterial _cone 0 "/Game/Materials/outposts/M_outpost_blue.M_outpost_blue"))
    (:pink
      (Rendering|Material|SetMaterial _cone 0 "/Game/Materials/outposts/M_outpost_pink.M_outpost_pink"))
    (:purple
      (goto _label))))

(fn IsOutpostBuildPhase
  (bind _assettlers_game_mode (Utilities|Casting|CastToSettlers_GameMode (Game|GetGameMode)))
  (return (== (Variables|/Game/Settlers_GameMode.Settlers_GameMode_C|Getphase _assettlers_game_mode) 3)))