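; Knight piece for a Settlers board game that its owning player can move once on their turn along the vertex graph.
; Clicking it switches the game phase and highlights knight-free vertices one edge away, or two when the first edge has a road.
; MoveTo turns the knight, eases it over with a timeline-driven lerp, restores the turn phase and flags it moved.
; An offset is applied when its vertex holds an outpost.
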(event OnClicked(Knight)
  (params (TouchedComponent :type Primitive%20Component%20Object%20Reference) (ButtonPressed :type Key%20Structure :default "None"))
  (CallFunction|MaybeTriggerKnightMovement))

(event Custom|run
  (params (endVertex :type Hex%20Vertex%20Object%20Reference))
  (Variables|Default|Setmoving true)
  (Timeline|Timeline_0 Play
    (:Update
      (Transformation|SetWorldLocation (Variables|Default|GetKnight) (Math|Vector|Lerp(Vector) (Transformation|GetWorldLocation (Variables|Default|GetKnight)) (Transformation|GetWorldLocation (Variables|/Game/Blueprints/HexVertex.HexVertex_C|GetSphere endVertex)) (Utilities|Time|GetWorldDeltaSeconds)) false false))
    (:Finished
      (Variables|Default|Setmoving false))))

(event EventBeginPlay)

(event Collision|EventActorBeginOverlap
  (params (OtherActor :type Actor%20Object%20Reference)))

(event EventTick
  (params (DeltaSeconds :type Float%20%28single-precision%29)))

(fn ConstructionScript
  (CallFunction|EditLocationifConflict))

(fn CheckforConflict
  (params (vertex :type Hex%20Vertex%20Object%20Reference))
  (return (Utilities|IsValid (Variables|/Game/Blueprints/HexVertex.HexVertex_C|Getoutpost vertex))))

(fn MaybeTriggerKnightMovement
  ;[1 1 1] First, check that we're in the turn phase.
  (bind _assettlers_game_mode (Utilities|Casting|CastToSettlers_GameMode (Game|GetGameMode)))
  (if (== (Variables|/Game/Settlers_GameMode.Settlers_GameMode_C|Getphase _assettlers_game_mode) 1)
    ;[1 1 1] Make sure it's the current player's knight being clicked.
    (if (== (Variables|/Game/Settlers_GameMode.Settlers_GameMode_C|GetcurrentPlayerIndex _assettlers_game_mode) (Variables|Default|GetownerIndex))
      ;[1 1 1] Check whether or not current player's knight has already been moved.
      (if (not (Variables|/Game/Blueprints/PlayerHandler.PlayerHandler_C|GetcurrentHasMovedKnight (Variables|/Game/Settlers_GameMode.Settlers_GameMode_C|GetplayerHandler _assettlers_game_mode)))
        ;[1 1 1] Set game phase to KnightMovement and highlight vertices.
        (Variables|/Game/Settlers_GameMode.Settlers_GameMode_C|Setphase _assettlers_game_mode 10)
        (CallFunction|HighlightValidMovements)))))

(fn HighlightValidMovements
  (bind _currentvertex (Variables|Default|GetcurrentVertex))
  ;[1 1 1] Travel along edges adjacent to current location
  (for _array_element (Variables|/Game/Blueprints/HexVertex.HexVertex_C|GetadjacentEdges _currentvertex)
    ;[1 1 1] Check other vertices on those edges
    (for _array_element_2 (Variables|/Game/Blueprints/HexEdge.HexEdge_C|GetadjacentVertices _array_element)
      (if (!= _array_element_2 _currentvertex)
        ;[1 1 1] Highlight!
        (CallFunction|HighlightVertexifValid _array_element_2)
        ;[1 1 1] Check for road, if there's a road, do another step.
        (if (Utilities|IsValid (Variables|/Game/Blueprints/HexEdge.HexEdge_C|Getroad _array_element))
          (for _array_element_3 (Variables|/Game/Blueprints/HexVertex.HexVertex_C|GetadjacentEdges _array_element_2)
            (if (!= _array_element_3 _array_element)
              (for _array_element_4 (Variables|/Game/Blueprints/HexEdge.HexEdge_C|GetadjacentVertices _array_element_3)
                (CallFunction|HighlightVertexifValid _array_element_4)))))))))

(fn Moveto
  (params (vertex :type Hex%20Vertex%20Object%20Reference))
  (Default|UnhighlightAllVertices vertex)
  (CallFunction|SetRunDirection vertex)
  (CallFunction|Run vertex)
  (Variables|Default|SetcurrentVertex vertex)
  (CallFunction|EditLocationifConflict)
  (bind _assettlers_game_mode (Utilities|Casting|CastToSettlers_GameMode (Game|GetGameMode)))
  (Variables|/Game/Settlers_GameMode.Settlers_GameMode_C|Setphase _assettlers_game_mode 1)
  (Variables|/Game/Blueprints/PlayerHandler.PlayerHandler_C|SetcurrentHasMovedKnight (Variables|/Game/Settlers_GameMode.Settlers_GameMode_C|GetplayerHandler _assettlers_game_mode) true))

(fn EditLocationifConflict
  (bind _currentvertex (Variables|Default|GetcurrentVertex))
  (bind _knight (Variables|Default|GetKnight))
  (bind _relativelocation (Variables|/Script/Engine.SceneComponent|GetRelativeLocation _knight))
  (bind (_x _y _z) (Math|Vector|BreakVector _relativelocation))
  (if (Utilities|IsValid _currentvertex)
    (bind _hasconflict (CallFunction|CheckforConflict _currentvertex))
    (if _hasconflict
      (Transformation|SetRelativeLocation _knight (Math|Vector|MakeVector _x (+ _y 1e+01) _z) false false))))

(fn Destroy
  (Components|DestroyComponent (Variables|Default|GetKnight))
  (Actor|DestroyActor))

(fn HighlightVertexifValid
  (params (vertex :type Hex%20Vertex%20Object%20Reference))
  (bind _outactors (Actor|GetAllActorsOfClass "Knight_C"))
  (for _array_element _outactors
    (if (== vertex (Variables|Knight_C|GetcurrentVertex _array_element))
      (return)))
  (Default|Highlight vertex))

(fn SetRunDirection
  (params (destination :type Hex%20Vertex%20Object%20Reference))
  (bind _sphere (Variables|/Game/Blueprints/HexVertex.HexVertex_C|GetSphere destination))
  (bind _currentvertex (Variables|Default|GetcurrentVertex))
  (bind _returnvalue (Transformation|GetWorldLocation _sphere))
  (bind _sphere_2 (Variables|/Game/Blueprints/HexVertex.HexVertex_C|GetSphere _currentvertex))
  (bind _returnvalue_2 (Transformation|GetWorldLocation _sphere_2))
  (bind _returnvalue_3 (Math|Rotator|FindLookatRotation _returnvalue_2 _returnvalue))
  (bind (_roll _pitch _yaw) (Math|Rotator|BreakRotator _returnvalue_3))
  ;[1 1 1] Compare current and target vertex locations and set knight rotation based on that.
  (Transformation|SetWorldRotation (Variables|Default|GetKnight) (Math|Rotator|MakeRotator _roll _pitch (+ _yaw -9e+01)) false false))