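; Lobby game mode for the Settlers multiplayer game, tracking joined players and launching the match map by server travel.
; On login, the server stores the controller, reads lobby settings from the game instance and sets up that player's menu.
; Joins and logouts trigger a refresh that sends player count and info to every controller, updates the host's kick menu and recomputes whether all are ready.
; It also handles kicking players by index.
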(event Custom|EveryoneUpdate
  (bind _allplayercontrollers (Variables|Default|GetallPlayerControllers))
  ;[1 1 1] updates all players' lobby info
  (bind _output_get (Variables|Default|SetcurrentPlayersNum (Utilities|Array|Length (Variables|Default|GetallPlayerControllers))))
  (if (> _output_get 0)
    (Utilities|Array|Clear (Variables|Default|GetconnectedPlayers))
    (for _array_element _allplayercontrollers
      (bind _aslobby_player_controller (Utilities|Casting|CastToLobbyPlayerController _array_element))
      (Utilities|Array|Add (Variables|Default|GetconnectedPlayers) (Variables|/Game/Blueprints/LobbyPlayerController.LobbyPlayerController_C|GetPlayerSettings _aslobby_player_controller))
      (Default|UpdateNumberOfPlayers _aslobby_player_controller (Variables|Default|GetcurrentPlayersNum) (Variables|Default|GetmaxPlayers)))
    (for _array_element_2 _allplayercontrollers
      (bind _aslobby_player_controller_2 (Utilities|Casting|CastToLobbyPlayerController _array_element_2))
      (Default|AddPlayerInfo _aslobby_player_controller_2 (Variables|Default|GetconnectedPlayers))
      (CallFunction|AddtoKickList))
    ;[1 1 1] check that all players are ready -- if they are, canStartGame!
    (Variables|Default|SetcanStartGame true)
    (bind _array_element_3 (Utilities|Array|ForEachLoopwithBreak (Variables|Default|GetallPlayerControllers))
      (:LoopBody
        (bind _aslobby_player_controller_3 (Utilities|Casting|CastToLobbyPlayerController _array_element_3))
        (if (Utilities|Enum|Equal(Enum) (.readyStatus (Utilities|Struct|BreakBP_PlayerStruct (Variables|/Game/Blueprints/LobbyPlayerController.LobbyPlayerController_C|GetPlayerSettings _aslobby_player_controller_3))) (Utilities|Text|MakeLiteralText "Not Ready!"))
          (Variables|Default|SetcanStartGame false)
          (CallFunction|Break))))))

(event Custom|Break
  ;[1 1 1] check that all players are ready -- if they are, canStartGame!
  (Utilities|Array|ForEachLoopwithBreak (Variables|Default|GetallPlayerControllers)) ; enters at Break
)

(event Custom|LaunchGame
  ;[1 1 1] launch game and opens level
  (Development|ExecuteConsoleCommand "servertravel /Game/Maps/SettlersOfKtah" (Game|GetPlayerController 0)))

(event Custom|PlayerHasBeenKicked
  (params (playerIndex :type Integer))
  ;[1 1 1] kicks selected player from lobby
  (bind _aslobby_player_controller (Utilities|Casting|CastToLobbyPlayerController (Utilities|Array|Get(acopy) (Variables|Default|GetallPlayerControllers) playerIndex)))
  (Default|Kicked _aslobby_player_controller))

(event Custom|AddToKickList
  ;[1 1 1] populate kick list when new player joins
  (bind _aslobby_player_controller (Utilities|Casting|CastToLobbyPlayerController (Game|GetPlayerController 0)))
  (Utilities|IsValid (Variables|/Game/Blueprints/LobbyPlayerController.LobbyPlayerController_C|GetLobbyMenuUI _aslobby_player_controller)
    (:Is%20Valid
      (if (Widget|IsVisible (Variables|/Game/Blueprints/UI/TitleScreen/LobbyMenuUI.LobbyMenuUI_C|GetkickMenu (Variables|/Game/Blueprints/LobbyPlayerController.LobbyPlayerController_C|GetLobbyMenuUI _aslobby_player_controller)))
        (Default|FillKickMenu (Variables|/Game/Blueprints/LobbyPlayerController.LobbyPlayerController_C|GetLobbyMenuUI _aslobby_player_controller))))))

(event EventOnLogout
  (params (ExitingController :type Controller%20Object%20Reference))
  ;[1 1 1] onLogout-- removes player controller and connected player
  (bind (_array_element _array_index) (Utilities|Array|ForEachLoopwithBreak (Variables|Default|GetallPlayerControllers) :!label _label)
    (:LoopBody
      (if (== _array_element ExitingController)
        (goto _label Break)))
    (:Completed
      (Utilities|Array|RemoveIndex (Variables|Default|GetallPlayerControllers) _array_index)
      (Utilities|Array|RemoveIndex (Variables|Default|GetconnectedPlayers) _array_index)
      (CallFunction|EveryoneUpdate))))

(event EventPostLogin
  (params (NewPlayer :type Player%20Controller%20Object%20Reference))
  ;[1 1 1] initial setup -- handles lobby set up and spawns player
  (Networking|SwitchHasAuthority
    (:Authority
      (Utilities|Array|Add (Variables|Default|GetallPlayerControllers) NewPlayer)
      (bind _assettlers_game_instance (Utilities|Casting|CastToSettlersGameInstance (Game|GetGameInstance)))
      (Variables|Default|SetmaxPlayers (Variables|/Game/Blueprints/SettlersGameInstance.SettlersGameInstance_C|GetmaxPlayers _assettlers_game_instance))
      (Variables|Default|SetserverName (Variables|/Game/Blueprints/SettlersGameInstance.SettlersGameInstance_C|GetserverName _assettlers_game_instance))
      (bind _aslobby_player_controller (Utilities|Casting|CastToLobbyPlayerController NewPlayer))
      (Default|InitialSetup _aslobby_player_controller)
      (Default|SetupLobbyMenu _aslobby_player_controller)
      (CallFunction|EveryoneUpdate))))

(fn ConstructionScript)