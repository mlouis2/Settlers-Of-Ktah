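; BP_Zombie is a minigame zombie that chases a single target chosen at random when it spawns.
; On BeginPlay it gathers the player character and every BP_Door_Target actor, stores one random pick as ZombieTarget, then clears the candidate list.
; Tick reissues AI MoveTo toward that target every frame, and the target is never re-evaluated afterwards.
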(event EventBeginPlay
  (bind _zombietargets (Variables|Default|GetZombieTargets))
  (Utilities|Array|Add (Variables|Default|GetZombieTargets) (Game|GetPlayerCharacter 0))
  (bind _outactors (Actor|GetAllActorsOfClass "/Game/Blueprints/MiniGame/BP_Door_Target.BP_Door_Target_C"))
  (for _array_element _outactors
    (bind _output_get (Variables|Default|SetDoor_Target1 _array_element))
    (Utilities|Array|Add _zombietargets _output_get))
  (Variables|Default|SetZombie_Target (Utilities|Array|Get(acopy) _zombietargets (Math|Random|RandomInteger (Utilities|Array|Length _zombietargets))))
  (Utilities|Array|Clear (Variables|Default|GetZombieTargets)))

(event Collision|EventActorBeginOverlap
  (params (OtherActor :type Actor%20Object%20Reference)))

(event EventTick
  (params (DeltaSeconds :type Float%20%28single-precision%29))
  (AI|AIMoveTo self "0, 0, 0" (Variables|Default|GetZombie_Target) 5.0 false))

(fn ConstructionScript)