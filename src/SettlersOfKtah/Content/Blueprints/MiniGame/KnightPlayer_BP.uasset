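; Player knight for a zombie minigame, with axis movement and four directional melee attacks.
; Each attack briefly shows its cube and, if a zombie overlaps it, calls ZombieTakeDamage with a "Side" or "FrontBack" hit type.
; Zombie contact with the knight's hitbox drains health through a delayed while-loop macro until contact ends.
; CastleTakeDamage also tracks castle health here, and either health reaching zero shows the GameOver widget.
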(event OnComponentEndOverlap(S_Cube)
  (params (OverlappedComponent :type Primitive%20Component%20Object%20Reference) (OtherActor :type Actor%20Object%20Reference) (OtherComp :type Primitive%20Component%20Object%20Reference) (OtherBodyIndex :type Integer))
  (if (== (Utilities|GetClass OtherActor) "/Game/Blueprints/MiniGame/BP_Zombie.BP_Zombie_C")
    (Variables|Default|SetZombieInS false)))

(event OnComponentBeginOverlap(KnightHitBox)
  (params (OverlappedComponent :type Primitive%20Component%20Object%20Reference) (OtherActor :type Actor%20Object%20Reference) (OtherComp :type Primitive%20Component%20Object%20Reference) (OtherBodyIndex :type Integer) (bFromSweep :type Boolean) (SweepResult :type Hit%20Result%20Structure%20%28by%20ref%29))
  (bind _knighthealth (Variables|Default|GetKnightHealth))
  (if (== (Utilities|GetClass OtherActor) "/Game/Blueprints/MiniGame/BP_Zombie.BP_Zombie_C")
    (Variables|Default|SetZombieAttacking true)
    (Development|PrintString "OM NOM")
    (Utilities|WhileLoopwithDelay (Variables|Default|GetZombieAttacking) 1.5
      (:LoopBody
        (bind _result (Math|Integer|DecrementInt _knighthealth)
          (:%20%20
            (Development|PrintString (Utilities|String|ToString(Integer) _result))
            (if (<= _knighthealth 0)
              (bind _returnvalue (UserInterface|CreateWidget "/Game/Blueprints/MiniGame/Widgets/GameOver.GameOver_C"))
              (UserInterface|Viewport|AddtoViewport _returnvalue 0))))))))

(event OnComponentEndOverlap(KnightHitBox)
  (params (OverlappedComponent :type Primitive%20Component%20Object%20Reference) (OtherActor :type Actor%20Object%20Reference) (OtherComp :type Primitive%20Component%20Object%20Reference) (OtherBodyIndex :type Integer))
  (if (== (Utilities|GetClass OtherActor) "/Game/Blueprints/MiniGame/BP_Zombie.BP_Zombie_C")
    (Variables|Default|SetZombieAttacking false)))

(event OnComponentBeginOverlap(E_Cube)
  (params (OverlappedComponent :type Primitive%20Component%20Object%20Reference) (OtherActor :type Actor%20Object%20Reference) (OtherComp :type Primitive%20Component%20Object%20Reference) (OtherBodyIndex :type Integer) (bFromSweep :type Boolean) (SweepResult :type Hit%20Result%20Structure%20%28by%20ref%29))
  (if (== (Utilities|GetClass OtherActor) "/Game/Blueprints/MiniGame/BP_Zombie.BP_Zombie_C")
    (Variables|Default|SetZombieInE true)))

(event OnComponentEndOverlap(E_Cube)
  (params (OverlappedComponent :type Primitive%20Component%20Object%20Reference) (OtherActor :type Actor%20Object%20Reference) (OtherComp :type Primitive%20Component%20Object%20Reference) (OtherBodyIndex :type Integer))
  (if (== (Utilities|GetClass OtherActor) "/Game/Blueprints/MiniGame/BP_Zombie.BP_Zombie_C")
    (Variables|Default|SetZombieInE false)))

(event OnComponentBeginOverlap(N_Cube)
  (params (OverlappedComponent :type Primitive%20Component%20Object%20Reference) (OtherActor :type Actor%20Object%20Reference) (OtherComp :type Primitive%20Component%20Object%20Reference) (OtherBodyIndex :type Integer) (bFromSweep :type Boolean) (SweepResult :type Hit%20Result%20Structure%20%28by%20ref%29))
  (if (== (Utilities|GetClass OtherActor) "/Game/Blueprints/MiniGame/BP_Zombie.BP_Zombie_C")
    (Variables|Default|SetZombieInN true)))

(event OnComponentEndOverlap(N_Cube)
  (params (OverlappedComponent :type Primitive%20Component%20Object%20Reference) (OtherActor :type Actor%20Object%20Reference) (OtherComp :type Primitive%20Component%20Object%20Reference) (OtherBodyIndex :type Integer))
  (if (== (Utilities|GetClass OtherActor) "/Game/Blueprints/MiniGame/BP_Zombie.BP_Zombie_C")
    (Variables|Default|SetZombieInN false)))

(event OnComponentBeginOverlap(W_Cube)
  (params (OverlappedComponent :type Primitive%20Component%20Object%20Reference) (OtherActor :type Actor%20Object%20Reference) (OtherComp :type Primitive%20Component%20Object%20Reference) (OtherBodyIndex :type Integer) (bFromSweep :type Boolean) (SweepResult :type Hit%20Result%20Structure%20%28by%20ref%29))
  (if (== (Utilities|GetClass OtherActor) "/Game/Blueprints/MiniGame/BP_Zombie.BP_Zombie_C")
    (Variables|Default|SetZombieInW true)))

(event OnComponentEndOverlap(W_Cube)
  (params (OverlappedComponent :type Primitive%20Component%20Object%20Reference) (OtherActor :type Actor%20Object%20Reference) (OtherComp :type Primitive%20Component%20Object%20Reference) (OtherBodyIndex :type Integer))
  (if (== (Utilities|GetClass OtherActor) "/Game/Blueprints/MiniGame/BP_Zombie.BP_Zombie_C")
    (Variables|Default|SetZombieInW false)))

(event OnComponentBeginOverlap(S_Cube)
  (params (OverlappedComponent :type Primitive%20Component%20Object%20Reference) (OtherActor :type Actor%20Object%20Reference) (OtherComp :type Primitive%20Component%20Object%20Reference) (OtherBodyIndex :type Integer) (bFromSweep :type Boolean) (SweepResult :type Hit%20Result%20Structure%20%28by%20ref%29))
  (if (== (Utilities|GetClass OtherActor) "/Game/Blueprints/MiniGame/BP_Zombie.BP_Zombie_C")
    (Variables|Default|SetZombieInS true)))

(event EventBeginPlay
  (Development|PrintString "BAZINGA" true true "(R=0.000000,G=0.660000,B=1.000000,A=1.000000)" 5.0)
  (Input|EnableInput (Game|GetPlayerController 0))
  (Variables|Default|SetGameMode (Game|GetGameMode)))

(event Collision|EventActorBeginOverlap
  (params (OtherActor :type Actor%20Object%20Reference)))

(event EventTick
  (params (DeltaSeconds :type Float%20%28single-precision%29)))

(event Input|ActionEvents|InputActionMiniGame_AttackEast
  (params (Key :type Key%20Structure :default "None"))
  (:Pressed
    (Variables|Default|SetHitType "Side")
    (Rendering|SetVisibility (Variables|Default|GetE_Cube) true false)
    (if (Variables|Default|GetZombieInE)
      (Development|PrintString "got em")
      (bind _asbp_zombie (Utilities|Casting|CastToBP_Zombie (stale OnComponentBeginOverlap(E_Cube) OtherActor)))
      (Default|ZombieTakeDamage _asbp_zombie (Variables|Default|GetHitType)))
    (Utilities|FlowControl|Delay 0.5)
    (Rendering|SetVisibility (Variables|Default|GetE_Cube) false false)))

(event Input|ActionEvents|InputActionMiniGame_AttackNorth
  (params (Key :type Key%20Structure :default "None"))
  (:Pressed
    (Variables|Default|SetHitType "FrontBack")
    (Rendering|SetVisibility (Variables|Default|GetN_Cube) true false)
    (if (Variables|Default|GetZombieInN)
      (Development|PrintString "got em")
      (bind _asbp_zombie (Utilities|Casting|CastToBP_Zombie (stale OnComponentBeginOverlap(N_Cube) OtherActor)))
      (Default|ZombieTakeDamage _asbp_zombie (Variables|Default|GetHitType)))
    (Utilities|FlowControl|Delay 0.5)
    (Rendering|SetVisibility (Variables|Default|GetN_Cube) false false)))

(event Input|ActionEvents|InputActionMiniGame_AttackSouth
  (params (Key :type Key%20Structure :default "None"))
  (:Pressed
    (Variables|Default|SetHitType "FrontBack")
    (Rendering|SetVisibility (Variables|Default|GetS_Cube) true false)
    (if (Variables|Default|GetZombieInS)
      (Development|PrintString "got em")
      (bind _asbp_zombie (Utilities|Casting|CastToBP_Zombie (stale OnComponentBeginOverlap(S_Cube) OtherActor)))
      (Default|ZombieTakeDamage _asbp_zombie (Variables|Default|GetHitType)))
    (Utilities|FlowControl|Delay 0.5)
    (Rendering|SetVisibility (Variables|Default|GetS_Cube) false false)))

(event Input|ActionEvents|InputActionMiniGame_AttackWest
  (params (Key :type Key%20Structure :default "None"))
  (:Pressed
    (Variables|Default|SetHitType "Side")
    (Rendering|SetVisibility (Variables|Default|GetW_Cube) true false)
    (if (Variables|Default|GetZombieInW)
      (Development|PrintString "got em")
      (bind _asbp_zombie (Utilities|Casting|CastToBP_Zombie (stale OnComponentBeginOverlap(W_Cube) OtherActor)))
      (Default|ZombieTakeDamage _asbp_zombie (Variables|Default|GetHitType)))
    (Utilities|FlowControl|Delay 0.5)
    (Rendering|SetVisibility (Variables|Default|GetW_Cube) false false)))

(event Input|AxisEvents|InputAxisMiniGame_MoveNorth
  (params (AxisValue :type Float%20%28single-precision%29))
  (if (Variables|Default|GetMovementEnabled)
    (Pawn|Input|AddMovementInput (Math|Vector|GetForwardVector (Variables|Collision|GetCapsuleComponent)) AxisValue false)))

(event Input|AxisEvents|InputAxisMiniGame_MoveEast
  (params (AxisValue :type Float%20%28single-precision%29))
  (if (Variables|Default|GetMovementEnabled)
    (Pawn|Input|AddMovementInput (Math|Vector|GetRightVector (Variables|Collision|GetCapsuleComponent)) AxisValue false)))

(fn ConstructionScript)

(fn CastleTakeDamage
  (bind _castlehealth (Variables|Default|GetCastleHealth))
  (bind _result (Math|Integer|DecrementInt _castlehealth)
    (:%20%20
      (Development|PrintString (Utilities|String|ToString(Integer) _result))
      (if (<= _castlehealth 0)
        (bind _returnvalue (UserInterface|CreateWidget "/Game/Blueprints/MiniGame/Widgets/GameOver.GameOver_C"))
        (UserInterface|Viewport|AddtoViewport _returnvalue 0)))))