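; MiniGame game mode that runs a timed zombie minigame with a HUD and a game-over screen.
; On BeginPlay it spawns a hex actor, then zombies at random spawn points through ForLoopDelay, a loop with random delays between iterations.
; The HUD setup and zombie count do not wait for that staggered spawning to finish.
; Tick uses a one-second Delay to count down TimeRemaining and shows game over at zero.
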(event EventBeginPlay
  (Utilities|FlowControl|Sequence
    (:then_0
      (Development|PrintString "Hello" true true "(R=0.000000,G=0.660000,B=1.000000,A=1.000000)" 5.0)
      (Development|PrintString "bitch")
      (Game|SpawnActorfromClass "/Game/Blueprints/MiniGame/MiniGame_Hex.MiniGame_Hex_C" (Variables|Default|GetNewVar_0) "Undefined" 0 0))
    (:then_1
      ;[1 1 1] Get Spawn Points
      (bind _outactors (Actor|GetAllActorsOfClass "/Game/Blueprints/MiniGame/BP_Zombie_SpawnPoint.BP_Zombie_SpawnPoint_C"))
      (bind _output_get (Variables|Default|SetZombie_SpawnPoints _outactors)))
    (:then_2
      ;[1 1 1] Spawn Zombies
      (Utilities|ForLoopDelay 0 (Variables|Default|GetNumZombies)
        (:LoopBody
          (bind _returnvalue (AI|SpawnAIFromClass "/Game/Blueprints/MiniGame/BP_Zombie.BP_Zombie_C" 0 (Transformation|GetWorldLocation (Variables|/Script/Engine.Actor|GetRootComponent (Utilities|Array|Get(acopy) _output_get (Math|Random|RandomInteger (Utilities|Array|Length _output_get))))) "0, 0, 0" false 0))
          (bind _asbp_zombie (Utilities|Casting|CastToBP_Zombie _returnvalue))
          (Default|ZombiesGo _asbp_zombie)
          (Development|PrintString "peepeepoopoo"))))
    (:then_3
      ;[1 1 1] Set HUD
      (bind _returnvalue_2 (UserInterface|CreateWidget "/Game/Blueprints/MiniGame/Widgets/MiniGameHUD.MiniGameHUD_C"))
      (UserInterface|Viewport|AddtoViewport _returnvalue_2 0)
      (Variables|Default|SetTimeRemaining (Variables|Default|GetTotalTime))
      (bind _outactors_2 (Actor|GetAllActorsOfClass "/Game/Blueprints/MiniGame/BP_Zombie.BP_Zombie_C"))
      (Variables|Default|SetZombiesRemaining (Utilities|Array|Length _outactors_2)))))

(event EventTick
  (params (DeltaSeconds :type Float%20%28single-precision%29))
  (bind _timeremaining (Variables|Default|GetTimeRemaining))
  ;[1 1 1] Timer
  (Utilities|FlowControl|Delay 1.0)
  (Math|Integer|DecrementInt _timeremaining
    (:%20%20
      (if (<= _timeremaining 0)
        (bind _returnvalue (UserInterface|CreateWidget "/Game/Blueprints/MiniGame/Widgets/GameOver.GameOver_C"))
        (UserInterface|Viewport|AddtoViewport _returnvalue 0)
        (Development|PrintString "time")))))

(fn ConstructionScript)