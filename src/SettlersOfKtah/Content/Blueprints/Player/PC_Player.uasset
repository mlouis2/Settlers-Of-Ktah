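; Player controller for Settlers of K'tah, a hex-grid board game, linking each player's input, UI and saved profile to the server.
; On non-pass-and-play login it loads the saved profile and passes it to Settlers_GameMode.
; C_ client events manage widgets, turn state, resource spinner and PlayerInfo refreshes from GameState.
; Hovers and clicks are gated to the current player, then routed through S_ server events to tiles and vertices.
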(event Custom|PassPlayerInfoToServer
  (params (playerInfo :type BP%20Player%20Struct%20Structure))
  ;[1 1 1] only on login -- pass player info to server
  (Variables|Default|SetPlayerInfo playerInfo)
  (bind _assettlers_game_mode (Utilities|Casting|CastToSettlers_GameMode (Game|GetGameMode)))
  (Default|RespawnPlayer _assettlers_game_mode self)
  (CallFunction|CallServerUpdate))

(event Custom|C_EndTurn
  ;[1 1 1] handle EndTurn button clicked on ActionPanel
  (CallFunction|SEndTurn))

(event Custom|S_EndTurn
  ;[1 1 1] handle EndTurn button clicked on ActionPanel
  (bind _returnvalue (Actor|GetActorOfClass "/Game/Blueprints/HexGrid/HexGrid.HexGrid_C"))
  (Default|UnhighlightAllTiles _returnvalue)
  (bind _assettlers_game_mode (Utilities|Casting|CastToSettlers_GameMode (Game|GetGameMode)))
  (Variables|/Game/Settlers_GameMode.Settlers_GameMode_C|Setphase _assettlers_game_mode 1)
  (Default|MovetoNextPlayer _assettlers_game_mode))

(event Custom|C_PlaySpinner
  (params (resource :type String))
  (bind _spinnerplayer (Variables|Widgets|GetspinnerPlayer))
  (bind _spinnerplayer_2 (Variables|Widgets|GetspinnerPlayer))
  ;[1 1 1] client side PC -- spinner logic -- disable all widgets (when spinner is going)
  (CallFunction|DisableAllWidgets)
  (UserInterface|Viewport|AddtoViewport (Variables|Widgets|GetspinnerUI) 0)
  (switch string resource
    (:wheat
      (Media|MediaPlayer|OpenSource _spinnerplayer "/Game/Movies/SpinnerWheat.SpinnerWheat"))
    (:wood
      (Media|MediaPlayer|OpenSource _spinnerplayer "/Game/Movies/SpinnerWood.SpinnerWood"))
    (:brick
      (Media|MediaPlayer|OpenSource _spinnerplayer_2 "/Game/Movies/SpinnerBrick.SpinnerBrick"))
    (:steel
      (Media|MediaPlayer|OpenSource _spinnerplayer_2 "/Game/Movies/SpinnerSteel.SpinnerSteel"))
    (:zombie
      (Media|MediaPlayer|OpenSource _spinnerplayer_2 "/Game/Movies/SpinnerZombie.SpinnerZombie"))))

(event Custom|C_ToggleActorVisibility
  (params (actor :type Actor%20Object%20Reference%20%28by%20ref%29) (mustHide :type Boolean))
  (bind _rootcomponent (Variables|/Script/Engine.Actor|GetRootComponent actor))
  ;[1 1 1] client PC -- toggle actor visibility
  (if mustHide
    (Rendering|SetVisibility _rootcomponent false true)
    (else
      (Rendering|SetVisibility _rootcomponent (== (.playerIndex (Utilities|Struct|BreakBP_PlayerStruct (Variables|Default|GetPlayerInfo))) (Variables|Default|GetcurrentPlayer)) true))))

(event Custom|DisableAllWidgets
  ;[1 1 1] client side PC -- spinner logic -- disable all widgets (when spinner is going)
  (bind _actionpanel (Variables|Widgets|GetactionPanel)
    (:then
      (Widget|SetVisibility _actionpanel "Collapsed")
      (bind _resourcepanel (Variables|Widgets|GetresourcePanel)
        (:then
          (Widget|SetIsEnabled (Variables|/Game/Blueprints/UI/ResourcesPanel.ResourcesPanel_C|GetshowBountyButton _resourcepanel) false)
          (Widget|SetIsEnabled (Variables|/Game/Blueprints/UI/ResourcesPanel.ResourcesPanel_C|GetdevCardButton _resourcepanel) false))
        (:else)))
    (:else)))

(event Custom|C_HandleClick
  (params (clickedActor :type Actor%20Object%20Reference))
  ;[1 1 1] client side PC -- route hovers and clicks to server if current player
  (Utilities|FlowControl|Delay 0.2)
  (if (== (Variables|Default|GetcurrentPlayer) (.playerIndex (Utilities|Struct|BreakBP_PlayerStruct (Variables|Default|GetPlayerInfo))))
    (CallFunction|SHandleClick clickedActor self)
    (else
      (Development|PrintString "not your turn!" true true "(R=0.725640,G=0.000000,B=0.005035,A=1.000000)" 2e+01))))

(event Custom|S_HandleClick
  (params (clickedActor :type Actor%20Object%20Reference) (client :type PC%20Player%20Object%20Reference))
  ;[1 1 1] server side PC -- handle hover events (only HexTile) and click events
  (CallFunction|HandleActorClicks clickedActor client))

(event Custom|SpinnerOnEnd
  (Media|MediaPlayer|Close (Variables|Widgets|GetspinnerPlayer) :!class /Script/MediaAssets.MediaPlayer)
  (Widget|RemovefromParent (Variables|Widgets|GetspinnerUI)))

(event Custom|C_HandleHover
  (params (hoveredActor :type Actor%20Object%20Reference) (serverAlreadyRouted :type Boolean))
  ;[1 1 1] client side PC -- route hovers and clicks to server if current player
  (Utilities|FlowControl|Delay 0.1)
  (if (== (Variables|Default|GetcurrentPlayer) (.playerIndex (Utilities|Struct|BreakBP_PlayerStruct (Variables|Default|GetPlayerInfo))))
    (bind _ashex_tile (Utilities|Casting|CastToHexTile hoveredActor))
    (if serverAlreadyRouted
      (Default|TileonHover _ashex_tile self true)
      (else
        (CallFunction|SHandleHover _ashex_tile self)))))

(event Custom|C_EnableNonTurnWidgets
  ;[1 1 1] client side PC -- enable widgets for player whose turn is not up yet
  ;[1 1 1] client PC -- update resource panel
  (Development|PrintString "enabling non player turn widget" true true "(R=0.254294,G=1.000000,B=0.000000,A=1.000000)" 2e+01)
  (bind _actionpanel (Variables|Widgets|GetactionPanel)
    (:then
      (Widget|SetVisibility _actionpanel "Collapsed")
      (bind _resourcepanel (Variables|Widgets|GetresourcePanel)
        (:then
          (Widget|SetIsEnabled (Variables|/Game/Blueprints/UI/ResourcesPanel.ResourcesPanel_C|GetshowBountyButton _resourcepanel) true)
          (Widget|SetIsEnabled (Variables|/Game/Blueprints/UI/ResourcesPanel.ResourcesPanel_C|GetdevCardButton _resourcepanel) true)
          (bind _dcardmodal (Variables|Widgets|GetdCardModal)
            (:then
              (Default|UpdateBuyButton _dcardmodal)
              (Default|UpdateUseButton _dcardmodal))
            (:else)))
        (:else)))
    (:else)))

(event Custom|C_MPInitialSetup
  ;[1 1 1] client side PC -- initial setup for multiplayer -- spawns all UI
  (Variables|Default|SetbShowMouseCursor true)
  (CallFunction|SpawnWidgets)
  (bind _returnvalue (UserInterface|CreateWidget "/Game/Blueprints/UI/ResourceSpinner.ResourceSpinner_C" self))
  (Variables|Widgets|SetspinnerUI _returnvalue)
  (Media|MediaPlayer|BindEventtoOnEndReached (Variables|Widgets|GetspinnerPlayer) (delegate Custom|SpinnerOnEnd)))

(event Custom|C_UpdateResourcePanel
  ;[1 1 1] client PC -- update resource panel
  (bind _resourcepanel (Variables|Widgets|GetresourcePanel)
    (:then
      (for _array_element (.numResourcesStructs (Utilities|Struct|BreakBP_PlayerStruct (Variables|Default|GetPlayerInfo)))
        (switch string (.resourceType (Utilities|Struct|BreakResourceStruct _array_element))
          (:wheat
            (Default|SetWheatAmount _resourcepanel (Utilities|String|ToString(Integer) (.count (Utilities|Struct|BreakResourceStruct _array_element)))))
          (:wood
            (Default|SetWoodAmount _resourcepanel (Utilities|String|ToString(Integer) (.count (Utilities|Struct|BreakResourceStruct _array_element)))))
          (:brick
            (Default|SetBrickAmount _resourcepanel (Utilities|String|ToString(Integer) (.count (Utilities|Struct|BreakResourceStruct _array_element)))))
          (:steel
            (Default|SetSteelAmount _resourcepanel (Utilities|String|ToString(Integer) (.count (Utilities|Struct|BreakResourceStruct _array_element))))))))
    (:else)))

(event Custom|C_UpdatePlayerInfo
  ;[1 1 1] client side PC -- update stored player info with the one from GameState
  (bind _assettlers_game_state (Utilities|Casting|CastToSettlersGameState (Game|GetGameState)))
  (for _array_element (Variables|/Game/Blueprints/SettlersGameState.SettlersGameState_C|GetallPlayersInfo _assettlers_game_state)
    (if (== (.playerIndex (Utilities|Struct|BreakBP_PlayerStruct _array_element)) (.playerIndex (Utilities|Struct|BreakBP_PlayerStruct (Variables|Default|GetPlayerInfo))))
      (Variables|Default|SetPlayerInfo _array_element))))

(event Custom|C_EnableTurnWidgets
  ;[1 1 1] client side PC -- enable widgets for player whose turn is up
  ;[1 1 1] client side PC -- enable widgets for player whose turn is not up yet
  (Development|PrintString "enabling player turn widgets" true true "(R=0.030849,G=1.000000,B=0.000000,A=1.000000)" 2e+01)
  (if (== (Variables|Default|GetPCgamePhase) 0)
    _
    (else
      (bind _actionpanel (Variables|Widgets|GetactionPanel)
        (:then
          (Widget|SetVisibility _actionpanel "Visible"))
        (:else))))
  (bind _resourcepanel (Variables|Widgets|GetresourcePanel)
    (:then
      (Widget|SetIsEnabled (Variables|/Game/Blueprints/UI/ResourcesPanel.ResourcesPanel_C|GetshowBountyButton _resourcepanel) true)
      (Widget|SetIsEnabled (Variables|/Game/Blueprints/UI/ResourcesPanel.ResourcesPanel_C|GetdevCardButton _resourcepanel) true)
      (bind _dcardmodal (Variables|Widgets|GetdCardModal)
        (:then
          (Default|UpdateBuyButton _dcardmodal)
          (Default|UpdateUseButton _dcardmodal))
        (:else)))
    (:else)))

(event Custom|CallServerUpdate
  ;[1 1 1] server side PC -- tell server to update everyone
  (bind _assettlers_game_mode (Utilities|Casting|CastToSettlers_GameMode (Game|GetGameMode)))
  (Default|EveryoneUpdate _assettlers_game_mode))

(event Custom|ClientUpdate
  ;[1 1 1] client side PC -- do whatever update necessary
  (CallFunction|CUpdatePlayerInfo)
  (if (== (Variables|Default|GetPCgamePhase) 0)
    (bind _playerpanel (Variables|Widgets|GetplayerPanel)
      (:then
        (Default|UpdatePlayerNames _playerpanel)
        (Default|UpdatePlayerIcons _playerpanel)
        (CallFunction|CUpdateResourcePanel))
      (:else))
    (else
      (CallFunction|CUpdateResourcePanel))))

(event Custom|RemoveLoadingScreen
  ;[1 1 1] removes loading screen when going from lobby to game
  (bind _foundwidgets (Widget|GetAllWidgetsOfClass "/Game/Blueprints/UI/LoadingScreen.LoadingScreen_C" true))
  (for _array_element _foundwidgets
    (Widget|RemovefromParent _array_element)))

(event Custom|C_StartTurn
  ;[1 1 1] client side PC -- update widgets on start of turn
  (bind _playerpanel (Variables|Widgets|GetplayerPanel)
    (:then
      (Default|UnhighlightPlayer _playerpanel (Variables|Default|GetpreviousPlayer))
      (Default|HighlightPlayer _playerpanel (Variables|Default|GetcurrentPlayer))
      (if (== (.playerIndex (Utilities|Struct|BreakBP_PlayerStruct (Variables|Default|GetPlayerInfo))) (Variables|Default|GetcurrentPlayer))
        (CallFunction|CEnableTurnWidgets)
        (else
          (CallFunction|CEnableNonTurnWidgets))))
    (:else)))

(event Custom|S_HandleHover
  (params (hoveredTile :type Hex%20Tile%20Object%20Reference) (client :type PC%20Player%20Object%20Reference))
  ;[1 1 1] server side PC -- handle hover events (only HexTile) and click events
  (Default|TileonHover hoveredTile client false))

(event Custom|C_TurnPhaseSetup
  ;[1 1 1] client side PC -- setup for turn phase
  (Variables|Default|SetPCgamePhase 1)
  (bind _resourcepanel (Variables|Widgets|GetresourcePanel)
    (:then
      (Default|ToggleBountyVisibility _resourcepanel true))
    (:else)))

(event EventBeginPlay
  ;[1 1 1] if pass and play, no extra handling; otherwise load player info and pass to server side player controller
  (bind _assettlers_game_instance (Utilities|Casting|CastToSettlersGameInstance (Game|GetGameInstance)))
  (if (not (Variables|/Game/Blueprints/SettlersGameInstance.SettlersGameInstance_C|GetisPassAndPlay _assettlers_game_instance))
    (if (Pawn|IsLocalController)
      (CallFunction|RemoveLoadingScreen)
      (CallFunction|LoadGame)
      (Pawn|SetControlRotation (Math|Rotator|MakeRotator 0.0 -51.049084 180.205505))
      (CallFunction|PassPlayerInfotoServer (Variables|Default|GetPlayerInfo)))))

(event Input|MouseEvents|LeftMouseButton
  (params (Key :type Key%20Structure :default "None"))
  (bind _returnvalue (Game|GetPlayerController 0))
  (bind _hitresult (Game|Player|GetHitResultUnderCursorbyChannel _returnvalue "TraceTypeQuery1" true))
  (bind (_bblockinghit _binitialoverlap _time _distance _location _impactpoint _normal _impactnormal _physmat _hitactor) (Collision|BreakHitResult _hitresult))
  ;[1 1 1] PC controls left click and routes via interface
  (:Pressed
    (if _bblockinghit
      (if (Utilities|DoesObjectImplementInterface _hitactor "/Game/Blueprints/InteractInterface.InteractInterface_C")
        (Class|InteractInterface|ClickInteract(Message) _hitactor)))))

(fn ConstructionScript)

(fn LoadGame
  (bind _returnvalue (SaveGame|LoadGamefromSlot (Variables|Default|GetPlayerSettingsSave)))
  (bind _asplayer_save_game (Utilities|Casting|CastToPlayerSaveGame _returnvalue))
  (if (== (.playerIndex (Utilities|Struct|BreakBP_PlayerStruct (Variables|Default|GetPlayerInfo))) -1)
    (Variables|Default|SetPlayerInfo (Variables|/Game/Blueprints/Player/PlayerSaveGame.PlayerSaveGame_C|GetS_PlayerInfo _asplayer_save_game))
    (else
      (Variables|Default|SetPlayerInfo (Utilities|Struct|MakeBP_PlayerStruct 0 0 0 "((\"wheat\", 0),(\"wood\", 0),(\"brick\", 0),(\"steel\", 0))" 0 0 0 (.name (Utilities|Struct|BreakBP_PlayerStruct (Variables|/Game/Blueprints/Player/PlayerSaveGame.PlayerSaveGame_C|GetS_PlayerInfo _asplayer_save_game))) false (.castleStyle (Utilities|Struct|BreakBP_PlayerStruct (Variables|/Game/Blueprints/Player/PlayerSaveGame.PlayerSaveGame_C|GetS_PlayerInfo _asplayer_save_game))) 0 "NewEnumerator0" 0 "Not Ready!" (.playerIndex (Utilities|Struct|BreakBP_PlayerStruct (Variables|Default|GetPlayerInfo))))))))

(fn HandleActorClicks
  (params (clickedActor :type Actor%20Object%20Reference%20%28by%20ref%29) (player :type PC%20Player%20Object%20Reference%20%28by%20ref%29))
  (bind _returnvalue (Utilities|GetClass clickedActor))
  (bind _playerinfo (Variables|PC_Player_C|GetPlayerInfo player))
  (bind (_castletiles _verticeswithoutposts) (Utilities|Struct|BreakBP_PlayerStruct _playerinfo))
  (if (Utilities|ClassIsChildOf _returnvalue "/Game/Blueprints/HexGrid/HexTile.HexTile_C")
    (bind _ashex_tile (Utilities|Casting|CastToHexTile clickedActor))
    (bind _spawnedcastle (Default|TileonClick _ashex_tile))
    (if _spawnedcastle
      (Utilities|Array|Add _castletiles _ashex_tile))
    (elif (Utilities|ClassIsChildOf _returnvalue "/Game/Blueprints/HexGrid/HexVertex.HexVertex_C")
      (bind _ashex_vertex (Utilities|Casting|CastToHexVertex clickedActor))
      (bind _spawnedoutpost (Default|VertexClicked _ashex_vertex))
      (if _spawnedoutpost
        (Utilities|Array|Add _verticeswithoutposts _ashex_vertex)))))

(fn CheckEnoughResources
  (params (resourcesToCheck :type Array%20of%20Resource%20Struct%20Structures))
  (for _array_element resourcesToCheck
    (for _array_element_2 (.numResourcesStructs (Utilities|Struct|BreakBP_PlayerStruct (Variables|Default|GetPlayerInfo)))
      (if (Utilities|Enum|Equal(Enum) (.resourceType (Utilities|Struct|BreakResourceStruct _array_element_2)) (.resourceType (Utilities|Struct|BreakResourceStruct _array_element)))
        (if (not (>= (.count (Utilities|Struct|BreakResourceStruct _array_element_2)) (.count (Utilities|Struct|BreakResourceStruct _array_element))))
          (return false)))))
  (return true))

(fn SpawnWidgets
  (bind _self self)
  (bind _self_2 self)
  (Utilities|FlowControl|Sequence
    (:then_0
      (bind _returnvalue (UserInterface|CreateWidget "/Game/Blueprints/UI/PlayerPanel/PlayerPanel.PlayerPanel_C" _self))
      (bind _output_get (Variables|Widgets|SetplayerPanel _returnvalue))
      (UserInterface|Viewport|AddtoViewport _output_get 0))
    (:then_1
      (bind _returnvalue_2 (UserInterface|CreateWidget "/Game/Blueprints/UI/ResourcesPanel.ResourcesPanel_C" _self))
      (bind _output_get_2 (Variables|Widgets|SetresourcePanel _returnvalue_2))
      (UserInterface|Viewport|AddtoViewport _output_get_2 0))
    (:then_2
      (bind _returnvalue_3 (UserInterface|CreateWidget "/Game/Blueprints/UI/ActionPanel.ActionPanel_C" _self))
      (bind _output_get_3 (Variables|Widgets|SetactionPanel _returnvalue_3))
      (UserInterface|Viewport|AddtoViewport _output_get_3 0)
      (Widget|SetVisibility _output_get_3 "Collapsed"))
    (:then_3
      (bind _returnvalue_4 (UserInterface|CreateWidget "/Game/Blueprints/UI/BuildPanel.BuildPanel_C" _self_2))
      (bind _output_get_4 (Variables|Widgets|SetbuildPanel _returnvalue_4))
      (UserInterface|Viewport|AddtoViewport _output_get_4 0)
      (Widget|SetVisibility _output_get_4 "Collapsed"))
    (:then_4
      (bind _returnvalue_5 (UserInterface|CreateWidget "/Game/Blueprints/UI/Trade/TradePanel.TradePanel_C" _self_2))
      (bind _output_get_5 (Variables|Widgets|SettradePanel _returnvalue_5))
      (UserInterface|Viewport|AddtoViewport _output_get_5 0)
      (Widget|SetVisibility _output_get_5 "Collapsed"))
    (:then_5
      (bind _returnvalue_6 (UserInterface|CreateWidget "/Game/Blueprints/UI/Settings/SettingsButton.SettingsButton_C" _self_2))
      (bind _output_get_6 (Variables|Widgets|SetsettingsButton _returnvalue_6))
      (UserInterface|Viewport|AddtoViewport _output_get_6 0))
    (:then_6
      (bind _returnvalue_7 (UserInterface|CreateWidget "/Game/Blueprints/UI/GameLog/GameLog.GameLog_C" _self_2))
      (bind _output_get_7 (Variables|Widgets|SetgameLog _returnvalue_7))
      (UserInterface|Viewport|AddtoViewport _output_get_7 0)
      (Default|AddMessage _output_get_7 (Utilities|Text|ToText(String) (Utilities|String|MakeLiteralString "Welcome to Settlers of K'tah!"))))
    (:then_7
      (bind _returnvalue_8 (UserInterface|CreateWidget "/Game/Blueprints/UI/DCards/DCards_Main.DCards_Main_C" self))
      (Variables|Widgets|SetdCardModal _returnvalue_8))))