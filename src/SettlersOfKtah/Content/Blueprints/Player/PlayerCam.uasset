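; PlayerCam is a player camera pawn that pans and zooms from axis input.
; The CameraMoveForward and CameraMoveRight axes add movement input along fixed world negative X and negative Y, independent of view rotation.
; ZoomIn moves the pawn along world Z, so zoom is a height change rather than an FOV or arm-length adjustment.
; BeginPlay, Tick, overlap and the construction script are empty.
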(event EventBeginPlay)

(event Collision|EventActorBeginOverlap
  (params (OtherActor :type Actor%20Object%20Reference)))

(event EventTick
  (params (DeltaSeconds :type Float%20%28single-precision%29)))

(event Input|AxisEvents|InputAxisZoomIn
  (params (AxisValue :type Float%20%28single-precision%29))
  (if (!= AxisValue 0.0)
    (Pawn|Input|AddMovementInput "0, 0,1.000000" AxisValue false)))

(event Input|AxisEvents|InputAxisCameraMoveRight
  (params (AxisValue :type Float%20%28single-precision%29))
  (if (!= AxisValue 0.0)
    (Pawn|Input|AddMovementInput "0,-1.000000,0.000000" AxisValue false)))

(event Input|AxisEvents|InputAxisCameraMoveForward
  (params (AxisValue :type Float%20%28single-precision%29))
  (if (!= AxisValue 0.0)
    (Pawn|Input|AddMovementInput "-1.000000, 0,0.000000" AxisValue false)))

(fn ConstructionScript)