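; PlayerHandler manages player elimination, victory checks and per-player upkeep for the Settlers game mode, and creates the PlayerPanel UI on BeginPlay.
; Players with all castle tiles infected are knocked out, triggering a lone-survivor check.
; That check, plus military and research point thresholds, calls EndGame on the game mode.
; Other functions decrement knights and expire timed road barricades, with knight and elimination changes pushed to the panel.
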(event EventBeginPlay
  (bind _returnvalue (UserInterface|CreateWidget "/Game/Blueprints/UI/PlayerPanel.PlayerPanel_C"))
  (UserInterface|Viewport|AddtoViewport _returnvalue 0)
  (Variables|Default|SetplayerUI _returnvalue))

(event Collision|EventActorBeginOverlap
  (params (OtherActor :type Actor%20Object%20Reference)))

(event EventTick
  (params (DeltaSeconds :type Float%20%28single-precision%29)))

(fn ConstructionScript)

(fn MaybeKickPlayerOut
  (params (playerIndex :type Integer))
  ;[1 1 1] kick player out of game if both their castle tiles are infected
  (bind _assettlers_game_mode (Utilities|Casting|CastToSettlers_GameMode (Game|GetGameMode)))
  (for _array_element (.castleTiles (Utilities|Struct|BreakBP_PlayerStruct (Utilities|Array|Get(acopy) (Variables|/Game/Settlers_GameMode.Settlers_GameMode_C|Getplayers _assettlers_game_mode) playerIndex)))
    (if (not (Variables|/Game/Blueprints/HexTile.HexTile_C|Getinfected _array_element))
      (return)))
  (Utilities|Struct|SetmembersinBP_PlayerStruct (Utilities|Array|Get(acopy) (Variables|/Game/Settlers_GameMode.Settlers_GameMode_C|Getplayers _assettlers_game_mode) playerIndex) true)
  (Default|UpdateLosingPlayerUI (Variables|Default|GetplayerUI) playerIndex)
  ;;[1 1 1] check if game over
  (CallFunction|CheckforLoneSurvivorVictory))

(fn CheckforMilitaryVictory
  (params (playerIndex :type Integer))
  (bind _assettlers_game_mode (Utilities|Casting|CastToSettlers_GameMode (Game|GetGameMode)))
  (if (>= (.numDefensePoints (Utilities|Struct|BreakBP_PlayerStruct (Utilities|Array|Get(acopy) (Variables|/Game/Settlers_GameMode.Settlers_GameMode_C|Getplayers _assettlers_game_mode) playerIndex))) 10)
    (Default|EndGame _assettlers_game_mode playerIndex)))

(fn CheckforLoneSurvivorVictory
  (bind _assettlers_game_mode (Utilities|Casting|CastToSettlers_GameMode (Game|GetGameMode)))
  (for (_array_element _array_index) (Variables|/Game/Settlers_GameMode.Settlers_GameMode_C|Getplayers _assettlers_game_mode)
    ;[1 1 1] if player hasn't lost and there is currently no potential winner, set them to be potential winner
    (if (not (.isOutOfGame (Utilities|Struct|BreakBP_PlayerStruct _array_element)))
      (if (== (Variables|Default|GetpotentialWinnerIndex) -1)
        (Variables|Default|SetpotentialWinnerIndex _array_index)
        (else
          ;;[1 1 1] if there is already another potential winner, game not over, reset potential winner index
          (Variables|Default|SetpotentialWinnerIndex -1)
          (return)))))
  ;[1 1 1] at the end of loop if potential winner index is not reset, we have a winner!
  (if (not (== (Variables|Default|GetpotentialWinnerIndex) -1))
    (Default|EndGame _assettlers_game_mode (Variables|Default|GetpotentialWinnerIndex) 1)))

(fn CheckforResearchVictory
  (params (playerIndex :type Integer))
  (bind _assettlers_game_mode (Utilities|Casting|CastToSettlers_GameMode (Game|GetGameMode)))
  (if (>= (.numResearchPoints (Utilities|Struct|BreakBP_PlayerStruct (Utilities|Array|Get(acopy) (Variables|/Game/Settlers_GameMode.Settlers_GameMode_C|Getplayers _assettlers_game_mode) playerIndex))) 10)
    (Default|EndGame _assettlers_game_mode playerIndex 2)))

(fn RemovePlayerKnights
  (params (playerIndex :type Integer))
  (bind _assettlers_game_mode (Utilities|Casting|CastToSettlers_GameMode (Game|GetGameMode)))
  (if (> (.numKnights (Utilities|Struct|BreakBP_PlayerStruct (Utilities|Array|Get(acopy) (Variables|/Game/Settlers_GameMode.Settlers_GameMode_C|Getplayers _assettlers_game_mode) playerIndex))) 0)
    (Utilities|Struct|SetmembersinBP_PlayerStruct (Utilities|Array|Get(acopy) (Variables|/Game/Settlers_GameMode.Settlers_GameMode_C|Getplayers _assettlers_game_mode) playerIndex) (- (.numKnights (Utilities|Struct|BreakBP_PlayerStruct (Utilities|Array|Get(acopy) (Variables|/Game/Settlers_GameMode.Settlers_GameMode_C|Getplayers _assettlers_game_mode) playerIndex))) 1))
    (Default|UpdatePlayerNumKnights (Variables|Default|GetplayerUI) playerIndex)))

(fn UpdateBarricades
  (params (playerIndex :type Integer))
  ;[1 1 1] First, get the player's roads.
  (bind _assettlers_game_mode (Utilities|Casting|CastToSettlers_GameMode (Game|GetGameMode)))
  ;[1 1 1] Check if the road is a barricade.
  (for _array_element (.edgesWithRoads (Utilities|Struct|BreakBP_PlayerStruct (Utilities|Array|Get(acopy) (Variables|/Game/Settlers_GameMode.Settlers_GameMode_C|Getplayers _assettlers_game_mode) playerIndex)))
    (if (Variables|/Game/Blueprints/HexEdge.HexEdge_C|GetisBarricade _array_element)
      ;[1 1 1] If the barricade has existed for 5 turns, get rid of it.
      (if (>= (Variables|/Game/Blueprints/HexEdge.HexEdge_C|GetbarricadeTurnCount _array_element) 4)
        (Variables|/Game/Blueprints/HexEdge.HexEdge_C|SetisBarricade _array_element false)
        (Variables|/Game/Blueprints/HexEdge.HexEdge_C|SetbarricadeTurnCount _array_element 0)
        (else
          ;[1 1 1] If the barricade is still ongoing, increase the turn count.
          (Variables|/Game/Blueprints/HexEdge.HexEdge_C|SetbarricadeTurnCount _array_element (+ (Variables|/Game/Blueprints/HexEdge.HexEdge_C|GetbarricadeTurnCount _array_element) 1)))))))