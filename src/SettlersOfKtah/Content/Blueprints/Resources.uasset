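; Resource manager for a Settlers-style turn-based game: picks random resources, plays spinner videos, updates the resources panel and checks build costs.
; Collection pays players bounties from uninfected hexes adjacent to their vertices, while a zombie result triggers infection spread through Settlers_GameMode.
; Player maps are edited via a temporary copy written back into the struct array.
; RemoveResourceFromPlayer's subtraction is unwired, so it deducts nothing.
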(event Custom|CloseSpinnerPlayer
  ;[1 1 1] close media player and remove widget, if turn phase (also means zombie not rolled), also update resources UI and show action panel
  (Media|MediaPlayer|Close (Variables|Default|GetspinnerPlayer) :!class /Script/MediaAssets.MediaPlayer)
  (Widget|RemovefromParent (stale EventBeginPlay _output_get))
  (bind _assettlers_game_mode (Utilities|Casting|CastToSettlers_GameMode (Game|GetGameMode)))
  (if (== (Variables|/Game/Settlers_GameMode.Settlers_GameMode_C|Getphase _assettlers_game_mode) 1)
    (CallFunction|UpdateResourcesUI)
    (Default|ShowActionPanel _assettlers_game_mode)))

(event EventBeginPlay
  (bind _returnvalue (UserInterface|CreateWidget "/Game/Blueprints/UI/ResourcesPanel.ResourcesPanel_C"))
  (Variables|Default|SetresourcesUI _returnvalue)
  (bind _returnvalue_2 (UserInterface|CreateWidget "/Game/Blueprints/UI/ResourceSpinner.ResourceSpinner_C"))
  (bind _output_get (Variables|Default|SetspinnerUI _returnvalue_2))
  (Media|MediaPlayer|BindEventtoOnEndReached (Variables|Default|GetspinnerPlayer) (delegate Custom|CloseSpinnerPlayer)))

(event Collision|EventActorBeginOverlap
  (params (OtherActor :type Actor%20Object%20Reference)))

(event EventTick
  (params (DeltaSeconds :type Float%20%28single-precision%29)))

(fn ConstructionScript)

(fn SelectRandomResource
  (bind _outactors (Actor|GetAllActorsOfClass "/Game/Blueprints/HexGrid.HexGrid_C"))
  (bind _keys (Utilities|Map|Keys (Variables|/Game/Blueprints/HexGrid.HexGrid_C|GetresourceAmounts (Utilities|Array|Get(acopy) _outactors))))
  (return (Utilities|Array|Get(acopy) _keys (Math|Random|RandomIntegerinRange 0 (- (Utilities|Map|Length (Variables|/Game/Blueprints/HexGrid.HexGrid_C|GetresourceAmounts (Utilities|Array|Get(acopy) _outactors))) 1)))))

(fn ShowResourcePanel
  (UserInterface|Viewport|AddtoViewport (Variables|Default|GetresourcesUI) 0)
  (CallFunction|UpdateResourcesUI))

(fn UpdateResourcesUI
  (bind _resourcesui (Variables|Default|GetresourcesUI))
  ;[1 1 1] Loop through current player's resource amounts
  (bind _assettlers_game_mode (Utilities|Casting|CastToSettlers_GameMode (Game|GetGameMode)))
  (if (> (Utilities|Array|Length (Variables|/Game/Settlers_GameMode.Settlers_GameMode_C|Getplayers _assettlers_game_mode)) 0)
    (bind _keys (Utilities|Map|Keys (.numResources (Utilities|Struct|BreakBP_PlayerStruct (Utilities|Array|Get(acopy) (Variables|/Game/Settlers_GameMode.Settlers_GameMode_C|Getplayers _assettlers_game_mode) (Variables|/Game/Settlers_GameMode.Settlers_GameMode_C|GetcurrentPlayerIndex _assettlers_game_mode))))))
    (bind _values (Utilities|Map|Values (.numResources (Utilities|Struct|BreakBP_PlayerStruct (Utilities|Array|Get(acopy) (Variables|/Game/Settlers_GameMode.Settlers_GameMode_C|Getplayers _assettlers_game_mode) (Variables|/Game/Settlers_GameMode.Settlers_GameMode_C|GetcurrentPlayerIndex _assettlers_game_mode))))))
    (for _index (range 0 (- (Utilities|Array|Length _keys) 1))
      ;[1 1 1] Update each text value of the resources UI panel accordingly
      (switch string (Utilities|Array|Get(acopy) _keys _index)
        (:wheat
          (Default|SetWheatAmount _resourcesui (Utilities|String|ToString(Integer) (Utilities|Array|Get(acopy) _values _index))))
        (:wood
          (Default|SetWoodAmount _resourcesui (Utilities|String|ToString(Integer) (Utilities|Array|Get(acopy) _values _index))))
        (:brick
          (Default|SetBrickAmount _resourcesui (Utilities|String|ToString(Integer) (Utilities|Array|Get(acopy) _values _index))))
        (:steel
          (Default|SetSteelAmount _resourcesui (Utilities|String|ToString(Integer) (Utilities|Array|Get(acopy) _values _index))))))))

(fn CollectResources
  (params (resource :type String))
  (bind _tempresourcemap (Variables|Default|GettempResourceMap))
  (bind _assettlers_game_mode (Utilities|Casting|CastToSettlers_GameMode (Game|GetGameMode)))
  (if (Utilities|Enum|Equal(Enum) resource "zombie")
    (Default|PlayerSpreadZombie _assettlers_game_mode)
    (else
      (for (_array_element _array_index) (Variables|/Game/Settlers_GameMode.Settlers_GameMode_C|Getplayers _assettlers_game_mode)
        (CallFunction|CopyResourcestoTempMap _array_index)
        ;[1 1 1] check if player has an outpost adjacent to a tile of that resource
        (for _array_element_2 (.vertices (Utilities|Struct|BreakBP_PlayerStruct _array_element))
          (for _array_element_3 (Variables|/Game/Blueprints/HexVertex.HexVertex_C|GetadjacentHexagons _array_element_2)
            (if (Utilities|Enum|Equal(Enum) resource (Variables|/Game/Blueprints/HexTile.HexTile_C|GetresourceType _array_element_3))
              ;[1 1 1] can't collect resource if tile is infected!
              (if (not (Variables|/Game/Blueprints/HexTile.HexTile_C|Getinfected _array_element_3))
                ;[1 1 1] add appropriate amount to temp map
                (Utilities|Map|Add _tempresourcemap resource (+ (.Value (Utilities|Map|Find _tempresourcemap resource)) (Variables|/Game/Blueprints/HexTile.HexTile_C|Getbounty _array_element_3)))))))
        ;[1 1 1] when done with that player, update their resources
        (bind _structout (Utilities|Struct|SetmembersinBP_PlayerStruct _array_element _tempresourcemap))
        (Utilities|Array|SetArrayElem (Variables|/Game/Settlers_GameMode.Settlers_GameMode_C|Getplayers _assettlers_game_mode) _array_index _structout)))))

(fn CollectInitialResources
  (params (vertex :type Hex%20Vertex%20Object%20Reference))
  (bind _tempresourcemap (Variables|Default|GettempResourceMap))
  (bind _assettlers_game_mode (Utilities|Casting|CastToSettlers_GameMode (Game|GetGameMode)))
  (CallFunction|CopyResourcestoTempMap (Variables|/Game/Settlers_GameMode.Settlers_GameMode_C|GetcurrentPlayerIndex _assettlers_game_mode))
  (for _array_element (Variables|/Game/Blueprints/HexVertex.HexVertex_C|GetadjacentHexagons vertex)
    (Utilities|Map|Add _tempresourcemap (Variables|/Game/Blueprints/HexTile.HexTile_C|GetresourceType _array_element) (+ (.Value (Utilities|Map|Find _tempresourcemap (Variables|/Game/Blueprints/HexTile.HexTile_C|GetresourceType _array_element))) (Variables|/Game/Blueprints/HexTile.HexTile_C|Getbounty _array_element))))
  (bind _structout (Utilities|Struct|SetmembersinBP_PlayerStruct (Utilities|Array|Get(acopy) (Variables|/Game/Settlers_GameMode.Settlers_GameMode_C|Getplayers _assettlers_game_mode) (Variables|/Game/Settlers_GameMode.Settlers_GameMode_C|GetcurrentPlayerIndex _assettlers_game_mode)) _tempresourcemap))
  (Utilities|Array|SetArrayElem (Variables|/Game/Settlers_GameMode.Settlers_GameMode_C|Getplayers _assettlers_game_mode) (Variables|/Game/Settlers_GameMode.Settlers_GameMode_C|GetcurrentPlayerIndex _assettlers_game_mode) _structout))

(fn PlayResourceSpinner
  (params (resource :type String))
  (bind _spinnerplayer (Variables|Default|GetspinnerPlayer))
  (UserInterface|Viewport|AddtoViewport (Variables|Default|GetspinnerUI) 0)
  (switch string resource
    (:wheat
      (Media|MediaPlayer|OpenSource _spinnerplayer "/Game/Movies/SpinnerWheat.SpinnerWheat"))
    (:wood
      (Media|MediaPlayer|OpenSource _spinnerplayer "/Game/Movies/SpinnerWood.SpinnerWood"))
    (:brick
      (Media|MediaPlayer|OpenSource _spinnerplayer "/Game/Movies/SpinnerBrick.SpinnerBrick"))
    (:steel
      (Media|MediaPlayer|OpenSource _spinnerplayer "/Game/Movies/SpinnerSteel.SpinnerSteel"))
    (:zombie
      (Media|MediaPlayer|OpenSource _spinnerplayer "/Game/Movies/SpinnerZombie.SpinnerZombie"))))

(fn CheckifEnoughResources
  (params (buildCosts :type Map%20of%20Strings%20to%20Integers))
  (bind _assettlers_game_mode (Utilities|Casting|CastToSettlers_GameMode (Game|GetGameMode)))
  (bind _keys (Utilities|Map|Keys buildCosts))
  (for _array_element _keys
    (if (not (>= (.Value (Utilities|Map|Find (.numResources (Utilities|Struct|BreakBP_PlayerStruct (Utilities|Array|Get(acopy) (Variables|/Game/Settlers_GameMode.Settlers_GameMode_C|Getplayers _assettlers_game_mode) (Variables|/Game/Settlers_GameMode.Settlers_GameMode_C|GetcurrentPlayerIndex _assettlers_game_mode)))) _array_element)) (.Value (Utilities|Map|Find buildCosts _array_element))))
      (return false)))
  (return true))

(fn RemoveResourcefromPlayer
  (params (resources :type Map%20of%20Strings%20to%20Integers))
  (Utilities|FlowControl|Sequence
    (:then_0
      (bind _assettlers_game_mode (Utilities|Casting|CastToSettlers_GameMode (Game|GetGameMode)))
      (CallFunction|CopyResourcestoTempMap (Variables|/Game/Settlers_GameMode.Settlers_GameMode_C|GetcurrentPlayerIndex _assettlers_game_mode)))
    (:then_1
      ;[1 1 1] update resource numbers
      (bind _keys (Utilities|Map|Keys resources))
      (for _array_element _keys
        _))
    (:then_2
      (bind _assettlers_game_mode_2 (Utilities|Casting|CastToSettlers_GameMode (Game|GetGameMode)))
      (bind _structout (Utilities|Struct|SetmembersinBP_PlayerStruct (Utilities|Array|Get(acopy) (Variables|/Game/Settlers_GameMode.Settlers_GameMode_C|Getplayers _assettlers_game_mode_2) (Variables|/Game/Settlers_GameMode.Settlers_GameMode_C|GetcurrentPlayerIndex _assettlers_game_mode_2)) (Variables|Default|GettempResourceMap)))
      (Utilities|Array|SetArrayElem (Variables|/Game/Settlers_GameMode.Settlers_GameMode_C|Getplayers _assettlers_game_mode_2) (Variables|/Game/Settlers_GameMode.Settlers_GameMode_C|GetcurrentPlayerIndex _assettlers_game_mode_2) _structout))))

(fn CopyResourcestoTempMap
  (params (playerIndex :type Integer))
  ;[1 1 1] make temp map a copy of that player's resource map
  (bind _assettlers_game_mode (Utilities|Casting|CastToSettlers_GameMode (Game|GetGameMode)))
  (bind _keys (Utilities|Map|Keys (.numResources (Utilities|Struct|BreakBP_PlayerStruct (Utilities|Array|Get(acopy) (Variables|/Game/Settlers_GameMode.Settlers_GameMode_C|Getplayers _assettlers_game_mode) playerIndex)))))
  (for _array_element _keys
    (Utilities|Map|Add (Variables|Default|GettempResourceMap) _array_element (.Value (Utilities|Map|Find (.numResources (Utilities|Struct|BreakBP_PlayerStruct (Utilities|Array|Get(acopy) (Variables|/Game/Settlers_GameMode.Settlers_GameMode_C|Getplayers _assettlers_game_mode) playerIndex))) _array_element)))))