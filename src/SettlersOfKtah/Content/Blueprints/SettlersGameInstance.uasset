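; SettlersGameInstance is the game instance that handles title-screen menus and multiplayer sessions for the game.
; Show events lazily create, cache and display the multiplayer, pass-and-play, host, join and customization widgets.
; LaunchLobby creates an optionally LAN session and opens the lobby as a listen server, while other events join or destroy sessions.
; SaveGameCheck reports whether the player settings save exists.
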(event Custom|ShowMultiplayerMainMenu
  (bind _returnvalue (Game|GetPlayerController 0))
  ;[1 1 1] show main menu for multiplayer
  (Utilities|IsValid (Variables|Widget|GetMainMenu)
    (:Is%20Valid
      _)
    (:Is%20Not%20Valid
      (bind _returnvalue_2 (UserInterface|CreateWidget "/Game/Blueprints/UI/TitleScreen/TitleScreenUI_Multiplayer.TitleScreenUI_Multiplayer_C" _returnvalue))
      (Variables|Widget|SetMainMenu _returnvalue_2)))
  (UserInterface|Viewport|AddtoViewport (Variables|Widget|GetMainMenu) 0)
  (Variables|/Script/Engine.PlayerController|SetbShowMouseCursor _returnvalue true)
  (Input|SetInputModeGameandUI _returnvalue _returnvalue_2 "DoNotLock" true))

(event Custom|ShowJoinMenu
  ;[1 1 1] show join menu
  (Utilities|IsValid (Variables|Widget|GetJoinMenu)
    (:Is%20Valid
      _)
    (:Is%20Not%20Valid
      (bind _returnvalue (UserInterface|CreateWidget "/Game/Blueprints/UI/TitleScreen/Multiplayer_Join.Multiplayer_Join_C" (Game|GetPlayerController 0)))
      (Variables|Widget|SetJoinMenu _returnvalue)))
  (UserInterface|Viewport|AddtoViewport (Variables|Widget|GetJoinMenu) 0))

(event Custom|ShowHostMenu
  ;[1 1 1] show host game menu
  (Utilities|IsValid (Variables|Widget|GetHostMenu)
    (:Is%20Valid
      _)
    (:Is%20Not%20Valid
      (bind _returnvalue (UserInterface|CreateWidget "/Game/Blueprints/UI/TitleScreen/Multiplayer_Host.Multiplayer_Host_C" (Game|GetPlayerController 0)))
      (Variables|Widget|SetHostMenu _returnvalue)))
  (UserInterface|Viewport|AddtoViewport (Variables|Widget|GetHostMenu) 0))

(event Custom|ShowPassAndPlayMenu
  ;[1 1 1] show pass and play menu
  (Utilities|IsValid (Variables|Widget|GetPassAndPlayMenu)
    (:Is%20Valid
      _)
    (:Is%20Not%20Valid
      (bind _returnvalue (UserInterface|CreateWidget "/Game/Blueprints/UI/TitleScreen/TitleScreenUI.TitleScreenUI_C" (Game|GetPlayerController 0)))
      (Variables|Widget|SetPassAndPlayMenu _returnvalue)))
  (UserInterface|Viewport|AddtoViewport (Variables|Widget|GetPassAndPlayMenu) 0))

(event Custom|LaunchLobby
  (params (serverName :type Text) (numberOfPlayers :type Integer) (enableLAN :type Boolean))
  ;[1 1 1] Launches lobby
  (bind _output_get (Variables|ServerSettings|SetmaxPlayers numberOfPlayers))
  (Variables|ServerSettings|SetserverName serverName)
  (|Session (Game|GetPlayerController 0) _output_get enableLAN
    (:OnSuccess
      (Game|OpenLevel(byName) "Lobby_Multiplayer" true "listen"))
    (:OnFailure
      (Development|PrintString "failed to create session!"))))

(event Custom|JoinServer
  (params (sessionToJoin :type Blueprint%20Session%20Result%20Structure))
  ;[1 1 1] join server -- called from join menu
  (|JoinSession (Game|GetPlayerController 0) sessionToJoin
    (:OnFailure
      (Development|PrintString "failed to join session!"))))

(event Custom|DestroySessionCaller
  (params (playerController :type Player%20Controller%20Object%20Reference))
  ;[1 1 1] destroys session -- called when exit lobby
  (|DestroySession playerController))

(event Custom|ShowCustomizationMenu
  (params (forwardToHostMenu :type Boolean))
  ;[1 1 1] show player customization menu
  (Utilities|IsValid (Variables|Widget|GetCustomizationMenu)
    (:Is%20Valid
      _)
    (:Is%20Not%20Valid
      (bind _returnvalue (UserInterface|CreateWidget "/Game/Blueprints/UI/TitleScreen/PlayerCustomizationMenu.PlayerCustomizationMenu_C" (Game|GetPlayerController 0) forwardToHostMenu))
      (Variables|Widget|SetCustomizationMenu _returnvalue)))
  (UserInterface|Viewport|AddtoViewport (Variables|Widget|GetCustomizationMenu) 0))

(fn SaveGameCheck
  (bind _returnvalue (SaveGame|DoesSaveGameExist (Variables|Default|GetPlayerSettingsSave)))
  (return _returnvalue))