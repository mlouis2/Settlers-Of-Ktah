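; ZombieHandler runs the zombie horde in a hex-tile Settlers-style game, covering infection spread, battles and player elimination.
; The horde randomly infects neighbors of infected tiles, fighting for castle tiles, while a phase-gated player action relocates an existing infection.
; Battles compare the grid's infected-tile count against the player's knights.
; Wins award defense points; losses remove knights and eliminate owners whose castle tiles are all infected.
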(event EventBeginPlay)

(event Collision|EventActorBeginOverlap
  (params (OtherActor :type Actor%20Object%20Reference)))

(event EventTick
  (params (DeltaSeconds :type Float%20%28single-precision%29)))

(fn ConstructionScript)

(fn PlayerSpreadZombie
  (bind _assettlers_game_mode (Utilities|Casting|CastToSettlers_GameMode (Game|GetGameMode)))
  (Variables|/Game/Settlers_GameMode.Settlers_GameMode_C|Setphase _assettlers_game_mode 2)
  (CallFunction|HighlightPossibleZombieTiles))

(fn MaybeGrowZombie
  (if (< (Math|Random|RandomFloat) 0.5)
    (bind _assettlers_game_mode (Utilities|Casting|CastToSettlers_GameMode (Game|GetGameMode)))
    (Default|AddMessage (Variables|/Game/Settlers_GameMode.Settlers_GameMode_C|GetgameLog _assettlers_game_mode) "The horde has infected another tile!")
    (CallFunction|SpreadZombie)))

(fn DetermineBattleOutcome
  (params (playerIndex :type Integer))
  (bind _assettlers_game_mode (Utilities|Casting|CastToSettlers_GameMode (Game|GetGameMode)))
  (bind _returnvalue (Actor|GetActorOfClass "/Game/Blueprints/HexGrid.HexGrid_C"))
  (return (> (Variables|/Game/Blueprints/HexGrid.HexGrid_C|GetnumTilesInfected _returnvalue) (.numKnights (Utilities|Struct|BreakBP_PlayerStruct (Utilities|Array|Get(acopy) (Variables|/Game/Settlers_GameMode.Settlers_GameMode_C|Getplayers _assettlers_game_mode) playerIndex))))))

(fn HandlePlayerVictory
  (params (playerIndex :type Integer) (battleTile :type Hex%20Tile%20Object%20Reference))
  (bind _assettlers_game_mode (Utilities|Casting|CastToSettlers_GameMode (Game|GetGameMode)))
  (Default|UninfectTile battleTile)
  (Utilities|Struct|SetmembersinBP_PlayerStruct (Utilities|Array|Get(acopy) (Variables|/Game/Settlers_GameMode.Settlers_GameMode_C|Getplayers _assettlers_game_mode) playerIndex) (+ (.numDefensePoints (Utilities|Struct|BreakBP_PlayerStruct (Utilities|Array|Get(acopy) (Variables|/Game/Settlers_GameMode.Settlers_GameMode_C|Getplayers _assettlers_game_mode) playerIndex))) 1))
  (Default|UpdatePlayerDefensePoints (Variables|/Game/Settlers_GameMode.Settlers_GameMode_C|GetplayerUI _assettlers_game_mode) playerIndex))

(fn HandlePlayerLoss
  (params (playerIndex :type Integer) (battleTile :type Hex%20Tile%20Object%20Reference))
  (bind _tileownerplayerindex (Variables|/Game/Blueprints/HexTile.HexTile_C|GettileOwnerPlayerIndex battleTile))
  (Default|InfectTile battleTile)
  ;[1 1 1] take away attacking player's knight
  (Default|RemovePlayerKnights battleTile playerIndex)
  ;[1 1 1] kick player who owns tile out of game if both their castle tiles are infected now
  (bind _assettlers_game_mode (Utilities|Casting|CastToSettlers_GameMode (Game|GetGameMode)))
  (for _array_element (.castleTiles (Utilities|Struct|BreakBP_PlayerStruct (Utilities|Array|Get(acopy) (Variables|/Game/Settlers_GameMode.Settlers_GameMode_C|Getplayers _assettlers_game_mode) _tileownerplayerindex)))
    (if (not (Variables|/Game/Blueprints/HexTile.HexTile_C|Getinfected _array_element))
      (return)))
  (Utilities|Struct|SetmembersinBP_PlayerStruct (Utilities|Array|Get(acopy) (Variables|/Game/Settlers_GameMode.Settlers_GameMode_C|Getplayers _assettlers_game_mode) _tileownerplayerindex) true)
  (bind _assettlers_game_mode_2 (Utilities|Casting|CastToSettlers_GameMode (Game|GetGameMode)))
  (Default|UpdateLosingPlayerUI (Variables|/Game/Settlers_GameMode.Settlers_GameMode_C|GetplayerUI _assettlers_game_mode_2) _tileownerplayerindex)
  (Default|CheckforLoneSurvivorVictory _assettlers_game_mode_2))

(fn HandleZombieBattle
  (params (attackingPlayerIndex :type Integer) (battleTile :type Hex%20Tile%20Object%20Reference))
  ;[1 1 1] Determines who won the battle and calls win/loss functions accordingly.
  (bind _assettlers_game_mode (Utilities|Casting|CastToSettlers_GameMode (Game|GetGameMode)))
  (bind _loss (CallFunction|DetermineBattleOutcome attackingPlayerIndex))
  (if _loss
    (CallFunction|HandlePlayerLoss attackingPlayerIndex battleTile)
    (else
      (CallFunction|HandlePlayerVictory attackingPlayerIndex battleTile)))
  (Default|AddPlayerVictoryorLossMessage (Variables|/Game/Settlers_GameMode.Settlers_GameMode_C|GetgameLog _assettlers_game_mode) _loss attackingPlayerIndex)
  (return _loss))

(fn MaybeInfectTile
  (params (tile :type Hex%20Tile%20Object%20Reference))
  ;[1 1 1] First, check that we're in zombie spread phase
  (bind _assettlers_game_mode (Utilities|Casting|CastToSettlers_GameMode (Game|GetGameMode)))
  (if (== (Variables|/Game/Settlers_GameMode.Settlers_GameMode_C|Getphase _assettlers_game_mode) 2)
    (if (Variables|/Game/Blueprints/HexTile.HexTile_C|Getinfected tile)
      ;[1 1 1] Cannot transfer zombie base tile
      (if (Utilities|Enum|NotEqual(Enum) (Variables|/Game/Blueprints/HexTile.HexTile_C|GetresourceType tile) "zombie")
        ;[1 1 1] Cannot transfer tile with castle
        (if (not (Utilities|IsValid (Variables|/Game/Blueprints/HexTile.HexTile_C|Getcastle tile)))
          ;[1 1 1] If the tile is infected, we'll transfer that infection, so set the tile to transfer.
          (Variables|Default|SettileToTransfer tile)
          (Development|PrintString "picked up tile to transfer")))
      (else
        ;[1 1 1] If the selected tile is not infected, check if we've already selected a tile to transfer (so that we can transfer to this tile).
        (if (Utilities|IsValid (Variables|Default|GettileToTransfer))
          (if (not (Utilities|IsValid (Variables|/Game/Blueprints/HexTile.HexTile_C|Getcastle tile)))
            (Default|InfectTile tile)
            (Default|UninfectTile (Variables|Default|GettileToTransfer))
            (Variables|Default|SettileToTransfer 0)
            (Variables|/Game/Settlers_GameMode.Settlers_GameMode_C|Setphase _assettlers_game_mode 1)
            (Default|UpdateButtons (Variables|/Game/Settlers_GameMode.Settlers_GameMode_C|GetactionsUI _assettlers_game_mode))))))))

(fn CheckifZombieRollIsValid
  ;[1 1 1] If there aren't two infected tiles, it's invalid.
  (bind _returnvalue (Actor|GetActorOfClass "/Game/Blueprints/HexGrid.HexGrid_C"))
  (if (>= (Variables|/Game/Blueprints/HexGrid.HexGrid_C|GetnumTilesInfected _returnvalue) 2)
    ;[1 1 1] Is there an infected tile...
    (bind _values (Utilities|Map|Values (Variables|/Game/Blueprints/HexGrid.HexGrid_C|GethexagonTileActors _returnvalue)))
    (for _array_element _values
      ;[1 1 1] ...without a castle...
      (if (Variables|/Game/Blueprints/HexTile.HexTile_C|Getinfected _array_element)
        (if (not (Utilities|IsValid (Variables|/Game/Blueprints/HexTile.HexTile_C|Getcastle _array_element)))
          ;[1 1 1] ...that isn't a zombie base...
          (if (not (Utilities|Enum|Equal(Enum) (Variables|/Game/Blueprints/HexTile.HexTile_C|GetresourceType _array_element) "zombie"))
            (return true)))))
    (return false)
    (else
      (return false))))

(fn HighlightPossibleZombieTiles
  (bind _outactors (Actor|GetAllActorsOfClass "/Game/Blueprints/HexTile.HexTile_C"))
  (for _array_element _outactors
    (bind _ashex_tile (Utilities|Casting|CastToHexTile _array_element))
    (if (not (Utilities|IsValid (Variables|/Game/Blueprints/HexTile.HexTile_C|Getcastle _ashex_tile)))
      (if (not (Variables|/Game/Blueprints/HexTile.HexTile_C|Getinfected _ashex_tile))
        (Default|HighlightTile _ashex_tile)))))

(fn SpreadZombie
  (bind _possiblezombiespreadtiles (Variables|Default|GetpossibleZombieSpreadTiles))
  (bind _returnvalue (Utilities|Array|Length _possiblezombiespreadtiles))
  ;[1 1 1] Loop through all hexagon tiles in grid
  (bind _returnvalue_2 (Actor|GetActorOfClass "/Game/Blueprints/HexGrid.HexGrid_C"))
  (bind _values (Utilities|Map|Values (Variables|/Game/Blueprints/HexGrid.HexGrid_C|GethexagonTileActors _returnvalue_2)))
  (for _array_element _values
    ;[1 1 1] If they're infected, look at their neighbors
    (if (Variables|/Game/Blueprints/HexTile.HexTile_C|Getinfected _array_element)
      (for _array_element_2 (Variables|/Game/Blueprints/HexTile.HexTile_C|GetadjacentHexagons _array_element)
        ;[1 1 1] If adjacent tile isn't infected, add it to possible spread tiles
        (if (not (Variables|/Game/Blueprints/HexTile.HexTile_C|Getinfected _array_element_2))
          (Utilities|Array|Add (Variables|Default|GetpossibleZombieSpreadTiles) _array_element_2)))))
  ;[1 1 1] Pick a random tile and spread zombie! Also check if there's a castle and handle battle accordingly.
  (if (> _returnvalue 0)
    (bind _output_get (Variables|Default|SettileToTransfer (Utilities|Array|Get(acopy) _possiblezombiespreadtiles (Math|Random|RandomInteger (- _returnvalue 1)))))
    (if (Utilities|IsValid (Variables|/Game/Blueprints/HexTile.HexTile_C|Getcastle _output_get))
      (bind _loss (Default|HandleZombieBattle _output_get (Variables|/Game/Blueprints/HexTile.HexTile_C|GettileOwnerPlayerIndex _output_get) _output_get))
      (if _loss
        (Default|InfectTile _output_get :!label _label)
        (Variables|/Game/Blueprints/HexGrid.HexGrid_C|SetnumTilesInfected _returnvalue_2 (+ (Variables|/Game/Blueprints/HexGrid.HexGrid_C|GetnumTilesInfected _returnvalue_2) 1))
        (Utilities|Array|Clear (Variables|Default|GetpossibleZombieSpreadTiles)))
      (else
        (goto _label)))
    (Variables|Default|SettileToTransfer 0)))

(fn HandlePlayerAttack)